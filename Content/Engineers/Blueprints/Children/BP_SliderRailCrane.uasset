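; Spline slider control that drives one axis of a rail crane, horizontal with the left-hand magnet key or inward with the right.
; While the powered key overlaps the ball, Tick pins it to the nearest spline point.
; With controls enabled, its normalized spline position, outside a central deadzone, sets crane physics velocity within travel limits.
; Key release or exit recenters the ball, halts the crane and fades out movement audio.
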(event Custom|SnapBackToMiddle
  (bind _craneobject (Variables|Default|GetCraneObject))
  (bind _path (Variables|Default|GetPath))
  (bind _craneobject_2 (Variables|Default|GetCraneObject))
  (bind _craneobject_3 (Variables|Default|GetCraneObject))
  (Transformation|SetWorldLocation (Variables|Default|GetBall) (Spline|GetLocationatDistanceAlongSpline _path (/ (Spline|GetSplineLength _path) 2.0) "World") false false)
  (switch Utilities|FlowControl|Switch|SwitchonSliderCraneTypes (Variables|Default|GetType)
    (:NewEnumerator0
      _)
    (:NewEnumerator1
      (Physics|SetPhysicsLinearVelocity (Variables|/Game/Engineers/Blueprints/Misc/BP_Crane.BP_Crane_C|GetMiddleRail _craneobject_2) "0, 0, 0" false "None")))
  (Physics|SetPhysicsLinearVelocity (Variables|/Game/Engineers/Blueprints/Misc/BP_Crane.BP_Crane_C|GetCraneTop _craneobject_2) "0, 0, 0" false "None")
  (switch Utilities|FlowControl|Switch|SwitchonSliderCraneTypes (Variables|Default|GetType)
    (:NewEnumerator0
      (Audio|Components|Audio|FadeOut (Variables|/Game/Engineers/Blueprints/Misc/BP_Crane.BP_Crane_C|GetCrane_Movement_Horizontal _craneobject) 0.5 0.0 :!class /Script/Engine.AudioComponent)
      (Utilities|FlowControl|DoOnce false) ; enters at Reset
    )
    (:NewEnumerator1
      (Audio|Components|Audio|FadeOut (Variables|/Game/Engineers/Blueprints/Misc/BP_Crane.BP_Crane_C|GetCrane_Movement_Inward _craneobject) 0.5 0.0 :!class /Script/Engine.AudioComponent)
      (Utilities|FlowControl|DoOnce false) ; enters at Reset
    )))

(event EventBeginPlay
  (bind _path (Variables|Default|GetPath))
  (Transformation|SetWorldLocation (Variables|Default|GetBall) (Spline|GetLocationatDistanceAlongSpline _path (/ (Spline|GetSplineLength _path) 2.0) "World") false true))

(event EventTick
  (params (DeltaSeconds :type Float%20%28single-precision%29))
  (bind _craneobject (Variables|Default|GetCraneObject))
  (bind _craneobject_2 (Variables|Default|GetCraneObject))
  (bind _path (Variables|Default|GetPath))
  (bind _craneobject_3 (Variables|Default|GetCraneObject))
  (bind _craneobject_4 (Variables|Default|GetCraneObject))
  (bind _magnetkey (Variables|Default|GetmagnetKey))
  (bind _path_2 (Variables|Default|GetPath))
  (bind _craneobject_5 (Variables|Default|GetCraneObject))
  (bind _middlerail (Variables|/Game/Engineers/Blueprints/Misc/BP_Crane.BP_Crane_C|GetMiddleRail _craneobject_3))
  (bind _middlerail_2 (Variables|/Game/Engineers/Blueprints/Misc/BP_Crane.BP_Crane_C|GetMiddleRail _craneobject_5))
  (bind _cranetop (Variables|/Game/Engineers/Blueprints/Misc/BP_Crane.BP_Crane_C|GetCraneTop _craneobject))
  (bind _cranetop_2 (Variables|/Game/Engineers/Blueprints/Misc/BP_Crane.BP_Crane_C|GetCraneTop _craneobject_2))
  (bind _magnettrigger (Variables|/Game/Engineers/Blueprints/Parents/BP_MagnetKey.BP_MagnetKey_C|GetMagnetTrigger _magnetkey))
  (bind _cranetop_3 (Variables|/Game/Engineers/Blueprints/Misc/BP_Crane.BP_Crane_C|GetCraneTop _craneobject_5))
  (bind _cranetop_4 (Variables|/Game/Engineers/Blueprints/Misc/BP_Crane.BP_Crane_C|GetCraneTop _craneobject_3))
  (bind _returnvalue (Transformation|GetComponentVelocity _cranetop_2))
  (bind _returnvalue_2 (Transformation|GetComponentVelocity _cranetop))
  (bind _returnvalue_3 (Transformation|GetComponentVelocity _cranetop_4))
  (bind _returnvalue_4 (Transformation|GetComponentVelocity _cranetop_3))
  (bind _returnvalue_5 (Transformation|GetWorldLocation _magnettrigger))
  (bind _returnvalue_6 (Spline|FindLocationClosesttoWorldLocation _path_2 _returnvalue_5 "World"))
  (if (and (Variables|Default|GetisInteractingWithMagnetKey) (Utilities|IsValid _magnetkey))
    (if (and (Variables|/Game/Engineers/Blueprints/Parents/BP_MagnetKey.BP_MagnetKey_C|GetisOn _magnetkey) (Class|PrimitiveComponent|IsOverlappingComponent _magnettrigger (Variables|Default|GetBall)))
      (Utilities|FlowControl|Sequence
        (:then_0
          (Utilities|FlowControl|DoOnce false
            (:Completed
              (switch Utilities|FlowControl|Switch|SwitchonSliderCraneTypes (Variables|Default|GetType)
                (:NewEnumerator0
                  (Audio|Components|Audio|FadeIn (Variables|/Game/Engineers/Blueprints/Misc/BP_Crane.BP_Crane_C|GetCrane_Movement_Horizontal _craneobject_4) 0.5 1.0 0.0 :!class /Script/Engine.AudioComponent))
                (:NewEnumerator1
                  (Audio|Components|Audio|FadeIn (Variables|/Game/Engineers/Blueprints/Misc/BP_Crane.BP_Crane_C|GetCrane_Movement_Inward _craneobject_4) 0.5 1.0 0.0 :!class /Script/Engine.AudioComponent))))))
        (:then_1
          (Transformation|SetWorldLocation (Variables|Default|GetBall) _returnvalue_6 false true)
          (bind _distance (CallFunction|FindDistanceAlongSpline _path _returnvalue_6))
          (Variables|Default|SetBallDistance (/ _distance (Math|Conversions|ToFloat(Integer) (- (Spline|GetNumberOfSplinePoints _path) 1))))
          (if (Variables|Default|GetcontrolsEnabled)
            (switch Utilities|FlowControl|Switch|SwitchonSliderCraneTypes (Variables|Default|GetType)
              (:NewEnumerator0
                (if (>= (Variables|Default|GetBallDistance) 0.55)
                  (if (<= (- (.y (Variables|/Script/Engine.SceneComponent|GetRelativeLocation _cranetop_2)) (.y (Transformation|GetActorLocation _craneobject_2))) 1e+03)
                    (Physics|SetPhysicsLinearVelocity _cranetop_2 (Math|Vector|MakeVector (.x _returnvalue) (Math|Float|MapRangeClamped (Variables|Default|GetBallDistance) 0.55 1.0 0.0 (Variables|Default|GetMaxCraneSpeed)) 0.0) false "None")
                    (else
                      (Physics|SetPhysicsLinearVelocity _cranetop_2 (Math|Vector|MakeVector (.x _returnvalue) 0.0 0.0) false "None")))
                  (elif (<= (Variables|Default|GetBallDistance) 0.45)
                    (if (>= (- (.y (Variables|/Script/Engine.SceneComponent|GetRelativeLocation _cranetop)) (.y (Transformation|GetActorLocation _craneobject))) 0.0)
                      (Physics|SetPhysicsLinearVelocity _cranetop (Math|Vector|MakeVector (.x _returnvalue_2) (Math|Float|MapRangeClamped (Variables|Default|GetBallDistance) 0.45 0.0 0.0 (* (Variables|Default|GetMaxCraneSpeed) -1.0)) 0.0) false "None")
                      (else
                        (Physics|SetPhysicsLinearVelocity _cranetop (Math|Vector|MakeVector (.x _returnvalue_2) 0.0 0.0) false "None"))))))
              (:NewEnumerator1
                (if (>= (Variables|Default|GetBallDistance) 0.55)
                  (if (<= (- (.x (Variables|/Script/Engine.SceneComponent|GetRelativeLocation _cranetop_4)) (.x (Transformation|GetActorLocation _craneobject_3))) 2.07e+03)
                    (Physics|SetPhysicsLinearVelocity _cranetop_4 (Math|Vector|MakeVector (Math|Float|MapRangeClamped (Variables|Default|GetBallDistance) 0.55 1.0 0.0 (Variables|Default|GetMaxCraneSpeed)) (.y _returnvalue_3) 0.0) false "None")
                    (Physics|SetPhysicsLinearVelocity _middlerail (Math|Vector|MakeVector (Math|Float|MapRangeClamped (Variables|Default|GetBallDistance) 0.55 1.0 0.0 (Variables|Default|GetMaxCraneSpeed)) 0.0 0.0) false "None")
                    (else
                      (Physics|SetPhysicsLinearVelocity _cranetop_4 (Math|Vector|MakeVector 0.0 (.y _returnvalue_3) 0.0) false "None")
                      (Physics|SetPhysicsLinearVelocity _middlerail "0, 0, 0" false "None")))
                  (elif (<= (Variables|Default|GetBallDistance) 0.45)
                    (if (>= (- (.x (Variables|/Script/Engine.SceneComponent|GetRelativeLocation _cranetop_3)) (.x (Transformation|GetActorLocation _craneobject_5))) 0.0)
                      (Physics|SetPhysicsLinearVelocity _cranetop_3 (Math|Vector|MakeVector (Math|Float|MapRangeClamped (Variables|Default|GetBallDistance) 0.45 0.0 0.0 (* (Variables|Default|GetMaxCraneSpeed) -1.0)) (.y _returnvalue_4) 0.0) false "None")
                      (Physics|SetPhysicsLinearVelocity _middlerail_2 (Math|Vector|MakeVector (Math|Float|MapRangeClamped (Variables|Default|GetBallDistance) 0.45 0.0 0.0 (* (Variables|Default|GetMaxCraneSpeed) -1.0)) 0.0 0.0) false "None")
                      (else
                        (Physics|SetPhysicsLinearVelocity _cranetop_3 (Math|Vector|MakeVector 0.0 (.y _returnvalue_4) 0.0) false "None")
                        (Physics|SetPhysicsLinearVelocity _middlerail_2 "0, 0, 0" false "None")))))))))))))

(event Collision|EventActorBeginOverlap
  (params (OtherActor :type Actor%20Object%20Reference))
  (bind _type (Variables|Default|GetType))
  (bind _asbp_magnet_key (Utilities|Casting|CastToBP_MagnetKey OtherActor))
  (if (or (and (Utilities|Enum|Equal(Enum) (Variables|/Game/Engineers/Blueprints/Parents/BP_MagnetKey.BP_MagnetKey_C|GetHand _asbp_magnet_key) "Left") (Utilities|Enum|Equal(Enum) _type "NewEnumerator0")) (and (Utilities|Enum|Equal(Enum) _type "NewEnumerator1") (Utilities|Enum|Equal(Enum) (Variables|/Game/Engineers/Blueprints/Parents/BP_MagnetKey.BP_MagnetKey_C|GetHand _asbp_magnet_key) "Right")))
    (Variables|Default|SetisInteractingWithMagnetKey true)
    (bind _output_get (Variables|Default|SetmagnetKey _asbp_magnet_key))
    (Default|TurnOffLight _asbp_magnet_key)
    (EventDispatchers|BindEventtoTurnedOff _output_get (delegate Custom|SnapBackToMiddle))))

(event Collision|EventActorEndOverlap
  (params (OtherActor :type Actor%20Object%20Reference))
  (Utilities|Casting|CastToBP_MagnetKey OtherActor)
  (Variables|Default|SetisInteractingWithMagnetKey false)
  (CallFunction|SnapBacktoMiddle)
  (EventDispatchers|UnbindEventfromTurnedOff (Variables|Default|GetmagnetKey) (delegate Custom|SnapBackToMiddle))
  (Variables|Default|SetmagnetKey 0))

(fn ConstructionScript
  (bind _path (Variables|Default|GetPath))
  (for _index (range 0 (- (Spline|GetNumberOfSplinePoints (Variables|Default|GetPath)) 2))
    (bind _returnvalue (AddComponent|AddSplineMeshComponent false))
    (Components|StaticMesh|SetStaticMesh _returnvalue (Variables|Default|GetpathMesh))
    (SplineMesh|SetForwardAxis _returnvalue (Variables|Default|GetForward%20Axis) true)
    (Transformation|AttachComponentToComponent _returnvalue (Variables|Default|GetPath) "None" "KeepRelative" "KeepRelative" "KeepRelative" true)
    (SplineMesh|SetStartandEnd _returnvalue (Spline|GetLocationatSplinePoint _path _index "Local") (Spline|GetTangentatSplinePoint _path _index "Local") (Spline|GetLocationatSplinePoint _path (+ _index 1) "Local") (Spline|GetTangentatSplinePoint _path (+ _index 1) "Local") true :!class /Script/Engine.SplineMeshComponent)))

(fn FindDistanceAlongSpline
  (params (Spline :type Spline%20Component%20Object%20Reference) (Location :type Vector))
  (return (Class|SplineComponent|FindInputKeyClosesttoWorldLocation Spline Location)))