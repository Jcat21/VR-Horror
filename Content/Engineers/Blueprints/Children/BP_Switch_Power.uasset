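; Power switch Blueprint: a hand-grabbable rotating lever that toggles between ON and OFF states.
; Grabable limits the lever to a rotational grab on one axis, snaps it to the OFF end at start if IsOff is set, and reports movement to Moved.
; Moved flips IsOff only near either end of travel, giving hysteresis, then updates the PowerButton color and caption and plays a click sound.
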(event Custom|Moved
  (params (Value :type Float%20%28single-precision%29))
  (bind _powerbutton (Variables|Default|GetPowerButton))
  (if (and (>= Value -1e+01) (Variables|Default|GetIsOff))
    (Variables|Default|SetIsOff false)
    (Default|ChangeButtonColor _powerbutton "(R=0.072538,G=1.000000,B=0.000000,A=1.000000)")
    (Default|SetCaption _powerbutton "ON")
    (Audio|PlaySoundatLocation "/Game/Artists/Audio/Sounds/Power_Button_02.Power_Button_02" (Transformation|GetActorLocation) "0, 0, 0" 0.25 :!label _label)
    (elif (and (<= Value -1.7e+02) (not (Variables|Default|GetIsOff)))
      (Variables|Default|SetIsOff true)
      (Default|ChangeButtonColor _powerbutton "(R=1.000000,G=0.000000,B=0.014146,A=1.000000)")
      (Default|SetCaption _powerbutton "OFF")
      (goto _label))))

(event EventBeginPlay
  (bind _grabable (Variables|Default|GetGrabable))
  (bind _switchlevertop (Variables|Default|GetSwitchLeverTop))
  (Default|SetRotationalGrab _grabable "Y" _switchlevertop _switchlevertop "14.000000, 0, 0" -1.8e+02 0.0 true 1e+01 "/Game/Artists/Animation/Anims/HandAnims/anim_fist.anim_fist")
  (EventDispatchers|BindEventtoMoveNotify _grabable (delegate Custom|Moved))
  (if (Variables|Default|GetIsOff)
    (Default|MovetoDistance _grabable -1.8e+02)))

(fn ConstructionScript)