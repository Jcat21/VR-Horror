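; Puzzle slider whose ball is dragged along a spline rail by a hand-matched BP_MagnetKey to rotate one colored anchor on a linked RotatorPuzzle.
; Tick pins the ball to the spline point nearest the active magnet and maps normalized spline input key to anchor roll.
; Magnet switch-off snaps to the nearest third, stores that color's value and opens the door when all three match.
; Construction script builds the rail from spline meshes.
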(event Custom|SnapAndSetColorValues
  (bind _path (Variables|Default|GetPath))
  (bind _rotatorpuzzle (Variables|Default|GetRotatorPuzzle))
  (bind _path_2 (Variables|Default|GetPath))
  (bind _rotatorpuzzle_2 (Variables|Default|GetRotatorPuzzle))
  (bind _currentvalues (Variables|/Game/Engineers/Blueprints/Children/BP_RotatorPuzzle_Cryo.BP_RotatorPuzzle_Cryo_C|GetCurrentValues _rotatorpuzzle))
  (bind _distance (CallFunction|FindDistanceAlongSpline _path_2 (Transformation|GetWorldLocation (Variables|Default|GetBall))))
  (bind _output (CallFunction|FindNearestThird (/ _distance (Math|Conversions|ToFloat(Integer) (- (Spline|GetNumberOfSplinePoints _path_2) 1)))))
  (Utilities|FlowControl|Sequence
    (:then_0
      (Transformation|SetWorldLocation (Variables|Default|GetBall) (Spline|GetLocationatDistanceAlongSpline _path (* (Spline|GetSplineLength _path) _output) "World") false true))
    (:then_1
      (switch Utilities|FlowControl|Switch|SwitchonSliderRotatorTypes (Variables|Default|GetType)
        (:NewEnumerator0
          (Transformation|SetRelativeRotation (Variables|/Game/Engineers/Blueprints/Children/BP_RotatorPuzzle_Cryo.BP_RotatorPuzzle_Cryo_C|GetRedAnchor _rotatorpuzzle_2) (Math|Rotator|MakeRotator (Math|Float|MapRangeClamped _output 0.0 1.0 0.0 2.7e+02) 0.0 0.0) false false)
          (Utilities|Map|Add _currentvalues "Red" (Math|Float|Truncate (* _output 3.0))))
        (:NewEnumerator1
          (Transformation|SetRelativeRotation (Variables|/Game/Engineers/Blueprints/Children/BP_RotatorPuzzle_Cryo.BP_RotatorPuzzle_Cryo_C|GetBlueAnchor _rotatorpuzzle_2) (Math|Rotator|MakeRotator (Math|Float|MapRangeClamped _output 0.0 1.0 0.0 2.7e+02) 0.0 0.0) false false)
          (Utilities|Map|Add _currentvalues "Blue" (Math|Float|Truncate (* _output 3.0))))
        (:NewEnumerator2
          (Transformation|SetRelativeRotation (Variables|/Game/Engineers/Blueprints/Children/BP_RotatorPuzzle_Cryo.BP_RotatorPuzzle_Cryo_C|GetPurpleAnchor _rotatorpuzzle_2) (Math|Rotator|MakeRotator (Math|Float|MapRangeClamped _output 0.0 1.0 0.0 2.7e+02) 0.0 0.0) false false)
          (Utilities|Map|Add _currentvalues "Purple" (Math|Float|Truncate (* _output 3.0))))))))

(event Custom|SnapAndCheckSolved
  (bind _rotatorpuzzle (Variables|Default|GetRotatorPuzzle))
  (bind _audio (Variables|Default|GetAudio))
  (if (not (Variables|/Game/Engineers/Blueprints/Children/BP_RotatorPuzzle_Cryo.BP_RotatorPuzzle_Cryo_C|GetisOpen (Variables|Default|GetRotatorPuzzle)))
    (CallFunction|SnapandSetColorValues)
    (if (not (Audio|Components|Audio|IsPlaying _audio))
      (Audio|Components|Audio|Play _audio 0.0)
      (bind _didsolve (CallFunction|CheckSolved))
      (if (and _didsolve (not (Variables|/Game/Engineers/Blueprints/Children/BP_RotatorPuzzle_Cryo.BP_RotatorPuzzle_Cryo_C|GetSolved _rotatorpuzzle)))
        (Default|OpenDoor _rotatorpuzzle)))))

(event EventBeginPlay
  (bind _ball (Variables|Default|GetBall))
  (Transformation|SetWorldLocation (Variables|Default|GetBall) (Spline|GetLocationatDistanceAlongSpline (Variables|Default|GetPath) 0.0 "World") false true)
  (switch Utilities|FlowControl|Switch|SwitchonSliderRotatorTypes (Variables|Default|GetType)
    (:NewEnumerator0
      (Rendering|Material|SetMaterial _ball 0 "/Game/Artists/Materials/M_LeftMagnetKeyTurnedON.M_LeftMagnetKeyTurnedON"))
    (:NewEnumerator1
      (Rendering|Material|SetMaterial _ball 0 "/Game/Artists/Materials/M_RightMagnetKeyTurnedON.M_RightMagnetKeyTurnedON"))
    (:NewEnumerator2
      (Rendering|Material|SetMaterial _ball 0 "/Game/Artists/Materials/M_MagnetKeyBothBright.M_MagnetKeyBothBright"))))

(event EventTick
  (params (DeltaSeconds :type Float%20%28single-precision%29))
  (bind _path (Variables|Default|GetPath))
  (bind _magnetkey (Variables|Default|GetmagnetKey))
  (bind _path_2 (Variables|Default|GetPath))
  (bind _rotatorpuzzle (Variables|Default|GetRotatorPuzzle))
  (bind _magnettrigger (Variables|/Game/Engineers/Blueprints/Parents/BP_MagnetKey.BP_MagnetKey_C|GetMagnetTrigger _magnetkey))
  (bind _returnvalue (Transformation|GetWorldLocation _magnettrigger))
  (bind _returnvalue_2 (Spline|FindLocationClosesttoWorldLocation _path_2 _returnvalue "World"))
  (if (and (Variables|Default|GetisInteractingWithMagnetKey) (Utilities|IsValid _magnetkey))
    (if (and (Variables|/Game/Engineers/Blueprints/Parents/BP_MagnetKey.BP_MagnetKey_C|GetisOn _magnetkey) (Class|PrimitiveComponent|IsOverlappingComponent _magnettrigger (Variables|Default|GetBall)))
      (Transformation|SetWorldLocation (Variables|Default|GetBall) _returnvalue_2 false true)
      (bind _distance (CallFunction|FindDistanceAlongSpline _path _returnvalue_2))
      (switch Utilities|FlowControl|Switch|SwitchonSliderRotatorTypes (Variables|Default|GetType)
        (:NewEnumerator0
          (Transformation|SetRelativeRotation (Variables|/Game/Engineers/Blueprints/Children/BP_RotatorPuzzle_Cryo.BP_RotatorPuzzle_Cryo_C|GetRedAnchor _rotatorpuzzle) (Math|Rotator|MakeRotator (Math|Float|MapRangeClamped (/ _distance (Math|Conversions|ToFloat(Integer) (- (Spline|GetNumberOfSplinePoints _path) 1))) 0.0 1.0 0.0 2.7e+02) 0.0 0.0) false false))
        (:NewEnumerator1
          (Transformation|SetRelativeRotation (Variables|/Game/Engineers/Blueprints/Children/BP_RotatorPuzzle_Cryo.BP_RotatorPuzzle_Cryo_C|GetBlueAnchor _rotatorpuzzle) (Math|Rotator|MakeRotator (Math|Float|MapRangeClamped (/ _distance (Math|Conversions|ToFloat(Integer) (- (Spline|GetNumberOfSplinePoints _path) 1))) 0.0 1.0 0.0 2.7e+02) 0.0 0.0) false false))
        (:NewEnumerator2
          (Transformation|SetRelativeRotation (Variables|/Game/Engineers/Blueprints/Children/BP_RotatorPuzzle_Cryo.BP_RotatorPuzzle_Cryo_C|GetPurpleAnchor _rotatorpuzzle) (Math|Rotator|MakeRotator (Math|Float|MapRangeClamped (/ _distance (Math|Conversions|ToFloat(Integer) (- (Spline|GetNumberOfSplinePoints _path) 1))) 0.0 1.0 0.0 2.7e+02) 0.0 0.0) false false))))))

(event Collision|EventActorBeginOverlap
  (params (OtherActor :type Actor%20Object%20Reference))
  (bind _type (Variables|Default|GetType))
  (bind _asbp_magnet_key (Utilities|Casting|CastToBP_MagnetKey OtherActor))
  (if (Math|Boolean|ORBoolean (and (Utilities|Enum|Equal(Enum) (Variables|/Game/Engineers/Blueprints/Parents/BP_MagnetKey.BP_MagnetKey_C|GetHand _asbp_magnet_key) "Left") (Utilities|Enum|Equal(Enum) _type "NewEnumerator0")) (Utilities|Enum|Equal(Enum) _type "NewEnumerator2") (and (Utilities|Enum|Equal(Enum) _type "NewEnumerator1") (Utilities|Enum|Equal(Enum) (Variables|/Game/Engineers/Blueprints/Parents/BP_MagnetKey.BP_MagnetKey_C|GetHand _asbp_magnet_key) "Right")))
    (if (not (Utilities|IsValid (Variables|Default|GetmagnetKey)))
      (Variables|Default|SetisInteractingWithMagnetKey true)
      (bind _output_get (Variables|Default|SetmagnetKey _asbp_magnet_key))
      (EventDispatchers|BindEventtoTurnedOff _output_get (delegate Custom|SnapAndCheckSolved))
      (Variables|/Game/Engineers/Blueprints/Parents/BP_MagnetKey.BP_MagnetKey_C|SetIsInteractingWithSomething _asbp_magnet_key true)
      (Default|TurnOffLight _asbp_magnet_key))))

(event Collision|EventActorEndOverlap
  (params (OtherActor :type Actor%20Object%20Reference))
  (bind _asbp_magnet_key (Utilities|Casting|CastToBP_MagnetKey OtherActor))
  (if (== _asbp_magnet_key (Variables|Default|GetmagnetKey))
    (if (not (Variables|/Game/Engineers/Blueprints/Parents/BP_MagnetKey.BP_MagnetKey_C|GetisOn _asbp_magnet_key))
      (Variables|Default|SetisInteractingWithMagnetKey false)
      (Variables|/Game/Engineers/Blueprints/Parents/BP_MagnetKey.BP_MagnetKey_C|SetIsInteractingWithSomething _asbp_magnet_key false)
      (EventDispatchers|UnbindEventfromTurnedOff _asbp_magnet_key (delegate Custom|SnapAndCheckSolved))
      (Variables|Default|SetmagnetKey 0))))

(fn ConstructionScript
  (bind _path (Variables|Default|GetPath))
  (for _index (range 0 (- (Spline|GetNumberOfSplinePoints (Variables|Default|GetPath)) 2))
    (bind _returnvalue (AddComponent|AddSplineMeshComponent false))
    (Components|StaticMesh|SetStaticMesh _returnvalue (Variables|Default|GetpathMesh))
    (SplineMesh|SetForwardAxis _returnvalue (Variables|Default|GetForward%20Axis) true)
    (Transformation|AttachComponentToComponent _returnvalue (Variables|Default|GetPath) "None" "KeepRelative" "KeepRelative" "KeepRelative" true)
    (SplineMesh|SetStartandEnd _returnvalue (Spline|GetLocationatSplinePoint _path _index "Local") (Spline|GetTangentatSplinePoint _path _index "Local") (Spline|GetLocationatSplinePoint _path (+ _index 1) "Local") (Spline|GetTangentatSplinePoint _path (+ _index 1) "Local") true :!class /Script/Engine.SplineMeshComponent)))

(fn FindDistanceAlongSpline
  (params (Spline :type Spline%20Component%20Object%20Reference) (Location :type Vector))
  (return (Class|SplineComponent|FindInputKeyClosesttoWorldLocation Spline Location)))

(fn FindNearestThird
  (params (Input :type Float%20%28single-precision%29))
  (LocalVariables|SetCurrentMinValue 1e+03)
  (for _index (range 0 3)
    (if (< (Math|Float|Absolute(Float) (- (/ (Math|Conversions|ToFloat(Integer) _index) 3.0) Input)) (LocalVariables|GetCurrentMinValue))
      (LocalVariables|SetCurrentMinValue (Math|Float|Absolute(Float) (- (/ (Math|Conversions|ToFloat(Integer) _index) 3.0) Input)))
      (LocalVariables|SetCurrentOutput (/ (Math|Conversions|ToFloat(Integer) _index) 3.0))))
  (return (LocalVariables|GetCurrentOutput)))

(fn CheckSolved
  (bind _rotatorpuzzle (Variables|Default|GetRotatorPuzzle))
  (bind _currentvalues (Variables|/Game/Engineers/Blueprints/Children/BP_RotatorPuzzle_Cryo.BP_RotatorPuzzle_Cryo_C|GetCurrentValues _rotatorpuzzle))
  (bind _winningvalues (Variables|/Game/Engineers/Blueprints/Children/BP_RotatorPuzzle_Cryo.BP_RotatorPuzzle_Cryo_C|GetWinningValues _rotatorpuzzle))
  (for _index (range 0 2)
    (switch int _index
      (:0
        (if (!= (.Value (Utilities|Map|Find _currentvalues "Blue")) (.Value (Utilities|Map|Find _winningvalues "Blue")))
          (return false)))
      (:1
        (if (!= (.Value (Utilities|Map|Find _currentvalues "Red")) (.Value (Utilities|Map|Find _winningvalues "Red")))
          (return false)))
      (:2
        (if (!= (.Value (Utilities|Map|Find _currentvalues "Purple")) (.Value (Utilities|Map|Find _winningvalues "Purple")))
          (return false)))))
  (return true))