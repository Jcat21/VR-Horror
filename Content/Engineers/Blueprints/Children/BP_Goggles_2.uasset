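; VR goggles actor that descends to the player's height once the PowerButton_0 power button fires, then carries the player to another area.
; StartMoving disables input and plays a timed startup and voice sequence before Tick lowers the actor and re-enables its trigger box.
; Overlapping the box once eases the pawn into position by timeline, fades the camera, teleports it to the PCMArea spawn and turns walking off.
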(event OnComponentBeginOverlap(Box)
  (params (OverlappedComponent :type Primitive%20Component%20Object%20Reference) (OtherActor :type Actor%20Object%20Reference) (OtherComp :type Primitive%20Component%20Object%20Reference) (OtherBodyIndex :type Integer) (bFromSweep :type Boolean) (SweepResult :type Hit%20Result%20Structure%20%28by%20ref%29))
  (bind _returnvalue (Game|GetPlayerCameraManager 0))
  (bind _returnvalue_2 (Game|Player|GetPlayerPawn 0))
  (bind _returnvalue_3 (Game|Player|GetPlayerPawn 0))
  (bind _scene (Variables|Default|GetScene))
  (bind _returnvalue_4 (Transformation|GetWorldLocation _scene))
  (bind _returnvalue_5 (Transformation|GetActorLocation _returnvalue_2))
  (bind _asvrpawn (Utilities|Casting|CastToVRPawn OtherActor))
  (Utilities|FlowControl|DoOnce false
    (:Completed
      (Input|DisableInput _asvrpawn (Game|GetPlayerController 0))
      (bind _alpha (Timeline|Timeline_0 PlayFromStart)
        (:Update
          (Transformation|SetActorLocationAndRotation (Game|Player|GetPlayerPawn 0) (Math|Vector|Lerp(Vector) _returnvalue_5 (Math|Vector|MakeVector (.x _returnvalue_4) (.y _returnvalue_4) (.Z (Math|Vector|BreakVector _returnvalue_5))) _alpha) (Math|Rotator|Lerp(Rotator) (Transformation|GetActorRotation (Game|Player|GetPlayerPawn 0)) (Transformation|GetWorldRotation (Variables|Default|GetArrow)) _alpha) false true))
        (:Finished
          (CameraFades|StartCameraFade :self _returnvalue :ToAlpha 1.0 :Duration (Variables|Default|GetCameraFadeTime) :bHoldWhenFinished true)
          (Utilities|FlowControl|Delay (Variables|Default|GetCameraFadeTime))
          (bind _outactors (Actor|GetAllActorsOfClass "/Game/Engineers/Blueprints/Misc/BP_Spawn.BP_Spawn_C"))
          (for _array_element _outactors
            (if (Utilities|Enum|Equal(Enum) (Variables|/Game/Engineers/Blueprints/Misc/BP_Spawn.BP_Spawn_C|GetName _array_element) "PCMArea")
              (Transformation|SetActorLocation _returnvalue_3 (Math|Vector|MakeVector (.x (Transformation|GetActorLocation _array_element)) (.y (Transformation|GetActorLocation _array_element)) (.z (Transformation|GetActorLocation _returnvalue_3))) false true)
              (CameraFades|StopCameraFade _returnvalue)
              (Input|EnableInput _returnvalue_3 (Game|GetPlayerController 0))
              (bind _asvrpawn_2 (Utilities|Casting|CastToVRPawn (Game|Player|GetPlayerPawn 0)))
              (Variables|/Game/Engineers/Blueprints/Parents/VRPawn.VRPawn_C|SetCanWalk _asvrpawn_2 false))))))))

(event Custom|StartMoving
  (bind _returnvalue (Transformation|GetActorLocation))
  (Variables|Default|SetHeightFromGround (- (.z (Transformation|GetActorLocation (Game|Player|GetPlayerPawn 0))) 215.0))
  (Input|DisableInput (Game|Player|GetPlayerPawn 0) (Game|GetPlayerController 0))
  (Audio|PlaySoundatLocation "/Game/Artists/Audio/Sounds/Whirring_Computer_Startup.Whirring_Computer_Startup" "0, 0, 0")
  (Utilities|FlowControl|Delay 2.0)
  (Audio|PlaySound2D "/Game/Artists/Audio/Sounds/Whirring_Computer_Loop.Whirring_Computer_Loop" 1.0 1.0 0.0 0 (Game|Player|GetPlayerPawn 0))
  (Audio|PlaySoundatLocation "/Game/Artists/Audio/Sounds/Percy_5sec.Percy_5sec" "0, 0, 0")
  (Utilities|FlowControl|Delay 2.0)
  (Audio|PlaySoundatLocation "/Game/Artists/Audio/Sounds/AI_Power_Restored.AI_Power_Restored" _returnvalue "0, 0, 0" 0.55)
  (Utilities|FlowControl|Delay 15.75)
  (Variables|Default|SetShouldMove true)
  (Audio|PlaySoundatLocation "/Game/Artists/Audio/Sounds/Goggle_Hydraulics_Descending.Goggle_Hydraulics_Descending" _returnvalue "0, 0, 0" 0.55)
  (Utilities|FlowControl|Delay 5.0)
  (Audio|PlaySoundatLocation 0 (Transformation|GetActorLocation (Game|Player|GetPlayerPawn 0))))

(event EventTick
  (params (DeltaSeconds :type Float%20%28single-precision%29))
  (if (Variables|Default|GetShouldMove)
    (if (Variables|Default|GetIsDown)
      (Transformation|AddActorLocalOffset (Math|Vector|MakeVector 0.0 0.0 0.5) false true)
      (if (>= (.Z (Math|Vector|BreakVector (Transformation|GetActorLocation))) (Variables|Default|GetinitialHeight))
        (Variables|Default|SetIsDown false)
        (Variables|Default|SetShouldMove false :!label _label)
        (Collision|SetCollisionEnabled (Variables|Default|GetBox) "QueryOnly"))
      (else
        (Transformation|AddActorLocalOffset (Math|Vector|MakeVector 0.0 0.0 -0.5) false true)
        (if (<= (.Z (Math|Vector|BreakVector (Transformation|GetActorLocation))) (Variables|Default|GetHeightFromGround))
          (Variables|Default|SetIsDown true)
          (goto _label))))))

(event EventBeginPlay
  (bind _outactors (Actor|GetAllActorsOfClass "/Game/Engineers/Blueprints/Children/BP_Button_Power.BP_Button_Power_C"))
  (for _array_element _outactors
    (if (Utilities|Enum|Equal(Enum) (Variables|/Game/Engineers/Blueprints/Children/BP_Button_Power.BP_Button_Power_C|GetButtonID _array_element) "PowerButton_0")
      (EventDispatchers|BindEventtoTrigger _array_element (delegate Custom|StartMoving))
      (Collision|SetCollisionEnabled (Variables|Default|GetBox) "NoCollision")
      (Variables|Default|SetinitialHeight (.z (Transformation|GetActorLocation))))))

(fn ConstructionScript)