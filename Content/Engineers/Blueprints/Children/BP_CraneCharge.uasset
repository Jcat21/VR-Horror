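; Crane charge station where holding both active hand magnet keys on the red and blue pads adds play time to the crane's timer.
; While both overlap, Tick raises the time, updates the control station text, brightens the skylight, plays audio and pulses haptics.
; Uncovered pads pulse emission through a timeline on dynamic materials.
; At full charge it locks, notifies listeners, disables magnet key lighting and starts CryopodDeath.
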(event OnComponentEndOverlap(RedSide)
  (params (OverlappedComponent :type Primitive%20Component%20Object%20Reference) (OtherActor :type Actor%20Object%20Reference) (OtherComp :type Primitive%20Component%20Object%20Reference) (OtherBodyIndex :type Integer))
  ;[1 1 1] Left Charge Button (End Overlap)
  (bind _asbp_magnet_key (Utilities|Casting|CastToBP_MagnetKey OtherActor))
  (if (Utilities|Enum|Equal(Enum) (Variables|/Game/Engineers/Blueprints/Parents/BP_MagnetKey.BP_MagnetKey_C|GetHand _asbp_magnet_key) "Left")
    (Variables|Default|SetLeftHand 0)
    (Audio|Components|Audio|FadeOut (Variables|Default|GetAudio) 0.2 0.0 :!class /Script/Engine.AudioComponent)))

(event OnComponentBeginOverlap(RedSide)
  (params (OverlappedComponent :type Primitive%20Component%20Object%20Reference) (OtherActor :type Actor%20Object%20Reference) (OtherComp :type Primitive%20Component%20Object%20Reference) (OtherBodyIndex :type Integer) (bFromSweep :type Boolean) (SweepResult :type Hit%20Result%20Structure%20%28by%20ref%29))
  ;[1 1 1] Left Charge Button (Begin Overlap)
  (bind _asbp_magnet_key (Utilities|Casting|CastToBP_MagnetKey OtherActor))
  (if (Utilities|Enum|Equal(Enum) (Variables|/Game/Engineers/Blueprints/Parents/BP_MagnetKey.BP_MagnetKey_C|GetHand _asbp_magnet_key) "Left")
    (Variables|Default|SetLeftHand _asbp_magnet_key)
    (if (Variables|Default|GetCanTransferPowerToTimer)
      (Rendering|Material|SetScalarParameterValue (Variables|Default|GetRedChargeMaterial) "Emission" 5e+01 :!class /Script/Engine.MaterialInstanceDynamic))))

(event OnComponentEndOverlap(BlueSide)
  (params (OverlappedComponent :type Primitive%20Component%20Object%20Reference) (OtherActor :type Actor%20Object%20Reference) (OtherComp :type Primitive%20Component%20Object%20Reference) (OtherBodyIndex :type Integer))
  ;[1 1 1] Right Charge Button (End Overlap)
  (bind _asbp_magnet_key (Utilities|Casting|CastToBP_MagnetKey OtherActor))
  (if (Utilities|Enum|Equal(Enum) (Variables|/Game/Engineers/Blueprints/Parents/BP_MagnetKey.BP_MagnetKey_C|GetHand _asbp_magnet_key) "Right")
    (Variables|Default|SetRightHand 0)
    (Audio|Components|Audio|FadeOut (Variables|Default|GetAudio) 0.2 0.0 :!class /Script/Engine.AudioComponent)))

(event OnComponentBeginOverlap(BlueSide)
  (params (OverlappedComponent :type Primitive%20Component%20Object%20Reference) (OtherActor :type Actor%20Object%20Reference) (OtherComp :type Primitive%20Component%20Object%20Reference) (OtherBodyIndex :type Integer) (bFromSweep :type Boolean) (SweepResult :type Hit%20Result%20Structure%20%28by%20ref%29))
  ;[1 1 1] Right Charge Button (Begin Overlap)
  (bind _asbp_magnet_key (Utilities|Casting|CastToBP_MagnetKey OtherActor))
  (if (Utilities|Enum|Equal(Enum) (Variables|/Game/Engineers/Blueprints/Parents/BP_MagnetKey.BP_MagnetKey_C|GetHand _asbp_magnet_key) "Right")
    (Variables|Default|SetRightHand _asbp_magnet_key)
    (if (Variables|Default|GetCanTransferPowerToTimer)
      (Rendering|Material|SetScalarParameterValue (Variables|Default|GetBlueChargeMaterial) "Emission" 5e+01 :!class /Script/Engine.MaterialInstanceDynamic))))

(event Custom|PulseChargeLights
  (bind _cantransferpowertotimer (Variables|Default|GetCanTransferPowerToTimer))
  (Utilities|FlowControl|FlipFlop :!label _label
    (:A
      (if _cantransferpowertotimer
        (bind _emission (Timeline|Timeline_0 PlayFromStart)
          (:Update
            (Utilities|FlowControl|Sequence
              (:then_0
                (if (not (Utilities|IsValid (Variables|Default|GetLeftHand)))
                  (Rendering|Material|SetScalarParameterValue (Variables|Default|GetRedChargeMaterial) "Emission" _emission :!class /Script/Engine.MaterialInstanceDynamic)))
              (:then_1
                (if (not (Utilities|IsValid (Variables|Default|GetRightHand)))
                  (Rendering|Material|SetScalarParameterValue (Variables|Default|GetBlueChargeMaterial) "Emission" _emission :!class /Script/Engine.MaterialInstanceDynamic)))))
          (:Finished
            (goto _label)))))
    (:B
      (if _cantransferpowertotimer
        (Timeline|Timeline_0 ReverseFromEnd)))))

(event EventTick
  (params (DeltaSeconds :type Float%20%28single-precision%29))
  (bind _returnvalue (Game|GetPlayerController 0))
  (bind _lefthand (Variables|Default|GetLeftHand))
  (bind _righthand (Variables|Default|GetRightHand))
  (bind _lefthand_2 (Variables|Default|GetLeftHand))
  (bind _righthand_2 (Variables|Default|GetRightHand))
  (bind _audio (Variables|Default|GetAudio))
  (bind _crane (Variables|Default|GetCrane))
  (bind _timetoplay (Variables|/Game/Engineers/Blueprints/Misc/BP_Crane.BP_Crane_C|GetTimeToPlay _crane))
  (bind _returnvalue_2 (Math|Conversions|ToFloat(Integer) _timetoplay))
  (if (Variables|Default|GetCanTransferPowerToTimer)
    (Utilities|FlowControl|Sequence
      (:then_0
        (if (and (Utilities|IsValid _lefthand_2) (Utilities|IsValid _righthand_2))
          (if (and (Variables|/Game/Engineers/Blueprints/Parents/BP_MagnetKey.BP_MagnetKey_C|GetisOn _lefthand_2) (Variables|/Game/Engineers/Blueprints/Parents/BP_MagnetKey.BP_MagnetKey_C|GetisOn _righthand_2))
            ;[1 1 1] Add Time to Playable Time
            (if (< (Variables|Default|GetCurrentTime) (Math|Conversions|ToFloat(Integer) _timetoplay))
              (if (Audio|Components|Audio|IsPlaying _audio)
                _
                (else
                  (Audio|Components|Audio|FadeIn _audio 0.2 1.0 0.0 :!class /Script/Engine.AudioComponent)))
              (bind _output_get (Variables|Default|SetCurrentTime (+ (Variables|Default|GetCurrentTime) (Variables|Default|GetTransferRate))))
              (Rendering|Components|TextRender|SetText (Variables|/Game/Engineers/Blueprints/Parents/BP_ControlStation.BP_ControlStation_C|GetTimer (Variables|Default|GetControlStation)) (Utilities|Text|ToText(Float) (Math|Float|Clamp(Float) _output_get 0.0 _returnvalue_2) "HalfToEven"))
              (Rendering|Components|Light|SetIntensity (Variables|/Script/Engine.SkyLight|GetLightComponent (Variables|Default|GetSkyLight)) (Math|Float|MapRangeClamped (Math|Float|Clamp(Float) _output_get 0.0 _returnvalue_2) 0.0 _returnvalue_2 0.0 1.0))
              (else
                (Variables|Default|SetCanTransferPowerToTimer false)
                (Rendering|Material|SetScalarParameterValue (Variables|Default|GetBlueChargeMaterial) "Emission" 1.0 :!class /Script/Engine.MaterialInstanceDynamic)
                (Default|CallHitFullCharge)
                (bind _outactors (Actor|GetAllActorsOfClass "/Game/Engineers/Blueprints/Parents/BP_MagnetKey.BP_MagnetKey_C"))
                (for _array_element _outactors
                  (Variables|/Game/Engineers/Blueprints/Parents/BP_MagnetKey.BP_MagnetKey_C|SetisUsingLighting _array_element false))
                (Audio|Components|Audio|FadeOut (Variables|Default|GetAudio) 0.5 0.0 :!class /Script/Engine.AudioComponent)
                (Audio|Components|Audio|Play (Variables|Default|GetCryopod_Death) 0.0))))))
      (:then_1
        (if (Utilities|IsValid _lefthand)
          (if (Variables|/Game/Engineers/Blueprints/Parents/BP_MagnetKey.BP_MagnetKey_C|GetisOn _lefthand)
            (Class|PlayerController|PlayHapticEffect _returnvalue "/Game/Misc/HapticEvents/Grab.Grab" "Left" 1.0 false))))
      (:then_2
        (if (Utilities|IsValid _righthand)
          (if (Variables|/Game/Engineers/Blueprints/Parents/BP_MagnetKey.BP_MagnetKey_C|GetisOn _righthand)
            (Class|PlayerController|PlayHapticEffect _returnvalue "/Game/Misc/HapticEvents/Grab.Grab" "Right" 1.0 false)))))))

(event EventBeginPlay
  (CallFunction|PulseChargeLights)
  (bind _outactors (Actor|GetAllActorsOfClass "/Script/Engine.SkyLight")))

(fn ConstructionScript
  (bind _returnvalue (Rendering|Material|CreateDynamicMaterialInstance (Variables|Default|GetBlueSide) 0 "/Game/Artists/Materials/M_RightMagnetKeyTurnedON.M_RightMagnetKeyTurnedON" :!class /Script/Engine.PrimitiveComponent))
  (Variables|Default|SetBlueChargeMaterial _returnvalue)
  (bind _returnvalue_2 (Rendering|Material|CreateDynamicMaterialInstance (Variables|Default|GetRedSide) 0 "/Game/Artists/Materials/M_LeftMagnetKeyTurnedON.M_LeftMagnetKeyTurnedON" :!class /Script/Engine.PrimitiveComponent))
  (Variables|Default|SetRedChargeMaterial _returnvalue_2))