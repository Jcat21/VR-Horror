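; Cryo charge station puzzle that the player powers by holding both switched-on magnet keys on it, left on red, right on blue.
; Side overlaps track each hand's key, and Tick adds power while both are on, driving percent text, material emission, lights, indicators, audio and haptics.
; At full charge it fires HitFullCharge, reveals the rotator's reference puzzle and plays the NOAH intro matinee with timed AI voice lines.
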(event OnComponentBeginOverlap(Box)
  (params (OverlappedComponent :type Primitive%20Component%20Object%20Reference) (OtherActor :type Actor%20Object%20Reference) (OtherComp :type Primitive%20Component%20Object%20Reference) (OtherBodyIndex :type Integer) (bFromSweep :type Boolean) (SweepResult :type Hit%20Result%20Structure%20%28by%20ref%29))
  ;[1 1 1] If in control room InControlRoom == True
)

(event OnComponentEndOverlap(Box)
  (params (OverlappedComponent :type Primitive%20Component%20Object%20Reference) (OtherActor :type Actor%20Object%20Reference) (OtherComp :type Primitive%20Component%20Object%20Reference) (OtherBodyIndex :type Integer))
  ;[1 1 1] If in control room InControlRoom == True
)

(event OnComponentEndOverlap(RedSide)
  (params (OverlappedComponent :type Primitive%20Component%20Object%20Reference) (OtherActor :type Actor%20Object%20Reference) (OtherComp :type Primitive%20Component%20Object%20Reference) (OtherBodyIndex :type Integer))
  ;[1 1 1] Left Charge Button (End Overlap)
  (bind _asbp_magnet_key (Utilities|Casting|CastToBP_MagnetKey OtherActor))
  (if (Utilities|Enum|Equal(Enum) (Variables|/Game/Engineers/Blueprints/Parents/BP_MagnetKey.BP_MagnetKey_C|GetHand _asbp_magnet_key) "Left")
    (Variables|Default|SetLeftHand 0)
    (Audio|Components|Audio|FadeOut (Variables|Default|GetChargeAudio) 0.2 0.0 :!class /Script/Engine.AudioComponent)))

(event OnComponentBeginOverlap(RedSide)
  (params (OverlappedComponent :type Primitive%20Component%20Object%20Reference) (OtherActor :type Actor%20Object%20Reference) (OtherComp :type Primitive%20Component%20Object%20Reference) (OtherBodyIndex :type Integer) (bFromSweep :type Boolean) (SweepResult :type Hit%20Result%20Structure%20%28by%20ref%29))
  ;[1 1 1] Left Charge Button (Begin Overlap)
  (bind _asbp_magnet_key (Utilities|Casting|CastToBP_MagnetKey OtherActor))
  (if (Utilities|Enum|Equal(Enum) (Variables|/Game/Engineers/Blueprints/Parents/BP_MagnetKey.BP_MagnetKey_C|GetHand _asbp_magnet_key) "Left")
    (Variables|Default|SetLeftHand _asbp_magnet_key)))

(event OnComponentEndOverlap(BlueSide)
  (params (OverlappedComponent :type Primitive%20Component%20Object%20Reference) (OtherActor :type Actor%20Object%20Reference) (OtherComp :type Primitive%20Component%20Object%20Reference) (OtherBodyIndex :type Integer))
  ;[1 1 1] Right Charge Button (End Overlap)
  (bind _asbp_magnet_key (Utilities|Casting|CastToBP_MagnetKey OtherActor))
  (if (Utilities|Enum|Equal(Enum) (Variables|/Game/Engineers/Blueprints/Parents/BP_MagnetKey.BP_MagnetKey_C|GetHand _asbp_magnet_key) "Right")
    (Variables|Default|SetRightHand 0)
    (Audio|Components|Audio|FadeOut (Variables|Default|GetChargeAudio) 0.2 0.0 :!class /Script/Engine.AudioComponent)))

(event OnComponentBeginOverlap(BlueSide)
  (params (OverlappedComponent :type Primitive%20Component%20Object%20Reference) (OtherActor :type Actor%20Object%20Reference) (OtherComp :type Primitive%20Component%20Object%20Reference) (OtherBodyIndex :type Integer) (bFromSweep :type Boolean) (SweepResult :type Hit%20Result%20Structure%20%28by%20ref%29))
  ;[1 1 1] Right Charge Button (Begin Overlap)
  (bind _asbp_magnet_key (Utilities|Casting|CastToBP_MagnetKey OtherActor))
  (if (Utilities|Enum|Equal(Enum) (Variables|/Game/Engineers/Blueprints/Parents/BP_MagnetKey.BP_MagnetKey_C|GetHand _asbp_magnet_key) "Right")
    (Variables|Default|SetRightHand _asbp_magnet_key)))

(event OnActorBeginOverlap(SteppedOut)
  (params (OverlappedActor :type Actor%20Object%20Reference) (OtherActor :type Actor%20Object%20Reference))
  ;[1 1 1] If in control room InControlRoom == True
  (Variables|Default|SetOutControlRoom true))

(event Custom|PulseChargeLights
  (bind _cantransferpower (Variables|Default|GetCanTransferPower))
  (Utilities|FlowControl|FlipFlop :!label _label
    (:A
      (if _cantransferpower
        (bind _emission (Timeline|Timeline_0 PlayFromStart)
          (:Update
            (Utilities|FlowControl|Sequence
              (:then_0
                (if (not (Utilities|IsValid (Variables|Default|GetLeftHand)))
                  (Rendering|Material|SetScalarParameterValue (Variables|Default|GetRedChargeMaterial) "Emission" _emission :!class /Script/Engine.MaterialInstanceDynamic)))
              (:then_1
                (if (not (Utilities|IsValid (Variables|Default|GetRightHand)))
                  (Rendering|Material|SetScalarParameterValue (Variables|Default|GetBlueChargeMaterial) "Emission" _emission :!class /Script/Engine.MaterialInstanceDynamic)))))
          (:Finished
            (goto _label)))))
    (:B
      (if _cantransferpower
        (Timeline|Timeline_0 ReverseFromEnd)))))

(event EventTick
  (params (DeltaSeconds :type Float%20%28single-precision%29))
  (bind _returnvalue (Game|GetPlayerController 0))
  (bind _chargeaudio (Variables|Default|GetChargeAudio))
  (bind _lefthand (Variables|Default|GetLeftHand))
  (bind _lefthand_2 (Variables|Default|GetLeftHand))
  (bind _righthand (Variables|Default|GetRightHand))
  (bind _maxpower (Variables|Default|GetMaxPower))
  (bind _righthand_2 (Variables|Default|GetRightHand))
  (if (Variables|Default|GetCanTransferPower)
    (Utilities|FlowControl|Sequence
      (:then_0
        (if (and (Utilities|IsValid _lefthand_2) (Utilities|IsValid _righthand))
          (if (and (Variables|/Game/Engineers/Blueprints/Parents/BP_MagnetKey.BP_MagnetKey_C|GetisOn _lefthand_2) (Variables|/Game/Engineers/Blueprints/Parents/BP_MagnetKey.BP_MagnetKey_C|GetisOn _righthand))
            ;[1 1 1] Charge
            (if (< (Variables|Default|GetCurrentPower) (Variables|Default|GetMaxPower))
              (if (Audio|Components|Audio|IsPlaying _chargeaudio)
                _
                (else
                  (Audio|Components|Audio|FadeIn _chargeaudio 0.2 1.0 0.0 :!class /Script/Engine.AudioComponent)))
              (bind _output_get (Variables|Default|SetCurrentPower (+ (Variables|Default|GetCurrentPower) (Variables|Default|GetTransferRate))))
              (bind _string (CallFunction|RoundFloat (Math|Float|Clamp(Float) _output_get 0.0 _maxpower)))
              (Rendering|Components|TextRender|SetText (Variables|Default|GetTextRender) (Utilities|Text|ToText(String) _string))
              (Rendering|Material|SetScalarParameterValue (Variables|Default|GetBlueChargeMaterial) "Emission" (Math|Float|Clamp(Float) _output_get 0.0 _maxpower) :!class /Script/Engine.MaterialInstanceDynamic)
              (for _array_element (Variables|Default|GetPointLights)
                (Rendering|Components|Light|SetIntensity (Variables|/Script/Engine.Light|GetLightComponent _array_element) (Math|Float|MapRangeClamped (Math|Float|Clamp(Float) _output_get 0.0 _maxpower) 0.0 _maxpower 0.0 1.0))
                (if (>= (- (/ (Math|Float|Truncate (Variables|Default|GetCurrentPower)) 10) 1) 0)
                  (if (Utilities|Enum|Equal(Enum) (Utilities|GetObjectName (Rendering|Material|GetMaterial (Variables|/Script/Engine.StaticMeshActor|GetStaticMeshComponent (Utilities|Array|Get(acopy) (Variables|Default|GetIndicators) (- (/ (Math|Float|Truncate (Variables|Default|GetCurrentPower)) 10) 1))) 0)) "PowwerUpLightOff")
                    (Rendering|Material|SetMaterial (Variables|/Script/Engine.StaticMeshActor|GetStaticMeshComponent (Utilities|Array|Get(acopy) (Variables|Default|GetIndicators) (- (/ (Math|Float|Truncate (Variables|Default|GetCurrentPower)) 10) 1))) 0 "/Game/Artists/Materials/PowerUpLightOn.PowerUpLightOn"))))
              (else
                (Variables|Default|SetCanTransferPower false)
                (Default|CallHitFullCharge)
                (Default|ShowReferencePuzzle (Variables|Default|GetRotatorPuzzle))
                (Audio|Components|Audio|Stop (Variables|Default|GetAudio))
                (Audio|Components|Audio|FadeOut (Variables|Default|GetChargeAudio) 0.2 0.0 :!class /Script/Engine.AudioComponent)
                ;[1 1 1] AI computer Dialog & end Logic
                (Utilities|FlowControl|Delay 2.0)
                (Audio|Components|Audio|Play (Variables|Default|GetNOAHintroMatinee))
                (Audio|PlaySoundatLocation "/Game/Artists/Audio/Sounds/DX/Line_1_V3.Line_1_V3" "3236.899902,-320.000000,371.649994")
                (Utilities|FlowControl|Delay 6.5)
                (Audio|Components|Audio|FadeIn (Variables|Default|GetWhirringComputer) 2.0 0.6 0.0 :!class /Script/Engine.AudioComponent)
                (Utilities|FlowControl|Delay 2.0)
                (Audio|PlaySoundatLocation "/Game/Artists/Audio/Sounds/DX/Line_2.Line_2" "3236.899902,-320.000000,371.649994")
                (Utilities|FlowControl|Delay 25.0)
                (Audio|PlaySoundatLocation (Variables|Default|GetDoorPuzzleDirections) "3236.899902,-320.000000,371.649994")
                (if (Variables|Default|GetOutControlRoom)
                  (Audio|Components|Audio|AdjustVolume (Variables|Default|GetAudio) 0.0 0.0 :!class /Script/Engine.AudioComponent)))))))
      (:then_1
        (if (Utilities|IsValid _righthand_2)
          (if (Variables|/Game/Engineers/Blueprints/Parents/BP_MagnetKey.BP_MagnetKey_C|GetisOn _righthand_2)
            (Class|PlayerController|PlayHapticEffect _returnvalue "/Game/Misc/HapticEvents/Grab.Grab" "Right" 1.0 false)))
        (if (Utilities|IsValid _lefthand)
          (if (Variables|/Game/Engineers/Blueprints/Parents/BP_MagnetKey.BP_MagnetKey_C|GetisOn _lefthand)
            (Class|PlayerController|PlayHapticEffect _returnvalue "/Game/Misc/HapticEvents/Grab.Grab" "Left" 1.0 false)))))))

(event EventBeginPlay)

(fn ConstructionScript
  (bind _returnvalue (Rendering|Material|CreateDynamicMaterialInstance (Variables|Default|GetBlueSide) 0 "/Game/Artists/Materials/M_RightMagnetKeyTurnedON.M_RightMagnetKeyTurnedON" :!class /Script/Engine.PrimitiveComponent))
  (Variables|Default|SetBlueChargeMaterial _returnvalue)
  (bind _returnvalue_2 (Rendering|Material|CreateDynamicMaterialInstance (Variables|Default|GetRedSide) 0 "/Game/Artists/Materials/M_LeftMagnetKeyTurnedON.M_LeftMagnetKeyTurnedON" :!class /Script/Engine.PrimitiveComponent))
  (Variables|Default|SetRedChargeMaterial _returnvalue_2)
  (Rendering|Material|SetScalarParameterValue (Variables|Default|GetRedChargeMaterial) "Emission" 1.0 :!class /Script/Engine.MaterialInstanceDynamic))

(fn RoundFloat
  (params (Float :type Float%20%28single-precision%29))
  (return (Utilities|String|Append (Utilities|String|ToString(Integer) (Math|Float|Floor Float)) "%")))