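; Cryo variant of the rotator puzzle that opens a sliding double door and can reveal its red, blue and purple reference puzzle.
; BeginPlay caches up to three slider rail rotators from the level.
; OpenDoor plays audio once, then uses a Delay loop to slide the doors, anchors, puzzle pieces and rails apart for a fixed step count, so speed is frame-dependent.
; Material tinting logic for the anchors is left unconnected.
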(event Custom|ShowReferencePuzzle
  (Rendering|SetVisibility (Variables|Default|GetReferencePurple) true false))

(event Custom|OpenDoor
  (bind _doorspeed (Variables|Default|GetDoorSpeed))
  (bind _counter (Variables|Default|GetCounter))
  (bind _returnvalue (* _doorspeed -1.0))
  (if (not (Variables|Default|GetisOpen))
    (Variables|Default|SetisOpen true)
    (Audio|Components|Audio|Play (Variables|Default|GetAudio) 0.0)
    (if (Variables|Default|GetDoorsCanMove) :!label _label
      (Transformation|AddWorldOffset (Variables|Default|GetReferenceAnchor) (Math|Vector|MakeVector 0.0 (Variables|Default|GetDoorSpeed) 0.0) false true)
      (Transformation|AddActorWorldOffset (Variables|Default|GetLeftDoor) (Math|Vector|MakeVector 0.0 (Variables|Default|GetDoorSpeed) 0.0) false true)
      (Transformation|AddWorldOffset (Variables|Default|GetRedAnchor) (Math|Vector|MakeVector 0.0 _returnvalue 0.0) false true)
      (Transformation|AddActorWorldOffset (Variables|Default|GetRightDoor) (Math|Vector|MakeVector 0.0 _returnvalue 0.0) false true)
      (Math|Integer|IncrementInt _counter
        (:%20%20
          (if (== _counter 700)
            (Variables|Default|SetDoorsCanMove false))
          (Utilities|FlowControl|Delay (Utilities|Time|GetWorldDeltaSeconds))
          (goto _label)))
      (else
        (Variables|Default|SetDoorsCanMove true)))))

(event EventBeginPlay
  (bind _outactors (Actor|GetAllActorsOfClass "/Game/Engineers/Blueprints/Children/BP_SliderRailRotator.BP_SliderRailRotator_C"))
  (for (_array_element _array_index) _outactors
    (switch int _array_index
      (:0
        (Variables|Default|SetSliderRail1 _array_element))
      (:1
        (Variables|Default|SetSliderRail2 _array_element))
      (:2
        (Variables|Default|SetSliderRail3 _array_element)))))

(fn ConstructionScript)