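; BP_ControlStation_Lab is the lab variant of a control station, with target amounts for red, purple and blue.
; Its construction script converts each color's correct amount to text and writes it to the matching target display, so the displays reflect the configured values.
; The file contains only this display setup, with no runtime events or checks against those amounts.
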(fn ConstructionScript
  (Rendering|Components|TextRender|SetText (Variables|Default|GetTargetAmountRed) (Utilities|Text|ToText(String) (Utilities|String|ToString(Integer) (Variables|Default|GetCorrectAmountRed))))
  (Rendering|Components|TextRender|SetText (Variables|Default|GetTargetAmountPurple) (Utilities|Text|ToText(String) (Utilities|String|ToString(Integer) (Variables|Default|GetCorrectAmountPurple))))
  (Rendering|Components|TextRender|SetText (Variables|Default|GetTargetAmountBlue) (Utilities|Text|ToText(String) (Utilities|String|ToString(Integer) (Variables|Default|GetCorrectAmountBlue)))))