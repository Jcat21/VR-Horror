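; Lab puzzle slider rail where a hand-matched magnet key drags a ball along a spline to set a red, blue or purple chemical amount.
; The construction script builds the rail from spline meshes, and Tick maps the ball's spline position to a percentage on the ControlStation.
; Magnet release or overlap end snaps near-correct values to the target and triggers one-time bubble and matinee effects.
; Chargers activate when all three amounts match.
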(event Custom|SnapAndChangeColor
  (bind _returnvalue (Math|Color|MakeColor 0.0 1.0 0.0))
  (bind _returnvalue_2 (Math|Color|MakeColor 0.0 0.0 0.0))
  (bind _returnvalue_3 (Math|Color|MakeColor 0.0 0.0 0.0))
  (bind _controlstation (Variables|Default|GetControlStation))
  (bind _controlstation_2 (Variables|Default|GetControlStation))
  (bind _controlstation_3 (Variables|Default|GetControlStation))
  (bind _controlstation_4 (Variables|Default|GetControlStation))
  (bind _returnvalue_4 (Math|Conversions|ToColor(LinearColor) _returnvalue))
  (bind _returnvalue_5 (Math|Conversions|ToColor(LinearColor) _returnvalue_2))
  (bind _returnvalue_6 (Math|Conversions|ToColor(LinearColor) _returnvalue_3))
  (bind _correctamountred (Variables|/Game/Engineers/Blueprints/Children/BP_ControlStation_Lab.BP_ControlStation_Lab_C|GetCorrectAmountRed _controlstation_2))
  (bind _correctamountpurple (Variables|/Game/Engineers/Blueprints/Children/BP_ControlStation_Lab.BP_ControlStation_Lab_C|GetCorrectAmountPurple _controlstation_2))
  (bind _correctamountblue (Variables|/Game/Engineers/Blueprints/Children/BP_ControlStation_Lab.BP_ControlStation_Lab_C|GetCorrectAmountBlue _controlstation_2))
  (bind _currentamountred (Variables|/Game/Engineers/Blueprints/Children/BP_ControlStation_Lab.BP_ControlStation_Lab_C|GetCurrentAmountRed _controlstation_3))
  (bind _currentamountblue (Variables|/Game/Engineers/Blueprints/Children/BP_ControlStation_Lab.BP_ControlStation_Lab_C|GetCurrentAmountBlue _controlstation_3))
  (bind _currentamountpurple (Variables|/Game/Engineers/Blueprints/Children/BP_ControlStation_Lab.BP_ControlStation_Lab_C|GetCurrentAmountPurple _controlstation_3))
  (Utilities|FlowControl|Sequence
    (:then_0
      (switch Utilities|FlowControl|Switch|SwitchonSliderRotatorTypes (Variables|Default|GetType)
        (:NewEnumerator0
          ;[1 1 1] Checking to see if Left Hand slider is close to the correct amount
          (if (Math|Integer|InRange(Integer) (Variables|Default|GetCurrentAmount) (- _correctamountred 2) (+ _correctamountred 2))
            (Utilities|FlowControl|Sequence
              (:then_0
                ;[1 1 1] Setting the text color to red or black
                (Rendering|Components|TextRender|SetTextRenderColor _currentamountred _returnvalue_4)
                ;[1 1 1] Changing current amount text render and snapping ball back to position
                (bind _output_get (Variables|Default|SetCurrentAmount (Variables|/Game/Engineers/Blueprints/Children/BP_ControlStation_Lab.BP_ControlStation_Lab_C|GetCorrectAmountRed _controlstation)))
                (CallFunction|SetCurrentAmountText _output_get)
                (CallFunction|SnapBallBack _output_get)
                (Variables|/Game/Engineers/Blueprints/Children/BP_ControlStation_Lab.BP_ControlStation_Lab_C|SetCurAmountRed _controlstation (Variables|Default|GetCurrentAmount) :!label _label))
              (:then_1
                (Utilities|FlowControl|DoOnce false
                  (:Completed
                    (bind _returnvalue_7 (Effects|SpawnEmitteratLocation "/Game/Artists/VFX/P_BubblesPD1.P_BubblesPD1" (Transformation|GetActorLocation (Variables|Default|GetTargetRedBubbles))))
                    (Audio|Components|Audio|Play (Variables|Default|GetMatineeRedChem))
                    (Audio|Components|Audio|Play (Variables|Default|GetDrawChemicals) 0.0)
                    (Utilities|FlowControl|Delay 2.0)
                    (bind _output_get_2 (Variables|Default|SetNewVar_0 _returnvalue_7))
                    (Components|Activation|Deactivate _output_get_2)))))
            (else
              (Rendering|Components|TextRender|SetTextRenderColor _currentamountred _returnvalue_6)
              (goto _label))))
        (:NewEnumerator1
          (if (Math|Integer|InRange(Integer) (Variables|Default|GetCurrentAmount) (- _correctamountblue 2) (+ _correctamountblue 2))
            (Utilities|FlowControl|Sequence
              (:then_0
                (Rendering|Components|TextRender|SetTextRenderColor _currentamountblue _returnvalue_4)
                (bind _output_get_3 (Variables|Default|SetCurrentAmount (Variables|/Game/Engineers/Blueprints/Children/BP_ControlStation_Lab.BP_ControlStation_Lab_C|GetCorrectAmountBlue _controlstation)))
                (CallFunction|SetCurrentAmountText _output_get_3)
                (CallFunction|SnapBallBack _output_get_3)
                (Variables|/Game/Engineers/Blueprints/Children/BP_ControlStation_Lab.BP_ControlStation_Lab_C|SetCurAmountBlue _controlstation (Variables|Default|GetCurrentAmount) :!label _label_2))
              (:then_1
                (Utilities|FlowControl|DoOnce false
                  (:Completed
                    (bind _returnvalue_8 (Effects|SpawnEmitteratLocation "/Game/Artists/VFX/P_BubblesPD1.P_BubblesPD1" (Transformation|GetActorLocation (Variables|Default|GetTargetBlueBubbles))))
                    (Audio|Components|Audio|Play (Variables|Default|GetMatineeBlueChem))
                    (Audio|Components|Audio|Play (Variables|Default|GetDrawChemicals) 0.0)
                    (Utilities|FlowControl|Delay 2.0)
                    (bind _output_get_4 (Variables|Default|SetNewVar_2 _returnvalue_8))
                    (Components|Activation|Deactivate _output_get_4)))))
            (else
              (Rendering|Components|TextRender|SetTextRenderColor _currentamountblue _returnvalue_6)
              (goto _label_2))))
        (:NewEnumerator2
          (if (Math|Integer|InRange(Integer) (Variables|Default|GetCurrentAmount) (- _correctamountpurple 2) (+ _correctamountpurple 2))
            (Utilities|FlowControl|Sequence
              (:then_0
                (Rendering|Components|TextRender|SetTextRenderColor _currentamountpurple _returnvalue_4)
                (bind _output_get_5 (Variables|Default|SetCurrentAmount (Variables|/Game/Engineers/Blueprints/Children/BP_ControlStation_Lab.BP_ControlStation_Lab_C|GetCorrectAmountPurple _controlstation)))
                (CallFunction|SetCurrentAmountText _output_get_5)
                (CallFunction|SnapBallBack _output_get_5)
                (Variables|/Game/Engineers/Blueprints/Children/BP_ControlStation_Lab.BP_ControlStation_Lab_C|SetCurAmountPurple _controlstation (Variables|Default|GetCurrentAmount) :!label _label_3))
              (:then_1
                (Utilities|FlowControl|DoOnce false
                  (:Completed
                    (bind _returnvalue_9 (Effects|SpawnEmitteratLocation "/Game/Artists/VFX/P_BubblesPD1.P_BubblesPD1" (Transformation|GetActorLocation (Variables|Default|GetTargetPurpBubbles))))
                    (Audio|Components|Audio|Play (Variables|Default|GetMatineePurpChem))
                    (Audio|Components|Audio|Play (Variables|Default|GetDrawChemicals) 0.0)
                    (Utilities|FlowControl|Delay 2.0)
                    (bind _output_get_6 (Variables|Default|SetNewVar_1 _returnvalue_9))
                    (Components|Activation|Deactivate _output_get_6)))))
            (else
              (Rendering|Components|TextRender|SetTextRenderColor :self _currentamountpurple)
              (goto _label_3))))))
    (:then_1
      (Utilities|FlowControl|DoOnce false) ; enters at Reset
    )
    (:then_2
      (bind _correct_ (CallFunction|CheckComplete))
      (if _correct_
        (Default|SetActive (Variables|Default|GetChargers))))))

(event EventBeginPlay
  (bind _ball (Variables|Default|GetBall))
  (Transformation|SetWorldLocation (Variables|Default|GetBall) (Spline|GetLocationatDistanceAlongSpline (Variables|Default|GetPath) 0.0 "World") false true)
  (switch Utilities|FlowControl|Switch|SwitchonSliderRotatorTypes (Variables|Default|GetType)
    (:NewEnumerator0
      (Rendering|Material|SetMaterial _ball 0 "/Game/Artists/Materials/M_LeftMagnetKeyDecal.M_LeftMagnetKeyDecal"))
    (:NewEnumerator1
      (Rendering|Material|SetMaterial _ball 0 "/Game/Artists/Materials/M_RightMagnetKeyDecal.M_RightMagnetKeyDecal"))
    (:NewEnumerator2
      (Rendering|Material|SetMaterial _ball 0 "/Game/Artists/Materials/M_MagnetKeyBoth.M_MagnetKeyBoth"))))

(event EventTick
  (params (DeltaSeconds :type Float%20%28single-precision%29))
  (bind _returnvalue (Math|Color|MakeColor 0.0 0.0 0.0))
  (bind _path (Variables|Default|GetPath))
  (bind _magnetkey (Variables|Default|GetmagnetKey))
  (bind _path_2 (Variables|Default|GetPath))
  (bind _controlstation (Variables|Default|GetControlStation))
  (bind _returnvalue_2 (Math|Conversions|ToColor(LinearColor) _returnvalue))
  (bind _magnettrigger (Variables|/Game/Engineers/Blueprints/Parents/BP_MagnetKey.BP_MagnetKey_C|GetMagnetTrigger _magnetkey))
  (bind _returnvalue_3 (Transformation|GetWorldLocation _magnettrigger))
  (bind _returnvalue_4 (Spline|FindLocationClosesttoWorldLocation _path_2 _returnvalue_3 "World"))
  (if (Utilities|IsValid _magnetkey)
    (if (and (Variables|/Game/Engineers/Blueprints/Parents/BP_MagnetKey.BP_MagnetKey_C|GetisOn _magnetkey) (Class|PrimitiveComponent|IsOverlappingComponent _magnettrigger (Variables|Default|GetBall)))
      (Transformation|SetWorldLocation (Variables|Default|GetBall) _returnvalue_4 false true)
      (bind _distance (CallFunction|FindDistanceAlongSpline _path _returnvalue_4))
      (CallFunction|SetCurrentAmountText (Math|Float|Truncate (Math|Float|MapRangeClamped (/ _distance (Math|Conversions|ToFloat(Integer) (- (Spline|GetNumberOfSplinePoints _path) 1))) 0.0 1.0 0.0 1e+02)))
      (Variables|Default|SetCurrentAmount (Math|Float|Truncate (Math|Float|MapRangeClamped (/ _distance (Math|Conversions|ToFloat(Integer) (- (Spline|GetNumberOfSplinePoints _path) 1))) 0.0 1.0 0.0 1e+02)))
      (Utilities|FlowControl|DoOnce false
        (:Completed
          (switch Utilities|FlowControl|Switch|SwitchonSliderRotatorTypes (Variables|Default|GetType)
            (:NewEnumerator0
              (Rendering|Components|TextRender|SetTextRenderColor (Variables|/Game/Engineers/Blueprints/Children/BP_ControlStation_Lab.BP_ControlStation_Lab_C|GetCurrentAmountRed _controlstation) _returnvalue_2))
            (:NewEnumerator1
              (Rendering|Components|TextRender|SetTextRenderColor (Variables|/Game/Engineers/Blueprints/Children/BP_ControlStation_Lab.BP_ControlStation_Lab_C|GetCurrentAmountBlue _controlstation) _returnvalue_2))
            (:NewEnumerator2
              (Rendering|Components|TextRender|SetTextRenderColor (Variables|/Game/Engineers/Blueprints/Children/BP_ControlStation_Lab.BP_ControlStation_Lab_C|GetCurrentAmountPurple _controlstation) _returnvalue_2))))))))

(event Collision|EventActorBeginOverlap
  (params (OtherActor :type Actor%20Object%20Reference))
  (bind _type (Variables|Default|GetType))
  (bind _asbp_magnet_key (Utilities|Casting|CastToBP_MagnetKey OtherActor))
  (if (Math|Boolean|ORBoolean (and (Utilities|Enum|Equal(Enum) (Variables|/Game/Engineers/Blueprints/Parents/BP_MagnetKey.BP_MagnetKey_C|GetHand _asbp_magnet_key) "Left") (Utilities|Enum|Equal(Enum) _type "NewEnumerator0")) (Utilities|Enum|Equal(Enum) _type "NewEnumerator2") (and (Utilities|Enum|Equal(Enum) _type "NewEnumerator1") (Utilities|Enum|Equal(Enum) (Variables|/Game/Engineers/Blueprints/Parents/BP_MagnetKey.BP_MagnetKey_C|GetHand _asbp_magnet_key) "Right")))
    (if (not (Utilities|IsValid (Variables|Default|GetmagnetKey)))
      (bind _output_get (Variables|Default|SetmagnetKey _asbp_magnet_key))
      (EventDispatchers|BindEventtoTurnedOff _output_get (delegate Custom|SnapAndChangeColor)))))

(event Collision|EventActorEndOverlap
  (params (OtherActor :type Actor%20Object%20Reference))
  (bind _asbp_magnet_key (Utilities|Casting|CastToBP_MagnetKey OtherActor))
  (if (== _asbp_magnet_key (Variables|Default|GetmagnetKey))
    (CallFunction|SnapandChangeColor)
    (if (Utilities|IsValid (Variables|Default|GetmagnetKey))
      (EventDispatchers|UnbindEventfromTurnedOff (Variables|Default|GetmagnetKey) (delegate Custom|SnapAndChangeColor))
      (Variables|Default|SetmagnetKey 0))))

(fn ConstructionScript
  (bind _path (Variables|Default|GetPath))
  (for _index (range 0 (- (Spline|GetNumberOfSplinePoints (Variables|Default|GetPath)) 2))
    (bind _returnvalue (AddComponent|AddSplineMeshComponent false))
    (Components|StaticMesh|SetStaticMesh _returnvalue (Variables|Default|GetpathMesh))
    (SplineMesh|SetForwardAxis _returnvalue (Variables|Default|GetForward%20Axis) true)
    (Transformation|AttachComponentToComponent _returnvalue (Variables|Default|GetPath) "None" "KeepRelative" "KeepRelative" "KeepRelative" true)
    (SplineMesh|SetStartandEnd _returnvalue (Spline|GetLocationatSplinePoint _path _index "Local") (Spline|GetTangentatSplinePoint _path _index "Local") (Spline|GetLocationatSplinePoint _path (+ _index 1) "Local") (Spline|GetTangentatSplinePoint _path (+ _index 1) "Local") true :!class /Script/Engine.SplineMeshComponent)))

(fn FindDistanceAlongSpline
  (params (Spline :type Spline%20Component%20Object%20Reference) (Location :type Vector))
  (return (Class|SplineComponent|FindInputKeyClosesttoWorldLocation Spline Location)))

(fn SetCurrentAmountText
  (params (Amount :type Integer))
  (bind _controlstation (Variables|Default|GetControlStation))
  (switch Utilities|FlowControl|Switch|SwitchonSliderRotatorTypes (Variables|Default|GetType)
    (:NewEnumerator0
      (Rendering|Components|TextRender|SetText (Variables|/Game/Engineers/Blueprints/Children/BP_ControlStation_Lab.BP_ControlStation_Lab_C|GetCurrentAmountRed _controlstation) (Utilities|Text|ToText(Integer) Amount)))
    (:NewEnumerator1
      (Rendering|Components|TextRender|SetText (Variables|/Game/Engineers/Blueprints/Children/BP_ControlStation_Lab.BP_ControlStation_Lab_C|GetCurrentAmountBlue _controlstation) (Utilities|Text|ToText(Integer) Amount)))
    (:NewEnumerator2
      (Rendering|Components|TextRender|SetText (Variables|/Game/Engineers/Blueprints/Children/BP_ControlStation_Lab.BP_ControlStation_Lab_C|GetCurrentAmountPurple _controlstation) (Utilities|Text|ToText(Integer) Amount)))))

(fn SnapBallBack
  (params (Amount :type Integer))
  (bind _path (Variables|Default|GetPath))
  (Transformation|SetWorldLocation (Variables|Default|GetBall) (Spline|GetLocationatDistanceAlongSpline _path (* (/ (Math|Conversions|ToFloat(Integer) Amount) 1e+02) (Spline|GetSplineLength _path)) "World") false true))

(fn CheckComplete
  (bind _controlstation (Variables|Default|GetControlStation))
  (return (Math|Boolean|ANDBoolean (== (Variables|/Game/Engineers/Blueprints/Children/BP_ControlStation_Lab.BP_ControlStation_Lab_C|GetCurAmountRed _controlstation) (Variables|/Game/Engineers/Blueprints/Children/BP_ControlStation_Lab.BP_ControlStation_Lab_C|GetCorrectAmountRed _controlstation)) (== (Variables|/Game/Engineers/Blueprints/Children/BP_ControlStation_Lab.BP_ControlStation_Lab_C|GetCurAmountBlue _controlstation) (Variables|/Game/Engineers/Blueprints/Children/BP_ControlStation_Lab.BP_ControlStation_Lab_C|GetCorrectAmountBlue _controlstation)) (== (Variables|/Game/Engineers/Blueprints/Children/BP_ControlStation_Lab.BP_ControlStation_Lab_C|GetCurAmountPurple _controlstation) (Variables|/Game/Engineers/Blueprints/Children/BP_ControlStation_Lab.BP_ControlStation_Lab_C|GetCorrectAmountPurple _controlstation)))))