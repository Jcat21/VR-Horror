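; Receptacle that takes a cryo pod and ends the crane game by moving the player to quarantine.
; When a cryo pod overlaps its trigger, it destroys the pod, fades the camera to red, teleports the player to QuarantineLoc, fades back in and unloads the CraneGame level.
; The correct-pod check makes no difference to the outcome.
; Level-loading nodes and an alternate fade-and-teleport chain are left disconnected.
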(event OnComponentBeginOverlap(RecepticleTrigger)
  (params (OverlappedComponent :type Primitive%20Component%20Object%20Reference) (OtherActor :type Actor%20Object%20Reference) (OtherComp :type Primitive%20Component%20Object%20Reference) (OtherBodyIndex :type Integer) (bFromSweep :type Boolean) (SweepResult :type Hit%20Result%20Structure%20%28by%20ref%29))
  (bind _playerref (Variables|Default|GetPlayerRef))
  (bind _playerref_2 (Variables|Default|GetPlayerRef))
  (bind _asbp_cryo_pod (Utilities|Casting|CastToBP_CryoPod OtherActor))
  (if (Variables|/Game/Engineers/Blueprints/Misc/BP_CryoPod.BP_CryoPod_C|GetisCorrectPod _asbp_cryo_pod)
    _
    (else
      _))
  (Actor|DestroyActor _asbp_cryo_pod)
  (CameraFades|StartCameraFade (Game|GetPlayerCameraManager 0) 0.0 1.0 5.0 "(R=1.000000,G=0.000000,B=0.000000,A=1.000000)" true true)
  (Utilities|FlowControl|Delay 5.0)
  (Default|SetNewTeleportLocs _playerref)
  (bind (_spawn _found_) (Default|FindTeleportLoc _playerref "QuarantineLoc"))
  (if _found_
    (Transformation|SetActorLocationAndRotation _playerref_2 (.location (Transformation|GetActorTransform _spawn)) (.rotation (Transformation|GetActorTransform _spawn)) false true)
    (Default|ResetPlayerHeight _playerref_2)
    (CameraFades|StartCameraFade (Game|GetPlayerCameraManager 0) 1.0 0.0 0.0 "(R=1.000000,G=0.000000,B=0.000000,A=1.000000)" true false)
    (Game|UnloadStreamLevel(byName) "CraneGame")))

(event EventBeginPlay
  (bind _asbp_main_pawn (Utilities|Casting|CastToBP_MainPawn (Game|Player|GetPlayerPawn 0)))
  (Variables|Default|SetPlayerRef _asbp_main_pawn))

(fn ConstructionScript)