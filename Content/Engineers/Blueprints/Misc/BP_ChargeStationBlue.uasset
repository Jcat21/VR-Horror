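; Blue charge station that gains power while the player's right-hand BP_MagnetKey overlaps it and is switched on.
; Overlap events flag the touching hand, and Tick adds transfer power, applies constant depletion and clamps the result.
; The current power drives a text readout, a slider widget's progress bar and the point light's intensity.
; Left-hand draining into the pawn's battery is left disconnected, and hand lookups search all key actors every frame.
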(event Collision|EventActorBeginOverlap
  (params (OtherActor :type Actor%20Object%20Reference))
  ;[1 1 1] Enable Power Sucking
  (bind _asbp_magnet_key (Utilities|Casting|CastToBP_MagnetKey OtherActor))
  (switch Utilities|FlowControl|Switch|SwitchonEControllerHand (Variables|/Game/Engineers/Blueprints/Parents/BP_MagnetKey.BP_MagnetKey_C|GetHand _asbp_magnet_key)
    (:Left
      (Variables|Default|SetIsBeingTouchedByLeft true))
    (:Right
      (Variables|Default|SetIsBeingTouhcedByRight true))))

(event Collision|EventActorEndOverlap
  (params (OtherActor :type Actor%20Object%20Reference))
  ;[1 1 1] Disable Power Sucking
  (bind _asbp_magnet_key (Utilities|Casting|CastToBP_MagnetKey OtherActor))
  (switch Utilities|FlowControl|Switch|SwitchonEControllerHand (Variables|/Game/Engineers/Blueprints/Parents/BP_MagnetKey.BP_MagnetKey_C|GetHand _asbp_magnet_key)
    (:Left
      (Variables|Default|SetIsBeingTouchedByLeft false))
    (:Right
      (Variables|Default|SetIsBeingTouhcedByRight false))))

(event EventTick
  (params (DeltaSeconds :type Float%20%28single-precision%29))
  (bind _minpower (Variables|Default|GetMinPower))
  (bind _maxpower (Variables|Default|GetMaxPower))
  (Variables|Default|SetDeltaTime DeltaSeconds)
  (Utilities|FlowControl|Sequence
    (:then_0
      (Utilities|FlowControl|Sequence
        (:then_0
          ;[1 1 1] Check if power can be transfered based on if right hand is in charge station and if it is on
          (bind _righthand (CallFunction|GetRightHand))
          (if (and (Variables|Default|GetIsBeingTouhcedByRight) (Variables|/Game/Engineers/Blueprints/Parents/BP_MagnetKey.BP_MagnetKey_C|GetisOn _righthand))
            (Variables|Default|SetIsTransferableRight true)
            (else
              (Variables|Default|SetIsTransferableRight false))))))
    (:then_1
      ;[1 1 1] Add power to this charge port
      (if (Variables|Default|GetIsTransferableRight)
        (bind _output_get (Variables|Default|SetCurrentPower (+ (Variables|Default|GetCurrentPower) (* (Variables|Default|GetTransferRate) (Variables|Default|GetDeltaTime)))))
        (Rendering|Components|TextRender|SetText (Actor|GetComponentbyClass "/Script/Engine.TextRenderComponent") (Utilities|Text|ToText(Float) _output_get "HalfToEven"))))
    (:then_2
      ;[1 1 1] Deplete current power and clamp current power
      (Variables|Default|SetCurrentPower (- (Variables|Default|GetCurrentPower) (* (/ (- (Variables|Default|GetMaxPower) (Variables|Default|GetMinPower)) (Variables|Default|GetDepleteFromFullTime)) DeltaSeconds)))
      (if (< (Variables|Default|GetCurrentPower) _minpower)
        (Variables|Default|SetCurrentPower _minpower)
        (elif (> (Variables|Default|GetCurrentPower) _maxpower)
          (Variables|Default|SetCurrentPower _maxpower)))
      (Rendering|Components|TextRender|SetText (Actor|GetComponentbyClass "/Script/Engine.TextRenderComponent") (Utilities|Text|ToText(String) (Utilities|Array|Get(acopy) (Utilities|String|ParseIntoArray (Utilities|String|ToString(Float) (Variables|Default|GetCurrentPower)) "."))))
      (bind _asbp_charge_station_slider_blue (Utilities|Casting|CastToBP_ChargeStationSliderBlue (UserInterface|GetUserWidgetObject (Variables|Default|GetWidget))))
      (Progress|SetPercent (Variables|/Game/Engineers/Blueprints/Misc/BP_ChargeStationSliderBlue.BP_ChargeStationSliderBlue_C|GetProgressBar_94 _asbp_charge_station_slider_blue) (* (/ (Variables|Default|GetCurrentPower) (Variables|Default|GetMaxPower)) 0.07)))
    (:then_3
      ;[1 1 1] Set light intensity
      (Rendering|Components|Light|SetIntensity (Variables|Default|GetPointLight) (* (/ (Variables|Default|GetCurrentPower) 1e+02) 1e+04)))))

(event EventBeginPlay
  ;[1 1 1] Set Hand and Player References
  (bind _asbp_main_pawn (Utilities|Casting|CastToBP_MainPawn (Game|Player|GetPlayerPawn 0)))
  (Variables|Default|SetPlayerPawn _asbp_main_pawn)
  (bind _outactors (Actor|GetAllActorsOfClass "/Game/Engineers/Blueprints/Parents/BP_MagnetKey.BP_MagnetKey_C"))
  (for _array_element _outactors
    (switch Utilities|FlowControl|Switch|SwitchonEControllerHand (Variables|/Game/Engineers/Blueprints/Parents/BP_MagnetKey.BP_MagnetKey_C|GetHand _array_element)
      (:Left
        (Variables|Default|SetLeftHand _array_element))
      (:Right
        (Variables|Default|SetRightHand _array_element)))))

(fn ConstructionScript
  (Rendering|Components|TextRender|SetText (Actor|GetComponentbyClass "/Script/Engine.TextRenderComponent") (Utilities|Text|ToText(Float) (Variables|Default|GetCurrentPower) "HalfToEven"))
  (Rendering|Components|Light|SetIntensity (Variables|Default|GetPointLight) (* (/ (Variables|Default|GetCurrentPower) 1e+02) 1e+04)))

(fn GetLeftHand
  (bind _outactors (Actor|GetAllActorsOfClass "/Game/Engineers/Blueprints/Parents/BP_MagnetKey.BP_MagnetKey_C"))
  (for _array_element _outactors
    (switch Utilities|FlowControl|Switch|SwitchonEControllerHand (Variables|/Game/Engineers/Blueprints/Parents/BP_MagnetKey.BP_MagnetKey_C|GetHand _array_element)
      (:Left
        (return _array_element)))))

(fn GetRightHand
  (bind _outactors (Actor|GetAllActorsOfClass "/Game/Engineers/Blueprints/Parents/BP_MagnetKey.BP_MagnetKey_C"))
  (for _array_element _outactors
    (switch Utilities|FlowControl|Switch|SwitchonEControllerHand (Variables|/Game/Engineers/Blueprints/Parents/BP_MagnetKey.BP_MagnetKey_C|GetHand _array_element)
      (:Right
        (return _array_element)))))