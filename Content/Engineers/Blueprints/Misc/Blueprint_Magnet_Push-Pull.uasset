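; Magnet-movable object that BP_MagnetKey actors carry around, with a HandType of Left, Right or Both that also picks its cube material.
; Overlap stores each hand's key until that key's TurnedOff event clears it; ending overlap only resets an interaction flag.
; While the required keys are on, Tick holds CubeA ahead of the key, matching yaw and keeping its height.
; Both requires two active keys but follows the left one.
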(event OnComponentEndOverlap(Sphere)
  (params (OverlappedComponent :type Primitive%20Component%20Object%20Reference) (OtherActor :type Actor%20Object%20Reference) (OtherComp :type Primitive%20Component%20Object%20Reference) (OtherBodyIndex :type Integer)))

(event Custom|LeftMagnetTurnOff
  (Variables|Default|SetIsInteractingWithMagnetKeyLeft false)
  (EventDispatchers|UnbindEventfromTurnedOff (Variables|Default|GetMagnetKey_L) (delegate Custom|LeftMagnetTurnOff))
  (Variables|Default|SetMagnetKey_L 0))

(event Custom|RightMagnetTurnOff
  (Variables|Default|SetIsInteractingWithMagnetKeyRight false)
  (EventDispatchers|UnbindEventfromTurnedOff (Variables|Default|GetMagnetKey_R) (delegate Custom|RightMagnetTurnOff))
  (Variables|Default|SetMagnetKey_R 0))

(event EventTick
  (params (DeltaSeconds :type Float%20%28single-precision%29))
  (bind _magnetkey_l (Variables|Default|GetMagnetKey_L))
  (bind _magnetkey_r (Variables|Default|GetMagnetKey_R))
  (bind _returnvalue (Utilities|IsValid _magnetkey_l))
  (bind _returnvalue_2 (Utilities|IsValid _magnetkey_r))
  (bind _ison (Variables|/Game/Engineers/Blueprints/Parents/BP_MagnetKey.BP_MagnetKey_C|GetisOn _magnetkey_l))
  (bind _ison_2 (Variables|/Game/Engineers/Blueprints/Parents/BP_MagnetKey.BP_MagnetKey_C|GetisOn _magnetkey_r))
  (switch Utilities|FlowControl|Switch|SwitchonObjectDragTypes (Variables|Default|GetHandType)
    (:NewEnumerator0
      (if _returnvalue
        (if _ison
          (CallFunction|SetObjectLocation (Variables|Default|GetMagnetKey_L) :!label _label))))
    (:NewEnumerator1
      (if _returnvalue_2
        (if _ison_2
          (CallFunction|SetObjectLocation (Variables|Default|GetMagnetKey_R)))))
    (:NewEnumerator2
      (if (and _returnvalue_2 _returnvalue)
        (if (and _ison_2 _ison)
          (goto _label))))))

(event Collision|EventActorBeginOverlap
  (params (OtherActor :type Actor%20Object%20Reference))
  (bind _asbp_magnet_key (Utilities|Casting|CastToBP_MagnetKey OtherActor))
  (switch Utilities|FlowControl|Switch|SwitchonEControllerHand (Variables|/Game/Engineers/Blueprints/Parents/BP_MagnetKey.BP_MagnetKey_C|GetHand _asbp_magnet_key)
    (:Left
      (Variables|Default|SetIsInteractingWithMagnetKeyLeft true)
      (bind _output_get (Variables|Default|SetMagnetKey_L _asbp_magnet_key))
      (EventDispatchers|BindEventtoTurnedOff _output_get (delegate Custom|LeftMagnetTurnOff)))
    (:Right
      (Variables|Default|SetIsInteractingWithMagnetKeyRight true)
      (bind _output_get_2 (Variables|Default|SetMagnetKey_R _asbp_magnet_key))
      (EventDispatchers|BindEventtoTurnedOff _output_get_2 (delegate Custom|RightMagnetTurnOff)))))

(event Collision|EventActorEndOverlap
  (params (OtherActor :type Actor%20Object%20Reference))
  (bind _asbp_magnet_key (Utilities|Casting|CastToBP_MagnetKey OtherActor))
  (switch Utilities|FlowControl|Switch|SwitchonEControllerHand (Variables|/Game/Engineers/Blueprints/Parents/BP_MagnetKey.BP_MagnetKey_C|GetHand _asbp_magnet_key)
    (:Left
      (Variables|Default|SetIsInteractingWithMagnetKeyLeft false))
    (:Right
      (Variables|Default|SetIsInteractingWithMagnetKeyRight false))))

(fn ConstructionScript
  (bind _cubea (Variables|Default|GetCubeA))
  (switch Utilities|FlowControl|Switch|SwitchonObjectDragTypes (Variables|Default|GetHandType)
    (:NewEnumerator0
      (Rendering|Material|SetMaterial _cubea 0 "/Game/Artists/Materials/test_M_2-2.test_M_2-2"))
    (:NewEnumerator1
      (Rendering|Material|SetMaterial _cubea 0 "/Game/Artists/Materials/bluedot.bluedot"))
    (:NewEnumerator2
      (Rendering|Material|SetMaterial _cubea 0 "/Game/Artists/Materials/M_MagnetKeyBoth.M_MagnetKeyBoth"))))

(fn SetObjectLocation
  (params (MagnetKey :type BP%20Magnet%20Key%20Object%20Reference))
  (bind _returnvalue (Transformation|GetActorForwardVector MagnetKey))
  (bind _returnvalue_2 (Transformation|GetActorLocation MagnetKey))
  (bind _returnvalue_3 (* _returnvalue 1.1e+02))
  (bind _returnvalue_4 (+ _returnvalue_2 _returnvalue_3))
  (bind (_x _y) (Math|Vector|BreakVector _returnvalue_4))
  (Transformation|SetWorldLocationAndRotation (Variables|Default|GetCubeA) (Math|Vector|MakeVector _x _y (.Z (Math|Vector|BreakVector (Transformation|GetWorldLocation (Variables|Default|GetCubeA))))) (Math|Rotator|MakeRotator 0.0 0.0 (.Yaw (Math|Rotator|BreakRotator (Transformation|GetActorRotation MagnetKey)))) false false))