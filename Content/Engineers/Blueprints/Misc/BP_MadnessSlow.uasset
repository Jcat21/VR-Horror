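; Trigger actor that depletes madness while the player's BP_MainPawn is inside its bounds.
; Overlap with MadnessBounds toggles IsDepleting, and Tick then calls DepleteMadness on MadnessSlow every frame, using the actor's location as the detection center.
; A second volume, FastDepleteTest, sets IsDepletingFast on the pawn while it overlaps.
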(event OnComponentBeginOverlap(MadnessBounds)
  (params (OverlappedComponent :type Primitive%20Component%20Object%20Reference) (OtherActor :type Actor%20Object%20Reference) (OtherComp :type Primitive%20Component%20Object%20Reference) (OtherBodyIndex :type Integer) (bFromSweep :type Boolean) (SweepResult :type Hit%20Result%20Structure%20%28by%20ref%29))
  (Utilities|Casting|CastToBP_MainPawn OtherActor)
  (Variables|Default|SetIsDepleting true))

(event OnComponentBeginOverlap(FastDepleteTest)
  (params (OverlappedComponent :type Primitive%20Component%20Object%20Reference) (OtherActor :type Actor%20Object%20Reference) (OtherComp :type Primitive%20Component%20Object%20Reference) (OtherBodyIndex :type Integer) (bFromSweep :type Boolean) (SweepResult :type Hit%20Result%20Structure%20%28by%20ref%29))
  ;[1 1 1] PD Additions
  (bind _asbp_main_pawn (Utilities|Casting|CastToBP_MainPawn OtherActor))
  (Variables|/Game/Engineers/Blueprints/Parents/BP_MainPawn.BP_MainPawn_C|SetIsDepletingFast _asbp_main_pawn true))

(event OnComponentEndOverlap(FastDepleteTest)
  (params (OverlappedComponent :type Primitive%20Component%20Object%20Reference) (OtherActor :type Actor%20Object%20Reference) (OtherComp :type Primitive%20Component%20Object%20Reference) (OtherBodyIndex :type Integer))
  ;[1 1 1] PD Additions
  (bind _asbp_main_pawn (Utilities|Casting|CastToBP_MainPawn OtherActor))
  (Variables|/Game/Engineers/Blueprints/Parents/BP_MainPawn.BP_MainPawn_C|SetIsDepletingFast _asbp_main_pawn false))

(event OnComponentEndOverlap(MadnessBounds)
  (params (OverlappedComponent :type Primitive%20Component%20Object%20Reference) (OtherActor :type Actor%20Object%20Reference) (OtherComp :type Primitive%20Component%20Object%20Reference) (OtherBodyIndex :type Integer))
  (Utilities|Casting|CastToBP_MainPawn OtherActor)
  (Variables|Default|SetIsDepleting false))

(event EventBeginPlay)

(event Collision|EventActorBeginOverlap
  (params (OtherActor :type Actor%20Object%20Reference)))

(event EventTick
  (params (DeltaSeconds :type Float%20%28single-precision%29))
  (if (Variables|Default|GetIsDepleting)
    (Default|DepleteMadness (Variables|Default|GetMadnessSlow) (Transformation|GetActorLocation) "0, 0, 0")))

(fn ConstructionScript)