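; Grid actor of sphere junctions that snaps a BP_SliderObject onto the junction it overlaps.
; On overlap it teleports the slider to that junction, flags whether it sits on an edge row or column, and resets its movement.
; Movement on the SliderObject reference re-enables after a short delay, then disables a second later if still colliding; end overlap clears all flags.
; A timeline-based lerp snap is left unconnected, and the Find edge functions duplicate the inline checks.
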(event Collision|EventActorBeginOverlap
  (params (OtherActor :type Actor%20Object%20Reference))
  (bind _sliderobject (Variables|Default|GetsliderObject))
  (bind _asbp_slider_object (Utilities|Casting|CastToBP_SliderObject OtherActor))
  (Variables|Default|SetisColliding true)
  (Variables|/Game/Engineers/Blueprints/Misc/BP_SliderObject.BP_SliderObject_C|SetcanMove _asbp_slider_object false)
  (for _array_element (Class|Actor|GetOverlappingComponents _asbp_slider_object)
    (if (== (Components|GetOwner _array_element) self)
      (Transformation|SetActorLocation _asbp_slider_object (Transformation|GetWorldLocation _array_element) false true)
      (Utilities|FlowControl|Sequence
        (:then_0
          (Variables|Default|SetisInTopRow (Math|Boolean|ORBoolean (== _array_element (Variables|Components|Getx0y0)) (== _array_element (Variables|Components|Getx0y1)) (== _array_element (Variables|Components|Getx0y2)) (== _array_element (Variables|Default|Getx0y3)) (== _array_element (Variables|Default|Getx0y4))))
          (Variables|Default|SetisInBottomRow (Math|Boolean|ORBoolean (== _array_element (Variables|Default|GetSphere15)) (== _array_element (Variables|Default|GetSphere18)) (== _array_element (Variables|Default|GetSphere17)) (== _array_element (Variables|Default|GetSphere16)) (== _array_element (Variables|Default|GetSphere19)))))
        (:then_1
          (Variables|Default|SetisInLeftColumn (Math|Boolean|ORBoolean (== _array_element (Variables|Components|Getx0y0)) (== _array_element (Variables|Components|GetSphere3)) (== _array_element (Variables|Default|GetSphere7)) (== _array_element (Variables|Default|GetSphere20)) (== _array_element (Variables|Default|GetSphere15))))
          (Variables|Default|SetisInRightColumn (Math|Boolean|ORBoolean (== _array_element (Variables|Default|Getx0y4)) (== _array_element (Variables|Default|GetSphere14)) (== _array_element (Variables|Default|GetSphere9)) (== _array_element (Variables|Default|GetSphere21)) (== _array_element (Variables|Default|GetSphere19))))))))
  (Default|ResetHorizontalMovement _asbp_slider_object)
  (Default|ResetVerticalMovement _asbp_slider_object)
  (Utilities|FlowControl|Delay 0.08)
  (Variables|/Game/Engineers/Blueprints/Misc/BP_SliderObject.BP_SliderObject_C|SetcanMove (Variables|Default|GetsliderObject) true)
  (Utilities|FlowControl|Delay 1.0)
  (if (Variables|Default|GetisColliding)
    (Utilities|IsValid _sliderobject
      (:Is%20Valid
        (Variables|/Game/Engineers/Blueprints/Misc/BP_SliderObject.BP_SliderObject_C|SetcanMove _sliderobject false)))))

(event Collision|EventActorEndOverlap
  (params (OtherActor :type Actor%20Object%20Reference))
  (Utilities|Casting|CastToBP_SliderObject OtherActor)
  (Variables|Default|SetisInTopRow false)
  (Variables|Default|SetisInBottomRow false)
  (Variables|Default|SetisInLeftColumn false)
  (Variables|Default|SetisInRightColumn false)
  (Variables|Default|SetisColliding false))

(fn ConstructionScript)

(fn FindIsinTopRow
  (params (ColliderJunction :type Sphere%20Component%20Object%20Reference))
  (return (Math|Boolean|ORBoolean (== ColliderJunction (Variables|Components|Getx0y0)) (== ColliderJunction (Variables|Components|Getx0y1)) (== ColliderJunction (Variables|Components|Getx0y2)) (== ColliderJunction (Variables|Default|Getx0y3)) (== ColliderJunction (Variables|Default|Getx0y4)))))

(fn FindIsinBottomRow
  (params (ColliderJunction :type Sphere%20Component%20Object%20Reference))
  (return (Math|Boolean|ORBoolean (== ColliderJunction (Variables|Default|GetSphere15)) (== ColliderJunction (Variables|Default|GetSphere18)) (== ColliderJunction (Variables|Default|GetSphere17)) (== ColliderJunction (Variables|Default|GetSphere16)) (== ColliderJunction (Variables|Default|GetSphere19)))))

(fn FindIsinLeftColumn
  (params (ColliderJunction :type Sphere%20Component%20Object%20Reference))
  (return (Math|Boolean|ORBoolean (== ColliderJunction (Variables|Components|Getx0y0)) (== ColliderJunction (Variables|Components|GetSphere3)) (== ColliderJunction (Variables|Default|GetSphere7)) (== ColliderJunction (Variables|Default|GetSphere20)) (== ColliderJunction (Variables|Default|GetSphere15)))))

(fn FindIsinRightColumn
  (params (ColliderJunction :type Sphere%20Component%20Object%20Reference))
  (return (Math|Boolean|ORBoolean (== ColliderJunction (Variables|Default|Getx0y4)) (== ColliderJunction (Variables|Default|GetSphere14)) (== ColliderJunction (Variables|Default|GetSphere9)) (== ColliderJunction (Variables|Default|GetSphere21)) (== ColliderJunction (Variables|Default|GetSphere19)))))