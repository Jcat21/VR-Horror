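; LaserInteract tracks focus and index-action state for an object, likely one targeted by laser pointers, judging by its name.
; A reference count lets several instigators share focus, signalling focus gain and loss as the first arrives and the last leaves.
; It records the instigator of the current index action and, when that instigator's reference is removed, fires the action stop before updating focus.
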(event Custom|IndexStart
  (params (instigator :type Hand%20BP%20Object%20Reference))
  (Variables|Default|SetIndexActionCaller instigator))

(event Custom|IndexStop
  (params (instigator :type Hand%20BP%20Object%20Reference))
  (if (== instigator (Variables|Default|GetIndexActionCaller))
    (Variables|Default|SetIndexActionCaller 0)))

(event EventBeginPlay
  (EventDispatchers|BindEventtoIndexAction (delegate Custom|IndexStart))
  (EventDispatchers|BindEventtoIndexActionStop (delegate Custom|IndexStop)))

(fn AddReference
  (params (Instigator :type Hand%20BP%20Object%20Reference))
  (bind _result (Math|Integer|IncrementInt (Variables|Default|GetRefCount))
    (:%20%20
      (if (== _result 1)
        (Default|CallFocusGain)))))

(fn RemoveReference
  (params (Instigator :type Hand%20BP%20Object%20Reference))
  (if (== Instigator (Variables|Default|GetIndexActionCaller))
    (Default|CallIndexActionStop Instigator)
    (Variables|Default|SetIndexActionCaller 0))
  (bind _result (Math|Integer|DecrementInt (Variables|Default|GetRefCount))
    (:%20%20
      (if (== _result 0)
        (Default|CallFocusLost)))))

(fn HasFocus
  (return (> (Variables|Default|GetRefCount) 0)))