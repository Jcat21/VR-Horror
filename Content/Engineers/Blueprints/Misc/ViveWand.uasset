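; Vive wand input component that translates motion controller keys into actions on its HandActor, filtered by whether it is the left or right hand.
; Grip is hold-to-grab and updates the hand animation; trigger and face button 3 drive index and thumb actions.
; Teleport uses the trackpad when empty-handed and face button 1 while holding an object.
; Shoulder buttons toggle the pawn's laser.
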(event EventTick
  (params (DeltaSeconds :type Float%20%28single-precision%29))
  (|CallParentFunction DeltaSeconds))

(event Input|KeyboardEvents|MotionControllerRightShoulder
  (params (Key :type Key%20Structure))
  (:Pressed
    (if (Utilities|Enum|Equal(Enum) (Variables|Default|GetHand) "Right")
      (Default|ToggleLaser (Variables|/Game/Engineers/Blueprints/Parents/HandBP.HandBP_C|GetMyPawn (Variables|Default|GetHandActor))))))

(event Input|KeyboardEvents|MotionControllerRightThumbstick
  (params (Key :type Key%20Structure))
  (bind _handactor (Variables|Default|GetHandActor))
  (bind _hand (Variables|Default|GetHand))
  (bind _value (Default|HoldingObject _handactor))
  (bind _returnvalue (Utilities|Enum|Equal(Enum) _hand "Right"))
  (bind _returnvalue_2 (not _value))
  ;[1 1 1] Teleporter while not holding anythings uses entire trackpad
  (:Pressed
    (if _returnvalue
      (if _returnvalue_2
        (Default|ActivateTeleport _handactor))))
  (:Released
    (if _returnvalue
      (if _returnvalue_2
        (Default|DeactivateTeleport _handactor)))))

(event Input|KeyboardEvents|MotionControllerRightTrigger
  (params (Key :type Key%20Structure))
  (bind _hand (Variables|Default|GetHand))
  (bind _handactor (Variables|Default|GetHandActor))
  (bind _returnvalue (Utilities|Enum|Equal(Enum) _hand "Right"))
  (:Pressed
    (if _returnvalue
      (Default|IndexAction _handactor)))
  (:Released
    (if _returnvalue
      (Default|IndexActionEnd _handactor))))

(event Input|KeyboardEvents|MotionControllerLeftShoulder
  (params (Key :type Key%20Structure))
  (:Pressed
    (if (Utilities|Enum|Equal(Enum) (Variables|Default|GetHand) "Left")
      (Default|ToggleLaser (Variables|/Game/Engineers/Blueprints/Parents/HandBP.HandBP_C|GetMyPawn (Variables|Default|GetHandActor))))))

(event Input|KeyboardEvents|MotionControllerLeftTrigger
  (params (Key :type Key%20Structure))
  (bind _hand (Variables|Default|GetHand))
  (bind _handactor (Variables|Default|GetHandActor))
  (bind _returnvalue (Utilities|Enum|Equal(Enum) _hand "Left"))
  (:Pressed
    (if _returnvalue
      (Default|IndexAction _handactor)))
  (:Released
    (if _returnvalue
      (Default|IndexActionEnd _handactor))))

(event Input|KeyboardEvents|MotionControllerRightGrip1
  (params (Key :type Key%20Structure))
  (bind _handactor (Variables|Default|GetHandActor))
  (bind _hand (Variables|Default|GetHand))
  (bind _returnvalue (Utilities|Enum|Equal(Enum) _hand "Right"))
  ;[1 1 1] Grabbing on VIve is push to grab, push to release
  (:Pressed
    (if _returnvalue
      (Default|AttemptGrab _handactor)
      (Default|UpdateHandAnimation _handactor 0.0 0.0 0.0 0.0 0.0)))
  (:Released
    (if _returnvalue
      (Default|Release _handactor)
      (Default|UpdateHandAnimation _handactor 0.5 0.8 0.8 0.8 0.8))))

(event Input|KeyboardEvents|MotionControllerLeftThumbstickUp
  (params (Key :type Key%20Structure))
  (bind _handactor (Variables|Default|GetHandActor))
  (bind _hand (Variables|Default|GetHand))
  (bind _value (Default|HoldingObject _handactor))
  (bind _returnvalue (Utilities|Enum|Equal(Enum) _hand "Left"))
  (bind _returnvalue_2 (not _value))
  ;[1 1 1] Teleporter while not holding anythings uses entire trackpad
  (:Pressed
    (if _returnvalue
      (if _returnvalue_2
        (Default|ActivateTeleport _handactor))))
  (:Released
    (if _returnvalue
      (if _returnvalue_2
        (Default|DeactivateTeleport _handactor)))))

(event Input|KeyboardEvents|MotionControllerLeftGrip1
  (params (Key :type Key%20Structure))
  (bind _handactor (Variables|Default|GetHandActor))
  (bind _hand (Variables|Default|GetHand))
  (bind _returnvalue (Utilities|Enum|Equal(Enum) _hand "Left"))
  ;[1 1 1] Grabbing on VIve is push to grab, push to release
  (:Pressed
    (if _returnvalue
      (Default|AttemptGrab _handactor)
      (Default|UpdateHandAnimation _handactor 0.0 0.0 0.0 0.0 0.0)))
  (:Released
    (if _returnvalue
      (Default|Release _handactor)
      (Default|UpdateHandAnimation _handactor 0.5 0.8 0.8 0.8 0.8))))

(event Input|KeyboardEvents|MotionControllerRightFaceButton1
  (params (Key :type Key%20Structure))
  (bind _hand (Variables|Default|GetHand))
  (bind _handactor (Variables|Default|GetHandActor))
  (bind _value (Default|HoldingObject _handactor))
  (bind _returnvalue (Utilities|Enum|Equal(Enum) _hand "Right"))
  ;[1 1 1] When holding an object, Face1 is used for teleporter
  (:Pressed
    (if _returnvalue
      (if _value
        (Default|ActivateTeleport _handactor))))
  (:Released
    (if _returnvalue
      (if _value
        (Default|DeactivateTeleport _handactor)))))

(event Input|KeyboardEvents|MotionControllerLeftFaceButton1
  (params (Key :type Key%20Structure))
  (bind _handactor (Variables|Default|GetHandActor))
  (bind _hand (Variables|Default|GetHand))
  (bind _value (Default|HoldingObject _handactor))
  (bind _returnvalue (Utilities|Enum|Equal(Enum) _hand "Left"))
  ;[1 1 1] When holding an object, Face1 is used for teleporter
  (:Pressed
    (if _returnvalue
      (if _value
        (Default|ActivateTeleport _handactor))))
  (:Released
    (if _returnvalue
      (if _value
        (Default|DeactivateTeleport _handactor)))))

(event Input|KeyboardEvents|MotionControllerRightFaceButton3
  (params (Key :type Key%20Structure))
  (bind _handactor (Variables|Default|GetHandActor))
  (bind _hand (Variables|Default|GetHand))
  (bind _returnvalue (Utilities|Enum|Equal(Enum) _hand "Right"))
  (:Pressed
    (if _returnvalue
      (Default|ThumbAction _handactor)))
  (:Released
    (if _returnvalue
      (Default|ThumbActionEnd _handactor))))

(event Input|KeyboardEvents|MotionControllerLeftFaceButton3
  (params (Key :type Key%20Structure))
  (bind _handactor (Variables|Default|GetHandActor))
  (bind _hand (Variables|Default|GetHand))
  (bind _returnvalue (Utilities|Enum|Equal(Enum) _hand "Left"))
  (:Pressed
    (if _returnvalue
      (Default|ThumbAction _handactor)))
  (:Released
    (if _returnvalue
      (Default|ThumbActionEnd _handactor))))

(fn ConstructionScript
  (|CallParentFunction))