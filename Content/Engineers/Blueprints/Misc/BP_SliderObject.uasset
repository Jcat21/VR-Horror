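; BP_SliderObject is a puzzle piece that a BP_MagnetKey drags around a SliderGrid, starting at the grid's start point.
; While the magnet is on and overlapping, Tick follows its trigger along the dominant velocity axis, Y or Z, blocking movement past edge rows and columns.
; Resettable DoOnce gates lock movement to one axis.
; When the magnet turns off or overlap ends, the piece snaps to the nearest grid sphere node.
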(event Custom|Reset%20Vertical%20Movement
  (Variables|Default|SetisMovingVertically false)
  (Utilities|FlowControl|DoOnce false) ; enters at Reset
)

(event Custom|SnapBackToNearestNode
  (Variables|Default|SetclosestNodeDistance 1e+07)
  (for _array_element (Actor|GetComponentsByClass (Variables|Default|GetsliderGrid) "/Script/Engine.SphereComponent")
    (if (< (Math|Vector|VectorLength (- (Transformation|GetWorldLocation _array_element) (Transformation|GetActorLocation))) (Variables|Default|GetclosestNodeDistance))
      (Variables|Default|SetclosestNode _array_element)
      (Variables|Default|SetclosestNodeDistance (Math|Vector|VectorLength (- (Transformation|GetWorldLocation _array_element) (Transformation|GetActorLocation))))))
  (Transformation|SetActorLocation (Transformation|GetWorldLocation (Variables|Default|GetclosestNode)) true false))

(event Custom|Reset%20Horizontal%20Movement
  (Variables|Default|SetisMovingHorizontally false)
  (Utilities|FlowControl|DoOnce false) ; enters at Reset
)

(event EventBeginPlay
  (Transformation|SetActorLocation (Transformation|GetWorldLocation (Variables|/Game/Engineers/Blueprints/Misc/BP_SliderGrid.BP_SliderGrid_C|GetStartPoint (Variables|Default|GetsliderGrid))) false true))

(event Collision|EventActorBeginOverlap
  (params (OtherActor :type Actor%20Object%20Reference))
  (bind _asbp_magnet_key (Utilities|Casting|CastToBP_MagnetKey OtherActor))
  (Variables|Default|SetisInteractingWithMagnetKey true)
  (bind _output_get (Variables|Default|SetmagnetKey _asbp_magnet_key))
  (EventDispatchers|BindEventtoTurnedOff _output_get (delegate Custom|SnapBackToNearestNode))
  (Variables|/Game/Engineers/Blueprints/Parents/BP_MagnetKey.BP_MagnetKey_C|SetIsInteractingWithSomething _output_get true)
  (Default|TurnOffLight _output_get))

(event EventTick
  (params (DeltaSeconds :type Float%20%28single-precision%29))
  (bind _returnvalue (Transformation|GetActorLocation))
  (bind _slidergrid (Variables|Default|GetsliderGrid))
  (bind _magnetkey (Variables|Default|GetmagnetKey))
  (bind _slidergrid_2 (Variables|Default|GetsliderGrid))
  (bind _magnetkey_2 (Variables|Default|GetmagnetKey))
  (bind _isintoprow (Variables|/Game/Engineers/Blueprints/Misc/BP_SliderGrid.BP_SliderGrid_C|GetisInTopRow _slidergrid))
  (bind _isinbottomrow (Variables|/Game/Engineers/Blueprints/Misc/BP_SliderGrid.BP_SliderGrid_C|GetisInBottomRow _slidergrid))
  (bind _isinrightcolumn (Variables|/Game/Engineers/Blueprints/Misc/BP_SliderGrid.BP_SliderGrid_C|GetisInRightColumn _slidergrid_2))
  (bind _isinleftcolumn (Variables|/Game/Engineers/Blueprints/Misc/BP_SliderGrid.BP_SliderGrid_C|GetisInLeftColumn _slidergrid_2))
  (bind _magnettrigger (Variables|/Game/Engineers/Blueprints/Parents/BP_MagnetKey.BP_MagnetKey_C|GetMagnetTrigger _magnetkey))
  (bind _returnvalue_2 (Transformation|GetWorldLocation _magnettrigger))
  (if (Variables|Default|GetcanMove)
    (if (and (Variables|Default|GetisInteractingWithMagnetKey) (Utilities|IsValid _magnetkey_2))
      (if (and (Variables|/Game/Engineers/Blueprints/Parents/BP_MagnetKey.BP_MagnetKey_C|GetisOn _magnetkey_2) (Collision|IsOverlappingActor (Variables|/Game/Engineers/Blueprints/Parents/BP_MagnetKey.BP_MagnetKey_C|GetMagnetTrigger _magnetkey_2) self :!class /Script/Engine.PrimitiveComponent))
        (bind _returnvalue_3 (Physics|GetPhysicsLinearVelocity (Variables|/Game/Engineers/Blueprints/Parents/BP_MagnetKey.BP_MagnetKey_C|GetMagnetTrigger (Variables|Default|GetmagnetKey)) "None"))
        (if (> (Math|Float|Absolute(Float) (.y _returnvalue_3)) (Math|Float|Absolute(Float) (.z _returnvalue_3)))
          (if (or _isinrightcolumn _isinleftcolumn)
            (if (not (or (and (> (.y _returnvalue_3) 0.0) _isinrightcolumn) (and _isinleftcolumn (< (.y _returnvalue_3) 0.0))))
              (Utilities|FlowControl|Sequence :!label _label
                (:then_0
                  (Utilities|FlowControl|DoOnce false
                    (:Completed
                      (if (not (Variables|Default|GetisMovingVertically))
                        (Variables|Default|SetisMovingHorizontally true)))))
                (:then_1
                  (if (and (Variables|Default|GetisMovingHorizontally) (not (Variables|Default|GetisMovingVertically)))
                    (Transformation|SetActorLocation (Math|Vector|MakeVector (.x _returnvalue) (.y _returnvalue_2) (.z _returnvalue)) false false)))))
            (else
              (goto _label)))
          (elif (or _isintoprow _isinbottomrow)
            (if (not (or (and (> (.z _returnvalue_3) 0.0) _isintoprow) (and _isinbottomrow (< (.z _returnvalue_3) 0.0))))
              (Utilities|FlowControl|Sequence :!label _label_2
                (:then_0
                  (Utilities|FlowControl|DoOnce false
                    (:Completed
                      (if (not (Variables|Default|GetisMovingHorizontally))
                        (Variables|Default|SetisMovingVertically true)))))
                (:then_1
                  (if (and (Variables|Default|GetisMovingVertically) (not (Variables|Default|GetisMovingHorizontally)))
                    (Transformation|SetActorLocation (Math|Vector|MakeVector (.x _returnvalue) (.y _returnvalue) (.z _returnvalue_2)) false false)))))
            (else
              (goto _label_2))))))))

(event Collision|EventActorEndOverlap
  (params (OtherActor :type Actor%20Object%20Reference))
  (bind _asbp_magnet_key (Utilities|Casting|CastToBP_MagnetKey OtherActor))
  (Variables|/Game/Engineers/Blueprints/Parents/BP_MagnetKey.BP_MagnetKey_C|SetIsInteractingWithSomething _asbp_magnet_key false)
  (if (Variables|/Game/Engineers/Blueprints/Parents/BP_MagnetKey.BP_MagnetKey_C|GetisOn _asbp_magnet_key)
    (Default|TurnonLight _asbp_magnet_key))
  (Default|ChangetoDimmerMaterial _asbp_magnet_key)
  (EventDispatchers|UnbindEventfromTurnedOff _asbp_magnet_key (delegate Custom|SnapBackToNearestNode))
  (Variables|Default|SetmagnetKey 0)
  (CallFunction|SnapBacktoNearestNode))

(fn ConstructionScript)