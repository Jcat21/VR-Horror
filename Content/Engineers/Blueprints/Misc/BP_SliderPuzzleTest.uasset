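; BP_SliderPuzzleTest is a test slider puzzle where a BP_MagnetKey drags a ball along Y or Z.
; Actor overlaps store or clear the key reference.
; While the key is on and its trigger overlaps the ball, Tick copies the trigger's Y or Z position to the ball, choosing the axis with greater trigger velocity.
; The left collider is meant to snap the ball to itself; the other four collider handlers are empty.
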(event Collision|EventActorBeginOverlap
  (params (OtherActor :type Actor%20Object%20Reference))
  (bind _asbp_magnet_key (Utilities|Casting|CastToBP_MagnetKey OtherActor))
  (Variables|Default|SetisInteractingWithMagnetKey true)
  (Variables|Default|SetmagnetKey _asbp_magnet_key))

(event EventTick
  (params (DeltaSeconds :type Float%20%28single-precision%29))
  (bind _magnetkey (Variables|Default|GetmagnetKey))
  (bind _ball (Variables|Default|GetBall))
  (bind _magnetkey_2 (Variables|Default|GetmagnetKey))
  (bind _returnvalue (Transformation|GetWorldLocation _ball))
  (bind _magnettrigger (Variables|/Game/Engineers/Blueprints/Parents/BP_MagnetKey.BP_MagnetKey_C|GetMagnetTrigger _magnetkey))
  (bind _returnvalue_2 (Transformation|GetWorldLocation _magnettrigger))
  (if (and (Variables|Default|GetisInteractingWithMagnetKey) (Utilities|IsValid _magnetkey_2))
    (if (and (Variables|/Game/Engineers/Blueprints/Parents/BP_MagnetKey.BP_MagnetKey_C|GetisOn _magnetkey_2) (Class|PrimitiveComponent|IsOverlappingComponent (Variables|/Game/Engineers/Blueprints/Parents/BP_MagnetKey.BP_MagnetKey_C|GetMagnetTrigger _magnetkey_2) (Variables|Default|GetBall)))
      (bind _returnvalue_3 (Physics|GetPhysicsLinearVelocity (Variables|/Game/Engineers/Blueprints/Parents/BP_MagnetKey.BP_MagnetKey_C|GetMagnetTrigger (Variables|Default|GetmagnetKey)) "None"))
      (if (> (Math|Float|Absolute(Float) (.y _returnvalue_3)) (Math|Float|Absolute(Float) (.z _returnvalue_3)))
        (Transformation|SetWorldLocation _ball (Math|Vector|MakeVector (.x _returnvalue) (.y _returnvalue_2) (.z _returnvalue)) false false)
        (else
          (Transformation|SetWorldLocation _ball (Math|Vector|MakeVector (.x _returnvalue) (.y _returnvalue) (.z _returnvalue_2)) false false))))))

(event Collision|EventActorEndOverlap
  (params (OtherActor :type Actor%20Object%20Reference))
  (Utilities|Casting|CastToBP_MagnetKey OtherActor)
  (Variables|Default|SetmagnetKey 0))

(event OnComponentBeginOverlap(Collider_Left)
  (params (OverlappedComponent :type Primitive%20Component%20Object%20Reference) (OtherActor :type Actor%20Object%20Reference) (OtherComp :type Primitive%20Component%20Object%20Reference) (OtherBodyIndex :type Integer) (bFromSweep :type Boolean) (SweepResult :type Hit%20Result%20Structure%20%28by%20ref%29))
  (bind _ball (Variables|Default|GetBall))
  (bind _collider_left (Variables|Default|GetCollider_Left))
  (bind _returnvalue (Transformation|GetWorldLocation _collider_left))
  (bind (_x _y _z) (Math|Vector|BreakVector _returnvalue))
  (Utilities|IsValid OtherActor
    (:Is%20Valid
      (if (== OtherActor _ball)
        (Transformation|SetWorldLocation _ball (Math|Vector|MakeVector _x _y _z) false true)))))

(event OnComponentBeginOverlap(Collider_Right)
  (params (OverlappedComponent :type Primitive%20Component%20Object%20Reference) (OtherActor :type Actor%20Object%20Reference) (OtherComp :type Primitive%20Component%20Object%20Reference) (OtherBodyIndex :type Integer) (bFromSweep :type Boolean) (SweepResult :type Hit%20Result%20Structure%20%28by%20ref%29)))

(event OnComponentBeginOverlap(Collider_Top)
  (params (OverlappedComponent :type Primitive%20Component%20Object%20Reference) (OtherActor :type Actor%20Object%20Reference) (OtherComp :type Primitive%20Component%20Object%20Reference) (OtherBodyIndex :type Integer) (bFromSweep :type Boolean) (SweepResult :type Hit%20Result%20Structure%20%28by%20ref%29)))

(event OnComponentBeginOverlap(Collider_Bottom)
  (params (OverlappedComponent :type Primitive%20Component%20Object%20Reference) (OtherActor :type Actor%20Object%20Reference) (OtherComp :type Primitive%20Component%20Object%20Reference) (OtherBodyIndex :type Integer) (bFromSweep :type Boolean) (SweepResult :type Hit%20Result%20Structure%20%28by%20ref%29)))

(event OnComponentBeginOverlap(Collider_Center)
  (params (OverlappedComponent :type Primitive%20Component%20Object%20Reference) (OtherActor :type Actor%20Object%20Reference) (OtherComp :type Primitive%20Component%20Object%20Reference) (OtherBodyIndex :type Integer) (bFromSweep :type Boolean) (SweepResult :type Hit%20Result%20Structure%20%28by%20ref%29)))

(fn ConstructionScript)