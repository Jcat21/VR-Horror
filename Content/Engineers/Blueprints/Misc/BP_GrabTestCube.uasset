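; BP_GrabTestCube is a test cube that a BP_MagnetKey can drag around.
; Overlapping a magnet key stores a reference to it and sets an interaction flag, which is never cleared here.
; Each tick, while the key is on and its trigger overlaps the mesh, the mesh snaps in front of the key, keeping its own height and copying only the key's yaw.
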(event EventBeginPlay)

(event EventTick
  (params (DeltaSeconds :type Float%20%28single-precision%29))
  (bind _magnetkeyref (Variables|Default|GetmagnetKeyRef))
  (bind _magnetkeyref_2 (Variables|Default|GetmagnetKeyRef))
  (bind _magnetkeyref_3 (Variables|Default|GetmagnetKeyRef))
  (bind _returnvalue (Transformation|GetActorForwardVector _magnetkeyref_3))
  (bind _returnvalue_2 (Transformation|GetActorLocation _magnetkeyref_2))
  (bind _returnvalue_3 (* _returnvalue 1e+02))
  (bind _returnvalue_4 (+ _returnvalue_2 _returnvalue_3))
  (bind (_x _y) (Math|Vector|BreakVector _returnvalue_4))
  (if (and (Utilities|IsValid _magnetkeyref) (Variables|Default|GetisInteracting))
    (if (and (Variables|/Game/Engineers/Blueprints/Parents/BP_MagnetKey.BP_MagnetKey_C|GetisOn _magnetkeyref) (Class|PrimitiveComponent|IsOverlappingComponent (Variables|/Game/Engineers/Blueprints/Parents/BP_MagnetKey.BP_MagnetKey_C|GetMagnetTrigger _magnetkeyref) (Variables|Debug|GetStaticMeshComponent)))
      (Transformation|SetWorldLocationAndRotation (Variables|Debug|GetStaticMeshComponent) (Math|Vector|MakeVector _x _y (.Z (Math|Vector|BreakVector (Transformation|GetWorldLocation (Variables|Debug|GetStaticMeshComponent))))) (Math|Rotator|MakeRotator 0.0 0.0 (.Yaw (Math|Rotator|BreakRotator (Transformation|GetActorRotation (Variables|Default|GetmagnetKeyRef))))) false false))))

(event Collision|EventActorBeginOverlap
  (params (OtherActor :type Actor%20Object%20Reference))
  (bind _asbp_magnet_key (Utilities|Casting|CastToBP_MagnetKey OtherActor))
  (Variables|Default|SetisInteracting true)
  (Variables|Default|SetmagnetKeyRef _asbp_magnet_key))

(fn ConstructionScript)