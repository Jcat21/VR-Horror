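; BP_DoorCryoCorridor is a two-panel sliding door that opens once when the main pawn enters its trigger.
; If the door is enabled, the first overlap starts the opening, plays audio and destroys an invisible wall.
; Tick then eases both panels toward their configured offsets with VInterpTo.
; A separate OpenDoor function shifts the panels instantly with a 2D sound and is not called within this Blueprint.
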(event OnComponentBeginOverlap(r)
  (params (OverlappedComponent :type Primitive%20Component%20Object%20Reference) (OtherActor :type Actor%20Object%20Reference) (OtherComp :type Primitive%20Component%20Object%20Reference) (OtherBodyIndex :type Integer) (bFromSweep :type Boolean) (SweepResult :type Hit%20Result%20Structure%20%28by%20ref%29))
  (Utilities|Casting|CastToBP_MainPawn OtherActor)
  (if (Variables|Default|GetDoorEnabled)
    (Utilities|FlowControl|DoOnce false
      (:Completed
        (Variables|Default|SetIsOpening true)
        (Audio|Components|Audio|Play (Variables|Default|GetAudio) 0.0)
        (Actor|DestroyActor (Variables|Default|GetInvisibleWall))))))

(event EventTick
  (params (DeltaSeconds :type Float%20%28single-precision%29))
  (bind _door_l (Variables|Default|GetDoor_L))
  (bind _door_r (Variables|Default|GetDoor_R))
  (if (and (Variables|Default|GetIsOpening) (Variables|Default|GetDoorEnabled))
    (Transformation|SetRelativeLocation _door_r (Math|Interpolation|VInterpTo (Variables|/Script/Engine.SceneComponent|GetRelativeLocation _door_r) (Math|Vector|MakeVector (Variables|Default|GetRightDoorOffset) 0.0 0.0) DeltaSeconds (Variables|Default|GetDoorSpeed)) false false)
    (Transformation|SetRelativeLocation _door_l (Math|Interpolation|VInterpTo (Variables|/Script/Engine.SceneComponent|GetRelativeLocation _door_l) (Math|Vector|MakeVector (Variables|Default|GetLeftDoorOffset) 0.0 0.0) DeltaSeconds (Variables|Default|GetDoorSpeed)) false false)))

(fn ConstructionScript)

(fn OpenDoor
  (Transformation|AddLocalOffset (Variables|Default|GetDoor_R) "-320.000000, 0, 0" false false)
  (Audio|PlaySound2D "/Game/Artists/Audio/Sounds/drawer_ascend.drawer_ascend")
  (Transformation|AddLocalOffset (Variables|Default|GetDoor_L) "200.000000, 0, 0" false false))