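; Timed claw-crane minigame in which the player positions a crane to grab a cryo pod.
; Fully charging the buttons enables two movement sliders and starts a countdown on the control station.
; At timeout the pipe descends, attaches any overlapped pod, then rises and travels to a drop point through frame-delay loops.
; A held pod is released with physics; otherwise the screen fades, the player teleports to quarantine and CraneGame unloads.
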(event OnComponentBeginOverlap(CraneCollider)
  (params (OverlappedComponent :type Primitive%20Component%20Object%20Reference) (OtherActor :type Actor%20Object%20Reference) (OtherComp :type Primitive%20Component%20Object%20Reference) (OtherBodyIndex :type Integer) (bFromSweep :type Boolean) (SweepResult :type Hit%20Result%20Structure%20%28by%20ref%29))
  (bind _asbp_cryo_pod (Utilities|Casting|CastToBP_CryoPod OtherActor))
  (if (not (Variables|Default|GetisHoldingCryoPod))
    (Variables|Default|SetisHoldingCryoPod true)
    (bind _output_get (Variables|Default|SetheldCryoPod _asbp_cryo_pod))
    (Transformation|AttachComponentToComponent _output_get (Variables|Default|GetCranePipe) "None" "KeepWorld" "KeepWorld" "KeepWorld" true)))

(event Custom|DecrementTimer
  (bind _timeremaining (Variables|Default|GetTimeRemaining))
  (if (> (Variables|Default|GetTimeRemaining) 0)
    (Math|Integer|DecrementInt _timeremaining
      (:%20%20
        (Rendering|Components|TextRender|SetText (Variables|/Game/Engineers/Blueprints/Parents/BP_ControlStation.BP_ControlStation_C|GetTimer (Variables|Default|GetCraneControlStation)) (Utilities|Text|ToText(Integer) _timeremaining))))
    (else
      (Utilities|Time|ClearandInvalidateTimerbyHandle (stale Custom|StartGame _returnvalue)))))

(event Custom|StartGame
  (bind _inwardslider (Variables|Default|GetInwardSlider))
  (bind _horizontalslider (Variables|Default|GetHorizontalSlider))
  (Utilities|FlowControl|Sequence
    (:then_0
      (Variables|/Game/Engineers/Blueprints/Children/BP_SliderRailCrane.BP_SliderRailCrane_C|SetcontrolsEnabled _inwardslider true)
      (Rendering|Material|SetMaterial (Variables|/Game/Engineers/Blueprints/Children/BP_SliderRailCrane.BP_SliderRailCrane_C|GetBall _inwardslider) 0 "/Game/Artists/Materials/M_RightMagnetKeyTurnedON.M_RightMagnetKeyTurnedON")
      (Variables|/Game/Engineers/Blueprints/Children/BP_SliderRailCrane.BP_SliderRailCrane_C|SetcontrolsEnabled _horizontalslider true)
      (Rendering|Material|SetMaterial (Variables|/Game/Engineers/Blueprints/Children/BP_SliderRailCrane.BP_SliderRailCrane_C|GetBall _horizontalslider) 0 "/Game/Artists/Materials/M_LeftMagnetKeyTurnedON.M_LeftMagnetKeyTurnedON"))
    (:then_1
      (bind _returnvalue (Utilities|Time|SetTimerbyEvent (delegate Custom|DecrementTimer) 1.0 true)))
    (:then_2
      (Utilities|Time|SetTimerbyEvent (delegate Custom|DropCrane) (Math|Conversions|ToFloat(Integer) (Variables|Default|GetTimeToPlay))))))

(event Custom|DropCrane
  (bind _returnvalue (Transformation|GetActorLocation))
  (bind _returnvalue_2 (Utilities|Time|GetWorldDeltaSeconds))
  (bind _returnvalue_3 (Utilities|Time|GetWorldDeltaSeconds))
  (bind _playerref (Variables|Default|GetPlayerRef))
  (bind _crane_movement_horizontal (Variables|Default|GetCrane_Movement_Horizontal))
  (bind _crane_movement_inward (Variables|Default|GetCrane_Movement_Inward))
  (bind _cranepipe (Variables|Default|GetCranePipe))
  (bind _cranetop (Variables|Default|GetCraneTop))
  (bind _cranetop_2 (Variables|Default|GetCraneTop))
  (bind _relativelocation (Variables|/Script/Engine.SceneComponent|GetRelativeLocation _cranetop_2))
  (bind _returnvalue_4 (- (.y _relativelocation) (.y _returnvalue)))
  (Utilities|FlowControl|Sequence
    (:then_0
      (Variables|/Game/Engineers/Blueprints/Children/BP_SliderRailCrane.BP_SliderRailCrane_C|SetcontrolsEnabled (Variables|Default|GetHorizontalSlider) false)
      (Variables|/Game/Engineers/Blueprints/Children/BP_SliderRailCrane.BP_SliderRailCrane_C|SetcontrolsEnabled (Variables|Default|GetInwardSlider) false)
      (Class|PrimitiveComponent|SetAllPhysicsLinearVelocity (Variables|Default|GetCraneTop) "0, 0, 0" false))
    (:then_1
      (Audio|Components|Audio|Play (Variables|Default|GetCrane_NoItem) 0.0)
      (if (and (>= (.z (Variables|/Script/Engine.SceneComponent|GetRelativeLocation (Variables|Default|GetCranePipe))) -1.2e+03) (not (Variables|Default|GetisHoldingCryoPod))) :!label _label
        (Utilities|FlowControl|Delay _returnvalue_3)
        (Transformation|AddLocalOffset _cranepipe (Math|Vector|MakeVector 0.0 0.0 -6.0) true false)
        (goto _label)
        (else
          (Utilities|FlowControl|Delay 1.5)
          (if (Variables|Default|GetisHoldingCryoPod)
            (Audio|Components|Audio|Play (Variables|Default|GetCrane_Item) 0.0)
            (else
              (Audio|Components|Audio|Play (Variables|Default|GetCrane_NoItem) 0.0)))
          (if (<= (.z (Variables|/Script/Engine.SceneComponent|GetRelativeLocation (Variables|Default|GetCranePipe))) 5e+02) :!label _label_2
            (Utilities|FlowControl|Delay _returnvalue_3)
            (if (Variables|Default|GetisHoldingCryoPod)
              (Transformation|AddLocalOffset _cranepipe (Math|Vector|MakeVector 0.0 0.0 2.0) false false)
              (goto _label_2)
              (else
                (Transformation|AddLocalOffset _cranepipe (Math|Vector|MakeVector 0.0 0.0 6.0) false false)
                (goto _label_2)))
            (else
              (Utilities|FlowControl|Delay 0.5)
              (Audio|Components|Audio|FadeIn _crane_movement_horizontal 0.1 1.0 0.0 :!class /Script/Engine.AudioComponent)
              (if (<= _returnvalue_4 5e+02) :!label _label_3
                (Utilities|FlowControl|Delay (Utilities|Time|GetWorldDeltaSeconds))
                (Transformation|AddLocalOffset (Variables|Default|GetCraneTop) (Math|Vector|MakeVector 0.0 2.0 0.0) false false)
                (goto _label_3)
                (else
                  (if (>= _returnvalue_4 5e+02) :!label _label_4
                    (Utilities|FlowControl|Delay _returnvalue_2)
                    (Transformation|AddLocalOffset _cranetop (Math|Vector|MakeVector 0.0 -2.0 0.0) false false)
                    (goto _label_4)
                    (else
                      (Audio|Components|Audio|FadeOut _crane_movement_horizontal 0.1 0.0 :!class /Script/Engine.AudioComponent)
                      (Utilities|FlowControl|Delay 0.5)
                      (Audio|Components|Audio|FadeIn _crane_movement_inward 0.1 1.0 0.0 :!class /Script/Engine.AudioComponent)
                      (if (<= (- (.x (Variables|/Script/Engine.SceneComponent|GetRelativeLocation (Variables|Default|GetCraneTop))) (.x (Transformation|GetActorLocation))) 2.07e+03) :!label _label_5
                        (Utilities|FlowControl|Delay _returnvalue_2)
                        (Transformation|AddLocalOffset _cranetop (Math|Vector|MakeVector 4.0 0.0 0.0) false false)
                        (Transformation|AddLocalOffset (Variables|Default|GetMiddleRail) "4.000000, 0, 0" false false)
                        (goto _label_5)
                        (else
                          (Audio|Components|Audio|FadeOut _crane_movement_inward 0.1 0.0 :!class /Script/Engine.AudioComponent)
                          (Utilities|FlowControl|Delay 1.0)
                          (Utilities|FlowControl|Sequence
                            (:then_0
                              (if (Variables|Default|GetisHoldingCryoPod)
                                (Transformation|DetachFromActor (Variables|Default|GetheldCryoPod) "KeepWorld" "KeepWorld" "KeepWorld")
                                (Rendering|Material|SetMaterial (Variables|/Game/Engineers/Blueprints/Misc/BP_CryoPod.BP_CryoPod_C|GetCube (Variables|Default|GetheldCryoPod)) 1 "/Game/Artists/Materials/buttonLight_BLUE.buttonLight_BLUE")
                                (Physics|SetSimulatePhysics (Variables|/Game/Engineers/Blueprints/Misc/BP_CryoPod.BP_CryoPod_C|GetCube (Variables|Default|GetheldCryoPod)) true)
                                (Variables|Default|SetheldCryoPod 0)
                                (Variables|Default|SetisHoldingCryoPod false)
                                (else
                                  (CameraFades|StartCameraFade (Game|GetPlayerCameraManager 0) 0.0 1.0 5.0 "(R=1.000000,G=0.000000,B=0.000000,A=1.000000)" true true)
                                  (Utilities|FlowControl|Delay 5.0)
                                  (Default|SetNewTeleportLocs _playerref)
                                  (bind (_spawn _found_) (Default|FindTeleportLoc _playerref "QuarantineLoc"))
                                  (if _found_
                                    (Transformation|SetActorLocationAndRotation _playerref (.location (Transformation|GetActorTransform _spawn)) (.rotation (Transformation|GetActorTransform _spawn)) false true)
                                    (Default|ResetPlayerHeight _playerref)
                                    (CameraFades|StartCameraFade (Game|GetPlayerCameraManager 0) 1.0 0.0 5.0 "(R=1.000000,G=0.000000,B=0.000000,A=1.000000)" false false)
                                    (Game|UnloadStreamLevel(byName) "CraneGame")))))))))))))))))))

(event EventBeginPlay
  (Variables|Default|SetTimeRemaining (Variables|Default|GetTimeToPlay))
  (Rendering|Components|TextRender|SetText (Variables|/Game/Engineers/Blueprints/Parents/BP_ControlStation.BP_ControlStation_C|GetTimer (Variables|Default|GetCraneControlStation)) (Utilities|Text|ToText(Integer) 0))
  (EventDispatchers|BindEventtoHitFullCharge (Variables|Default|GetChargeButtons) (delegate Custom|StartGame))
  (bind _asbp_main_pawn (Utilities|Casting|CastToBP_MainPawn (Game|Player|GetPlayerPawn 0)))
  (Variables|Default|SetPlayerRef _asbp_main_pawn))

(event EventTick
  (params (DeltaSeconds :type Float%20%28single-precision%29))
  (bind _cranebottom (Variables|Default|GetCraneBottom))
  (bind _returnvalue (Transformation|GetWorldLocation _cranebottom))
  (bind (_x _y _z) (Math|Vector|BreakVector _returnvalue))
  (if (Variables|/Game/Engineers/Blueprints/Children/BP_SliderRailCrane.BP_SliderRailCrane_C|GetcontrolsEnabled (Variables|Default|GetInwardSlider))
    (Collision|LineTraceByChannel _returnvalue (Math|Vector|MakeVector _x _y (- _z 1e+05)) "TraceTypeQuery1" false 0 "ForOneFrame")))

(fn ConstructionScript)