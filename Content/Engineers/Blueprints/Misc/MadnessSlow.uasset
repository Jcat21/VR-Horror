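; MadnessSlow is a Blueprint that drains the player pawn's madness level according to proximity to a detection point.
; On BeginPlay it caches player 0 as a BP_MainPawn.
; DepleteMadness subtracts a base amount plus a rate divided by the VR camera's distance to the given center, so depletion grows as the camera nears it.
; Nothing in this Blueprint calls DepleteMadness, and its StartPosition input is unused.
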(event EventBeginPlay
  (bind _asbp_main_pawn (Utilities|Casting|CastToBP_MainPawn (Game|Player|GetPlayerPawn 0)))
  (Variables|Default|SetPlayerPawn _asbp_main_pawn))

(event EventTick
  (params (DeltaSeconds :type Float%20%28single-precision%29)))

(fn DepleteMadness
  (params (DetectionCenter :type Vector) (StartPosition :type Vector))
  (bind _playerpawn (Variables|Default|GetPlayerPawn))
  (Variables|/Game/Engineers/Blueprints/Parents/BP_MainPawn.BP_MainPawn_C|SetMadnessLevel _playerpawn (- (Variables|/Game/Engineers/Blueprints/Parents/BP_MainPawn.BP_MainPawn_C|GetMadnessLevel _playerpawn) (+ (/ (Variables|Default|GetDepleteRate) (Math|Vector|VectorLength (- DetectionCenter (Transformation|GetWorldLocation (Components|GetChildComponent (Variables|/Game/Engineers/Blueprints/Parents/BP_MainPawn.BP_MainPawn_C|GetVROrigin (Variables|Default|GetPlayerPawn)) 0))))) (Variables|Default|GetInitialDeplete)))))