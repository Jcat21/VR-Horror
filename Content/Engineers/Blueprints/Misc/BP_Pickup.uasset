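; BP_Pickup is an object whose Cube is carried by a magnet key.
; Overlapping a BP_MagnetKey starts interaction; while the key is on, Tick sweeps the Cube in front of it and arms ReadyToDon, until TurnedOff releases it.
; A second Tick branch moves the armed Cube once before the pawn camera after a pawn hit and capsule overlap.
; That branch stays inactive here because the MainPawnRef assignment is unconnected.
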(event Custom|TurnOffMagnet
  (Variables|Default|SetisInteracting false)
  (EventDispatchers|UnbindEventfromTurnedOff (Variables|Default|GetmagkeyReference) (delegate Custom|TurnOffMagnet)))

(event EventTick
  (params (DeltaSeconds :type Float%20%28single-precision%29))
  (bind _magkeyreference (Variables|Default|GetmagkeyReference))
  (bind _magkeyreference_2 (Variables|Default|GetmagkeyReference))
  (bind _mainpawnref (Variables|Default|GetmainPawnRef))
  (bind _magkeyreference_3 (Variables|Default|GetmagkeyReference))
  (bind _returnvalue (Transformation|GetActorForwardVector _magkeyreference_3))
  (bind _returnvalue_2 (Transformation|GetActorLocation _magkeyreference_2))
  (bind _returnvalue_3 (* _returnvalue 5e+01))
  (bind _returnvalue_4 (+ _returnvalue_2 _returnvalue_3))
  (bind (_x _y _z) (Math|Vector|BreakVector _returnvalue_4))
  (Utilities|FlowControl|Sequence
    (:then_0
      (if (and (Utilities|IsValid _magkeyreference) (Variables|Default|GetisInteracting))
        (if (Variables|/Game/Engineers/Blueprints/Parents/BP_MagnetKey.BP_MagnetKey_C|GetisOn _magkeyreference)
          (Transformation|SetWorldLocationAndRotation (Variables|Default|GetCube) (Math|Vector|MakeVector _x _y _z) (Transformation|GetActorRotation (Variables|Default|GetmagkeyReference)) true false)
          (Variables|Default|SetreadyToDon true))))
    (:then_1
      (if (and (Variables|Default|GetisInteractingwithPawn) (Utilities|IsValid _mainpawnref))
        (if (and (Variables|Default|GetreadyToDon) (Class|PrimitiveComponent|IsOverlappingComponent (Variables|/Game/Engineers/Blueprints/Parents/BP_MainPawn.BP_MainPawn_C|GetCapsule _mainpawnref) (Variables|Default|GetCube)))
          (Transformation|SetWorldLocationAndRotation (Variables|Default|GetCube) (+ (Transformation|GetWorldLocation (Variables|/Game/Engineers/Blueprints/Parents/BP_MainPawn.BP_MainPawn_C|GetCamera (Variables|Default|GetmainPawnRef))) (* (Math|Vector|GetForwardVector (Variables|/Game/Engineers/Blueprints/Parents/BP_MainPawn.BP_MainPawn_C|GetCamera (Variables|Default|GetmainPawnRef))) 1e+02)) (Transformation|GetSocketRotation (Variables|/Game/Engineers/Blueprints/Parents/BP_MainPawn.BP_MainPawn_C|GetCamera (Variables|Default|GetmainPawnRef)) "None") true false)
          (Variables|Default|SetreadyToDon false))))))

(event Collision|EventActorBeginOverlap
  (params (OtherActor :type Actor%20Object%20Reference))
  (bind _asbp_magnet_key (Utilities|Casting|CastToBP_MagnetKey OtherActor))
  (Variables|Default|SetisInteracting true)
  (bind _output_get (Variables|Default|SetmagkeyReference _asbp_magnet_key))
  (EventDispatchers|BindEventtoTurnedOff _output_get (delegate Custom|TurnOffMagnet)))

(event Collision|EventHit
  (params (MyComp :type Primitive%20Component%20Object%20Reference) (Other :type Actor%20Object%20Reference) (OtherComp :type Primitive%20Component%20Object%20Reference) (bSelfMoved :type Boolean) (HitLocation :type Vector :default "0, 0, 0") (HitNormal :type Vector :default "0, 0, 0") (NormalImpulse :type Vector :default "0, 0, 0") (Hit :type Hit%20Result%20Structure%20%28by%20ref%29))
  (bind _asbp_main_pawn (Utilities|Casting|CastToBP_MainPawn Other))
  (Variables|Default|SetisInteractingwithPawn true))

(fn ConstructionScript)