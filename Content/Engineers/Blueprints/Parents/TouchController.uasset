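; Oculus Touch motion controller for VR that drives one hand's HandActor and sets the left or right controller mesh and AnimBP.
; Tick copies input axes to animation values, derives finger curl, feeds thumbstick angle into teleport rotation, and shows or hides the hand with input focus.
; Trigger, face buttons and grip, filtered by hand, drive index, thumb and grab actions.
; Right thumbstick toggles teleport; Special Right toggles the pawn's laser.
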(event EventSetControllerType
  (params (New%20Type :type EControllerHand%20Enum :default "Left"))
  (bind _controller (Variables|Default|GetController))
  (|CallParentFunction New%20Type)
  (switch Utilities|FlowControl|Switch|SwitchonEControllerHand New%20Type
    (:Left
      (Class|SkinnedMeshComponent|SetSkeletalMesh _controller "/Game/Artists/Models/HandModel(Inport)/left_touch_controller_model_skel.left_touch_controller_model_skel" true)
      (Components|SkeletalMesh|SetAnimInstanceClass _controller "/Game/Artists/Models/HandModel(Inport)/LeftTouchAnimBP.LeftTouchAnimBP_C"))
    (:Right
      (Class|SkinnedMeshComponent|SetSkeletalMesh _controller "/Game/Artists/Models/HandModel(Inport)/right_touch_controller_model_skel.right_touch_controller_model_skel" true)
      (Components|SkeletalMesh|SetAnimInstanceClass _controller "/Game/Artists/Models/HandModel(Inport)/RightTouchAnimBP.RightTouchAnimBP_C"))))

(event EventTick
  (params (DeltaSeconds :type Float%20%28single-precision%29))
  (bind _returnvalue (Class|OculusFunctionLibrary|HasInputFocus))
  (bind _handactor (Variables|Default|GetHandActor))
  (|CallParentFunction DeltaSeconds)
  (Utilities|FlowControl|Sequence
    (:then_0
      (CallFunction|UpdateAnimationValues)
      (CallFunction|UpdateHandAnimations)
      (CallFunction|UpdateTeleportRotation))
    (:then_1
      (if (Math|Boolean|NotEqual(Boolean) (Variables|Default|GetInputFocus) _returnvalue)
        (bind _output_get (Variables|Default|SetInputFocus _returnvalue))
        (if _output_get
          (Default|ActivateHand _handactor)
          (else
            (Rendering|SetActorHiddenInGame true)
            (Default|DeactivateHand _handactor)))))))

(event EventBeginPlay
  (Input|EnableInput (Game|GetPlayerController 0)))

(event Input|TouchEvents|OculusTouchRightThumbstick
  (params (AxisValue :type Float%20%28single-precision%29))
  (if (Math|Boolean|ANDBoolean (<= AxisValue 0.2) (Default|IsTeleportActive (Variables|Default|GetHandActor)) (Utilities|Enum|Equal(Enum) (Variables|Default|GetHand) "Right") (< (Math|Float|Absolute(Float) (Class|Actor|GetInputAxisKeyValue)) 0.3) (< (Math|Float|Absolute(Float) (Class|Actor|GetInputAxisKeyValue)) 0.3))
    (Default|DeactivateTeleport (Variables|Default|GetHandActor))))

(event Input|KeyboardEvents|MotionControllerRightThumbstickY
  (params (AxisValue :type Float%20%28single-precision%29))
  (if (Math|Boolean|ANDBoolean (<= AxisValue -0.6) (not (Default|IsTeleportActive (Variables|Default|GetHandActor))) (Utilities|Enum|Equal(Enum) (Variables|Default|GetHand) "Right"))
    (Default|ActivateTeleport (Variables|Default|GetHandActor))))

(event Input|GamepadEvents|GamepadSpecialRight
  (params (Key :type Key%20Structure))
  (:Pressed
    (Default|ToggleLaser (Variables|/Game/Engineers/Blueprints/Parents/HandBP.HandBP_C|GetMyPawn (Variables|Default|GetHandActor)))))

(event Input|KeyboardEvents|MotionControllerRightTrigger
  (params (Key :type Key%20Structure))
  (bind _hand (Variables|Default|GetHand))
  (bind _handactor (Variables|Default|GetHandActor))
  (bind _returnvalue (Utilities|Enum|Equal(Enum) _hand "Right"))
  (:Pressed
    (if _returnvalue
      (Default|IndexAction _handactor)))
  (:Released
    (if _returnvalue
      (Default|IndexActionEnd _handactor))))

(event Input|KeyboardEvents|MotionControllerLeftGrip1
  (params (Key :type Key%20Structure))
  (bind _hand (Variables|Default|GetHand))
  (bind _handactor (Variables|Default|GetHandActor))
  (bind _returnvalue (Utilities|Enum|Equal(Enum) _hand "Left"))
  (:Pressed
    (if _returnvalue
      (Default|AttemptGrab _handactor)))
  (:Released
    (if _returnvalue
      (Default|Release _handactor))))

(event Input|KeyboardEvents|MotionControllerLeftTrigger
  (params (Key :type Key%20Structure))
  (bind _handactor (Variables|Default|GetHandActor))
  (bind _hand (Variables|Default|GetHand))
  (bind _returnvalue (Utilities|Enum|Equal(Enum) _hand "Left"))
  (:Pressed
    (if _returnvalue
      (Default|IndexAction _handactor)))
  (:Released
    (if _returnvalue
      (Default|IndexActionEnd _handactor))))

(event Input|KeyboardEvents|MotionControllerRightGrip1
  (params (Key :type Key%20Structure))
  (bind _hand (Variables|Default|GetHand))
  (bind _handactor (Variables|Default|GetHandActor))
  (bind _returnvalue (Utilities|Enum|Equal(Enum) _hand "Right"))
  (:Pressed
    (if _returnvalue
      (Default|AttemptGrab _handactor)))
  (:Released
    (if _returnvalue
      (Default|Release _handactor))))

(event Input|KeyboardEvents|MotionControllerRightFaceButton1
  (params (Key :type Key%20Structure))
  (bind _handactor (Variables|Default|GetHandActor))
  (bind _hand (Variables|Default|GetHand))
  (bind _returnvalue (Utilities|Enum|Equal(Enum) _hand "Right"))
  (:Pressed
    (if _returnvalue
      (Default|ThumbAction _handactor)))
  (:Released
    (if _returnvalue
      (Default|ThumbActionEnd _handactor))))

(event Input|KeyboardEvents|MotionControllerLeftFaceButton1
  (params (Key :type Key%20Structure))
  (bind _handactor (Variables|Default|GetHandActor))
  (bind _hand (Variables|Default|GetHand))
  (bind _returnvalue (Utilities|Enum|Equal(Enum) _hand "Left"))
  (:Pressed
    (if _returnvalue
      (Default|ThumbAction _handactor)))
  (:Released
    (if _returnvalue
      (Default|ThumbActionEnd _handactor))))

(event Input|KeyboardEvents|MotionControllerRightFaceButton2
  (params (Key :type Key%20Structure))
  (bind _handactor (Variables|Default|GetHandActor))
  (bind _hand (Variables|Default|GetHand))
  (bind _returnvalue (Utilities|Enum|Equal(Enum) _hand "Right"))
  (:Pressed
    (if _returnvalue
      (Default|ThumbAction _handactor)))
  (:Released
    (if _returnvalue
      (Default|ThumbActionEnd _handactor))))

(event Input|KeyboardEvents|MotionControllerLeftFaceButton2
  (params (Key :type Key%20Structure))
  (bind _handactor (Variables|Default|GetHandActor))
  (bind _hand (Variables|Default|GetHand))
  (bind _returnvalue (Utilities|Enum|Equal(Enum) _hand "Left"))
  (:Pressed
    (if _returnvalue
      (Default|ThumbAction _handactor)))
  (:Released
    (if _returnvalue
      (Default|ThumbActionEnd _handactor))))

(fn ConstructionScript
  (|CallParentFunction))

(fn UpdateAnimationValues
  (switch Utilities|FlowControl|Switch|SwitchonEControllerHand (Variables|Default|GetHand)
    (:Left
      (Variables|Default|SetThumbstickX (Class|Actor|GetInputAxisKeyValue))
      (Variables|Default|SetThumbstickY (Class|Actor|GetInputAxisKeyValue))
      (Variables|Default|SetTriggerAxis (Class|Actor|GetInputAxisKeyValue))
      (Variables|Default|SetGripAxis (Class|Actor|GetInputAxisKeyValue)))
    (:Right
      (Variables|Default|SetThumbstickX (Class|Actor|GetInputAxisKeyValue))
      (Variables|Default|SetThumbstickY (Class|Actor|GetInputAxisKeyValue))
      (Variables|Default|SetTriggerAxis (Class|Actor|GetInputAxisKeyValue))
      (Variables|Default|SetGripAxis (Class|Actor|GetInputAxisKeyValue)))))

(fn UpdateHandAnimations
  (bind _returnvalue (Class|Actor|GetInputAxisKeyValue))
  (bind _returnvalue_2 (Class|Actor|GetInputAxisKeyValue))
  (bind _returnvalue_3 (- 1.0 _returnvalue_2))
  (bind _returnvalue_4 (- 1.0 _returnvalue))
  (bind _returnvalue_5 (* _returnvalue_3 0.75))
  (bind _returnvalue_6 (* _returnvalue_4 0.75))
  (switch Utilities|FlowControl|Switch|SwitchonEControllerHand (Variables|Default|GetHand)
    (:Left
      (Default|UpdateHandAnimation (Variables|Default|GetHandActor) (Math|Float|Clamp(Float) (Class|Actor|GetInputAxisKeyValue) (Math|Float|Clamp(Float) _returnvalue_6 0.0 0.5)) (Math|Float|Clamp(Float) (Class|Actor|GetInputAxisKeyValue) _returnvalue_6) _returnvalue_6 _returnvalue_6 _returnvalue_6))
    (:Right
      (Default|UpdateHandAnimation (Variables|Default|GetHandActor) (Math|Float|Clamp(Float) (Class|Actor|GetInputAxisKeyValue) (Math|Float|Clamp(Float) _returnvalue_5 0.0 0.5)) (Math|Float|Clamp(Float) (Class|Actor|GetInputAxisKeyValue) _returnvalue_5) _returnvalue_5 _returnvalue_5 _returnvalue_5))))

(fn UpdateTeleportRotation
  (bind _hand (Variables|Default|GetHand))
  (bind _returnvalue (Utilities|Enum|Equal(Enum) _hand "Right"))
  (if (or (Utilities|Enum|Equal(Enum) _hand "Left") _returnvalue)
    (Default|AddTeleportRotation (Variables|Default|GetHandActor) (select _returnvalue (Class|KismetMathLibrary|DegAtan2 (Class|Actor|GetInputAxisKeyValue) (* (Class|Actor|GetInputAxisKeyValue) -1.0)) (Class|KismetMathLibrary|DegAtan2 (Class|Actor|GetInputAxisKeyValue) (* (Class|Actor|GetInputAxisKeyValue) -1.0))))))