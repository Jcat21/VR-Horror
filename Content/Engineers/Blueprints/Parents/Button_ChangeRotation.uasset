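; VR button that toggles the pawn between snap and smooth rotation and updates its caption.
; An overlapping index-finger collider pushes the inner mesh along the frame's local Y, scaling glow and haptics until full press; laser interaction also triggers it.
; Triggering plays a sound, starts a brief input cooldown and runs a glow timeline, which toggles the mode when finished.
; The construction script applies size meshes, icon, colors and initial caption.
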(event Custom|Laser%20Call
  (params (instigator :type Hand%20BP%20Object%20Reference))
  ;[1 1 1] Called by laser
  (if (not (> (Variables|Default|GetIgnoreTime) 0.0))
    (CallFunction|Triggered)
    (Class|PlayerController|PlayHapticEffect (Game|GetPlayerController 0) "/Game/Misc/HapticEvents/ButtonClick.ButtonClick" (Variables|/Game/Engineers/Blueprints/Parents/HandBP.HandBP_C|GetHandType instigator) 1.0 false)))

(event Custom|Triggered
  ;[1 1 1] Called
  (Audio|PlaySoundatLocation "/Engine/VREditor/Sounds/UI/Click_on_Button.Click_on_Button" (Transformation|GetActorLocation))
  (Default|CallTrigger)
  (Utilities|IsValid self ; In some cases, button may become invalid after trigger - destroyed
    (:Is%20Valid
      (Variables|Default|SetIgnoreTime 0.35)
      (bind _intensity (Timeline|Timeline_0 PlayFromStart)
        (:Update
          (Rendering|Material|SetScalarParameterValueonMaterials (Variables|Default|GetOutside) "Intensity" _intensity)
          (Variables|Default|SetAnimationRunning true))
        (:Finished
          (Transformation|SetRelativeLocation (Variables|Default|GetInside) (Math|Vector|MakeVector 0.0 (Variables|Default|GetDefaultDistance) 0.0) false false)
          (Variables|Default|SetAnimationRunning false)
          (bind _asvrpawn (Utilities|Casting|CastToVRPawn (Game|Player|GetPlayerPawn 0)))
          (if (Variables|/Game/Engineers/Blueprints/Parents/VRPawn.VRPawn_C|GetSnap%20Rotation%20ON _asvrpawn)
            (Variables|/Game/Engineers/Blueprints/Parents/VRPawn.VRPawn_C|SetSnap%20Rotation%20ON _asvrpawn false)
            (CallFunction|SetCaption "ROTATION MODE: SMOOTH")
            (else
              (Variables|/Game/Engineers/Blueprints/Parents/VRPawn.VRPawn_C|SetSnap%20Rotation%20ON _asvrpawn true)
              (CallFunction|SetCaption "ROTATION MODE: SNAP"))))))))

(event Collision|EventActorBeginOverlap
  (params (OtherActor :type Actor%20Object%20Reference))
  ;[1 1 1] Add new collider
  (if (not (> (Variables|Default|GetIgnoreTime) 0.0))
    (bind _asindex_collider (Utilities|Casting|CastToIndexCollider OtherActor))
    (Default|CallFocusGain)
    (Variables|Default|SetOverlapping%20Collider _asindex_collider)))

(event EventTick
  (params (DeltaSeconds :type Float%20%28single-precision%29))
  (bind _defaultdistance (Variables|Default|GetDefaultDistance))
  (bind _inside (Variables|Default|GetInside))
  ;[1 1 1] Adjust ignore time
  (Variables|Default|SetIgnoreTime (Math|Float|Max(Float) (- (Variables|Default|GetIgnoreTime) DeltaSeconds) 0.0))
  (Utilities|IsValid (Variables|Default|GetOverlapping%20Collider)
    (:Is%20Valid
      ;[1 1 1] Process activation related to index finger activity
      (Transformation|SetRelativeRotation _inside "180.000000,0.000000, 0" false false)
      (Variables|Default|SetProgress (- 1.0 (/ (Math|Float|Clamp(Float) (.Y (Math|Vector|BreakVector (Math|Transform|InverseTransformLocation (Transformation|GetWorldTransform (Variables|Default|GetOutside)) (Transformation|GetWorldLocation (Variables|/Game/Engineers/Blueprints/Parents/IndexCollider.IndexCollider_C|GetSphere (Variables|Default|GetOverlapping%20Collider)))))) 0.0 _defaultdistance) _defaultdistance)))
      (Transformation|SetRelativeLocation _inside (Math|Vector|MakeVector 0.0 (Math|Float|Clamp(Float) (.Y (Math|Vector|BreakVector (Math|Transform|InverseTransformLocation (Transformation|GetWorldTransform (Variables|Default|GetOutside)) (Transformation|GetWorldLocation (Variables|/Game/Engineers/Blueprints/Parents/IndexCollider.IndexCollider_C|GetSphere (Variables|Default|GetOverlapping%20Collider)))))) 0.0 _defaultdistance) 0.0) false false)
      (if (== (Variables|Default|GetProgress) 1.0)
        (Class|PlayerController|PlayHapticEffect (Game|GetPlayerController 0) "/Game/Misc/HapticEvents/ButtonClick.ButtonClick" (Variables|/Game/Engineers/Blueprints/Parents/IndexCollider.IndexCollider_C|GetHand (Variables|Default|GetOverlapping%20Collider)) 1.0 false)
        (Variables|Default|SetOverlapping%20Collider 0)
        (CallFunction|Triggered)
        (else
          (Rendering|Material|SetScalarParameterValueonMaterials (Variables|Default|GetOutside) "Intensity" (Variables|Default|GetProgress))
          (Class|PlayerController|SetHapticsbyValue (Game|GetPlayerController 0) 0.0 (/ (Variables|Default|GetProgress) 2.0) (Variables|/Game/Engineers/Blueprints/Parents/IndexCollider.IndexCollider_C|GetHand (Variables|Default|GetOverlapping%20Collider))))))
    (:Is%20Not%20Valid
      ;[1 1 1] Focus by laser, but only if animation is not running
      (if (not (Variables|Default|GetAnimationRunning))
        (Rendering|Material|SetScalarParameterValueonMaterials (Variables|Default|GetOutside) "Intensity" (Math|Float|SelectFloat 0.65 0.0 (Default|HasFocus (Variables|Default|GetLaserInteract))))))))

(event EventBeginPlay
  (EventDispatchers|BindEventtoIndexAction (Variables|Default|GetLaserInteract) (delegate Custom|Laser%20Call))
  (Variables|Default|SetDefaultDistance (.Y (Math|Vector|BreakVector (Variables|/Script/Engine.SceneComponent|GetRelativeLocation (Variables|Default|GetInside))))))

(event Collision|EventActorEndOverlap
  (params (OtherActor :type Actor%20Object%20Reference))
  ;[1 1 1] Clear collider
  (if (== OtherActor (Variables|Default|GetOverlapping%20Collider))
    (Default|CallFocusLost)
    (Class|PlayerController|StopHapticEffect (Game|GetPlayerController 0) (Variables|/Game/Engineers/Blueprints/Parents/IndexCollider.IndexCollider_C|GetHand (Variables|Default|GetOverlapping%20Collider)))
    (Variables|Default|SetOverlapping%20Collider 0)
    (Transformation|SetRelativeLocation (Variables|Default|GetInside) (Math|Vector|MakeVector 0.0 (Variables|Default|GetDefaultDistance) 0.0) false false)
    (Rendering|Material|SetScalarParameterValueonMaterials (Variables|Default|GetOutside) "Intensity" 0.0)))

(fn ConstructionScript
  (bind _returnvalue (Rendering|Material|CreateDynamicMaterialInstance (Variables|Default|GetInside) 0 "/Game/Artists/Materials/ButtonFront.ButtonFront" :!class /Script/Engine.PrimitiveComponent))
  (bind _output_get (Variables|Default|SetIconMat _returnvalue))
  (Rendering|Material|SetVectorParameterValue _output_get "Color" (Variables|Default|GetInnerColor) :!class /Script/Engine.MaterialInstanceDynamic)
  (CallFunction|SetIcon (Variables|Default|GetIcon))
  (CallFunction|SetType (Variables|Default|GetType))
  (CallFunction|SetCaption (Variables|Default|GetCaptionText))
  (Rendering|Material|SetVectorParameterValueonMaterials (Variables|Default|GetOutside) "Color" (Math|Conversions|ToVector(LinearColor) (Variables|Default|GetOuterColor))))

(fn SetIcon
  (params (Icon :type Texture%20Object%20Reference))
  (bind _output_get (Variables|Default|SetIcon Icon))
  (Rendering|Material|SetTextureParameterValue (Variables|Default|GetIconMat) "Icon" _output_get))

(fn SetType
  (params (Type :type ButtonTypes%20Enum :default "NewEnumerator0"))
  (switch Utilities|FlowControl|Switch|SwitchonButtonTypes Type
    (:NewEnumerator0
      (Components|StaticMesh|SetStaticMesh (Variables|Default|GetOutside) "/Game/Artists/Models/Static/ButtonInteract/ButtonBorder.ButtonBorder")
      (Components|StaticMesh|SetStaticMesh (Variables|Default|GetInside) "/Game/Artists/Models/Static/ButtonInteract/Button.Button"))
    (:NewEnumerator2
      (Components|StaticMesh|SetStaticMesh (Variables|Default|GetOutside) "/Game/Artists/Models/Static/ButtonInteract/2x1ButtonBorder.2x1ButtonBorder")
      (Components|StaticMesh|SetStaticMesh (Variables|Default|GetInside) "/Game/Artists/Models/Static/ButtonInteract/2x1Button.2x1Button"))
    (:NewEnumerator3
      (Components|StaticMesh|SetStaticMesh (Variables|Default|GetOutside) "/Game/Artists/Models/Static/ButtonInteract/4x1_b.4x1_b")
      (Components|StaticMesh|SetStaticMesh (Variables|Default|GetInside) "/Game/Artists/Models/Static/ButtonInteract/4x1.4x1"))
    (:NewEnumerator1
      (Components|StaticMesh|SetStaticMesh (Variables|Default|GetOutside) "/Game/Artists/Models/Static/ButtonInteract/UIButtonWideBorder.UIButtonWideBorder")
      (Components|StaticMesh|SetStaticMesh (Variables|Default|GetInside) "/Game/Artists/Models/Static/ButtonInteract/UIButtonWide.UIButtonWide"))
    (:NewEnumerator4
      (Components|StaticMesh|SetStaticMesh (Variables|Default|GetOutside) "/Game/Artists/Models/Static/ButtonInteract/2x2_b.2x2_b")
      (Components|StaticMesh|SetStaticMesh (Variables|Default|GetInside) "/Game/Artists/Models/Static/ButtonInteract/2x2.2x2"))
    (:NewEnumerator5
      (Components|StaticMesh|SetStaticMesh (Variables|Default|GetOutside) "/Game/Artists/Models/Static/ButtonInteract/4x4_b.4x4_b")
      (Components|StaticMesh|SetStaticMesh (Variables|Default|GetInside) "/Game/Artists/Models/Static/ButtonInteract/4x4.4x4"))
    (:NewEnumerator6
      (Components|StaticMesh|SetStaticMesh (Variables|Default|GetOutside) "/Game/Artists/Models/Static/ButtonInteract/6x6_b.6x6_b")
      (Components|StaticMesh|SetStaticMesh (Variables|Default|GetInside) "/Game/Artists/Models/Static/ButtonInteract/6x6.6x6"))))

(fn SetCaption
  (params (Text :type Text))
  (bind _output_get (Variables|Default|SetCaptionText Text))
  (Rendering|Components|TextRender|SetText (Variables|Default|GetCaption) _output_get))