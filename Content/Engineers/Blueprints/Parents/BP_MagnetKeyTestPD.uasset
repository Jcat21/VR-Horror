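; Magnet key test Blueprint that gives visual feedback for a left or right hand key using a decal and two point lights.
; BeginPlay tints the lights red or blue and sets the decal by Hand, then binds handlers for turning on and off.
; Turning on brightens the decal if IsInteractingWithSomething, otherwise shows only PointLight1.
; Turning off restores the dimmer decal and hides both lights.
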(event Custom|TurnOFF
  (Variables|Default|SetisOn false)
  (CallFunction|ChangetoDimmerMaterial)
  (CallFunction|TurnOffLight))

(event Custom|TurnON
  (Variables|Default|SetisOn true)
  (if (Variables|Default|GetIsInteractingWithSomething)
    (CallFunction|ChangetoBrighterMaterial)
    (else
      (CallFunction|TurnonLight))))

(event Custom|ChangeToBrighterMaterial
  (bind _decal (Variables|Default|GetDecal))
  (switch Utilities|FlowControl|Switch|SwitchonEControllerHand (Variables|Default|GetHand)
    (:Left
      (Rendering|Components|Decal|SetDecalMaterial _decal "/Game/Artists/Materials/M_LeftMagnetKeyTurnedON.M_LeftMagnetKeyTurnedON"))
    (:Right
      (Rendering|Components|Decal|SetDecalMaterial _decal "/Game/Artists/Materials/M_RightMagnetKeyTurnedON.M_RightMagnetKeyTurnedON"))))

(event Custom|TurnOnLight
  (Rendering|SetVisibility (Variables|Default|GetPointLight1) true false))

(event Custom|ChangeToDimmerMaterial
  (bind _decal (Variables|Default|GetDecal))
  (switch Utilities|FlowControl|Switch|SwitchonEControllerHand (Variables|Default|GetHand)
    (:Left
      (Rendering|Components|Decal|SetDecalMaterial _decal "/Game/Artists/Materials/M_LeftMagnetKeyDecal.M_LeftMagnetKeyDecal"))
    (:Right
      (Rendering|Components|Decal|SetDecalMaterial _decal "/Game/Artists/Materials/M_RightMagnetKeyDecal.M_RightMagnetKeyDecal"))))

(event Custom|TurnOffLight
  (Rendering|SetVisibility (Variables|Default|GetPointLight) false false)
  (Rendering|SetVisibility (Variables|Default|GetPointLight1) false false))

(event EventBeginPlay
  (bind _pointlight (Variables|Default|GetPointLight))
  (bind _decal (Variables|Default|GetDecal))
  (bind _pointlight1 (Variables|Default|GetPointLight1))
  (Utilities|FlowControl|Sequence
    (:then_0
      (switch Utilities|FlowControl|Switch|SwitchonEControllerHand (Variables|Default|GetHand)
        (:Left
          (Rendering|Components|Light|SetLightColor _pointlight1 "(R=1.000000,G=0.040000,B=0.000000,A=1.000000)" true)
          (Rendering|Components|Decal|SetDecalMaterial _decal "/Game/Artists/Materials/M_LeftMagnetKeyDecal.M_LeftMagnetKeyDecal")
          (Rendering|Components|Light|SetLightColor _pointlight "(R=1.000000,G=0.040000,B=0.000000,A=1.000000)" true))
        (:Right
          (Rendering|Components|Light|SetLightColor _pointlight1 "(R=0.000000,G=0.150000,B=1.000000,A=1.000000)" true)
          (Rendering|Components|Decal|SetDecalMaterial _decal "/Game/Artists/Materials/M_RightMagnetKeyDecal.M_RightMagnetKeyDecal")
          (Rendering|Components|Light|SetLightColor _pointlight "(R=0.000000,G=0.150000,B=1.000000,A=1.000000)" true))))
    (:then_1
      (EventDispatchers|BindEventtoTurnedon (delegate Custom|TurnON)))
    (:then_2
      (EventDispatchers|BindEventtoTurnedOff (delegate Custom|TurnOFF)))))

(fn ConstructionScript)