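; Handheld VR magnet key for the left or right hand, doubling as a pause menu pointer.
; On/off events swap hand-specific materials, fade audio and toggle optional lighting.
; Clicking presses through its widget interaction or takes pointer focus from the other controller; the left starts inactive.
; Tick fakes collision: when the capsule overlaps static mesh actors, it shifts the owning pawn horizontally toward the last valid position with haptics.
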(event Custom|Release
  ;[1 1 1] Pause Menu Interaction
  (Class|WidgetInteractionComponent|ReleasePointerKey (Variables|Default|GetWidgetInteraction) "LeftMouseButton"))

(event Custom|TurnOFF
  (Variables|Default|SetisOn false)
  (CallFunction|ChangetoDimmerMaterial)
  (CallFunction|TurnOffLight)
  (Audio|Components|Audio|FadeOut (Variables|Default|GetAudio) 0.5 0.0 :!class /Script/Engine.AudioComponent))

(event Custom|Click
  (params (OtherController :type BP%20Magnet%20Key%20Object%20Reference))
  (bind _widgetinteraction (Variables|Default|GetWidgetInteraction))
  ;[1 1 1] Pause Menu Interaction
  (if (Components|Activation|IsActive _widgetinteraction)
    (Class|WidgetInteractionComponent|PressPointerKey _widgetinteraction "LeftMouseButton")
    (else
      (Components|Activation|SetActive (Variables|BP_MagnetKey_C|GetWidgetInteraction OtherController) false false)
      (Components|Activation|SetActive _widgetinteraction true false))))

(event Custom|TurnON
  (Variables|Default|SetisOn true)
  (if (Variables|Default|GetisUsingLighting)
    (CallFunction|TurnonLight))
  (CallFunction|ChangetoBrighterMaterial)
  (Audio|Components|Audio|FadeIn (Variables|Default|GetAudio) 0.5 1.0 0.0 :!class /Script/Engine.AudioComponent))

(event Custom|ChangeToBrighterMaterial
  (bind _key (Variables|Default|GetKey))
  (switch Utilities|FlowControl|Switch|SwitchonEControllerHand (Variables|Default|GetHand)
    (:Left
      (Rendering|Material|SetMaterial _key 1 "/Game/Artists/Materials/M_LeftMagnetKeyTurnedON.M_LeftMagnetKeyTurnedON"))
    (:Right
      (Rendering|Material|SetMaterial _key 1 "/Game/Artists/Materials/M_RightMagnetKeyTurnedON.M_RightMagnetKeyTurnedON"))))

(event Custom|TurnOnLight
  ;[1 1 1] Light ON
  (Rendering|SetVisibility (Variables|Default|GetPointLight) true false))

(event Custom|ChangeToDimmerMaterial
  (bind _key (Variables|Default|GetKey))
  (switch Utilities|FlowControl|Switch|SwitchonEControllerHand (Variables|Default|GetHand)
    (:Left
      (Rendering|Material|SetMaterial _key 1 "/Game/Artists/Materials/M_LeftMagnetKeyDecal.M_LeftMagnetKeyDecal"))
    (:Right
      (Rendering|Material|SetMaterial _key 1 "/Game/Artists/Materials/M_RightMagnetKeyDecal.M_RightMagnetKeyDecal"))))

(event Custom|TurnOffLight
  (Rendering|SetVisibility (Variables|Default|GetPointLight) false false)
  (Rendering|SetVisibility (Variables|Default|GetSpotLight) false false))

(event EventBeginPlay
  (bind _key (Variables|Default|GetKey))
  (Utilities|FlowControl|Sequence
    (:then_0
      (switch Utilities|FlowControl|Switch|SwitchonEControllerHand (Variables|Default|GetHand)
        (:Left
          (Rendering|Material|SetMaterial _key 1 "/Game/Artists/Materials/M_LeftMagnetKeyDecal.M_LeftMagnetKeyDecal")
          (Components|Activation|SetActive (Variables|Default|GetWidgetInteraction) false false))
        (:Right
          (Rendering|Material|SetMaterial _key 1 "/Game/Artists/Materials/M_RightMagnetKeyDecal.M_RightMagnetKeyDecal"))))
    (:then_1
      (EventDispatchers|BindEventtoTurnedon (delegate Custom|TurnON)))
    (:then_2
      (EventDispatchers|BindEventtoTurnedOff (delegate Custom|TurnOFF)))))

(event EventTick
  (params (DeltaSeconds :type Float%20%28single-precision%29))
  (bind _returnvalue (Game|GetPlayerController 0))
  (Utilities|FlowControl|Sequence
    (:then_0
      ;[1 1 1] Simulate collision
      (if (> (Utilities|Array|Length (Collision|GetOverlappingActors (Variables|Default|GetCapsule) "/Script/Engine.StaticMeshActor" :!class /Script/Engine.PrimitiveComponent)) 0)
        (Transformation|AddActorWorldOffset (Variables|Default|GetOwningPawn) (Math|Vector|MakeVector (.X (Math|Vector|BreakVector (- (Variables|Default|GetLastValidPosition) (Transformation|GetWorldLocation (Variables|Default|GetCapsule))))) (.Y (Math|Vector|BreakVector (- (Variables|Default|GetLastValidPosition) (Transformation|GetWorldLocation (Variables|Default|GetCapsule))))) 0.0) false true)
        (switch Utilities|FlowControl|Switch|SwitchonEControllerHand (Variables|Default|GetHand)
          (:Left
            (Class|PlayerController|PlayHapticEffect _returnvalue "/Game/Misc/HapticEvents/Grab.Grab" "Left" 1.0 false))
          (:Right
            (Class|PlayerController|PlayHapticEffect _returnvalue "/Game/Misc/HapticEvents/Grab.Grab" "Right" 1.0 false)))
        (else
          (Variables|Default|SetLastValidPosition (Transformation|GetWorldLocation (Variables|Default|GetCapsule))))))))

(fn ConstructionScript)