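; Goggles pickup that the player carries with two magnet keys and puts on to travel to another level.
; Left and right handle overlaps register each hand's key; while both are on, Tick holds the goggles midway between points in front of them.
; Touching the pawn's capsule hides the pickup, fades out, applies level-specific actor changes, streams in LevelName and teleports the player to TeleportName before fading back in.
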(event OnComponentBeginOverlap(Goggles)
  (params (OverlappedComponent :type Primitive%20Component%20Object%20Reference) (OtherActor :type Actor%20Object%20Reference) (OtherComp :type Primitive%20Component%20Object%20Reference) (OtherBodyIndex :type Integer) (bFromSweep :type Boolean) (SweepResult :type Hit%20Result%20Structure%20%28by%20ref%29))
  (bind _playerreference (Variables|Default|GetPlayerReference))
  (bind _asbp_main_pawn (Utilities|Casting|CastToBP_MainPawn OtherActor))
  (Utilities|Casting|CastToCapsuleComponent OtherComp)
  (if (not (Variables|Default|GetisConnectedToPlayer))
    (Variables|Default|SetisConnectedToPlayer true)
    (Rendering|SetActorHiddenInGame true)
    (Rendering|SetVisibility (Variables|/Game/Engineers/Blueprints/Parents/BP_MainPawn.BP_MainPawn_C|GetGoggles _asbp_main_pawn) true true)
    (CameraFades|StartCameraFade :self (Game|GetPlayerCameraManager 0) :ToAlpha 1.0 :Duration 5.0 :bHoldWhenFinished true)
    (Utilities|FlowControl|Delay 5.0)
    (if (Utilities|Enum|Equal(Enum) (Variables|Default|GetLevelName) "SCENE_AJMedicalRoom")
      (bind _outactors (Actor|GetAllActorsOfClass "/Script/Engine.StaticMeshActor"))
      (for _array_element _outactors
        (Rendering|SetActorHiddenInGame _array_element true))
      (bind _outactors_2 (Actor|GetAllActorsOfClass "/Game/Engineers/Blueprints/Misc/BP_DoorCryoCorridor.BP_DoorCryoCorridor_C"))
      (for _array_element_2 _outactors_2
        (Rendering|SetActorHiddenInGame _array_element_2 true))
      (else
        (bind _outactors_3 (Actor|GetAllActorsOfClass "/Game/Engineers/Blueprints/Parents/BP_MagnetKey.BP_MagnetKey_C"))
        (for _array_element_3 _outactors_3
          (Variables|/Game/Engineers/Blueprints/Parents/BP_MagnetKey.BP_MagnetKey_C|SetisUsingLighting _array_element_3 true))))
    (Game|LoadStreamLevel(byName) (Utilities|String|StringToName (Variables|Default|GetLevelName)) true)
    (Default|SetNewTeleportLocs _playerreference)
    (bind (_spawn _found_) (Default|FindTeleportLoc _playerreference (Variables|Default|GetTeleportName)))
    (Rendering|SetVisibility (Variables|/Game/Engineers/Blueprints/Parents/BP_MainPawn.BP_MainPawn_C|GetGoggles _playerreference) false true)
    (if _found_
      (Transformation|SetActorLocationAndRotation _playerreference (Transformation|GetActorLocation _spawn) (Transformation|GetActorRotation _spawn) false true)
      (Default|Reset _playerreference)
      (CameraFades|StartCameraFade :self (Game|GetPlayerCameraManager 0) :FromAlpha 1.0 :Duration 5.0)
      (if (Utilities|Enum|Equal(Enum) (Variables|Default|GetLevelName) "CraneGame")
        (Audio|PlaySound2D "/Game/Artists/Audio/Sounds/DX/Line_6.Line_6")))))

(event OnComponentBeginOverlap(LeftHandle)
  (params (OverlappedComponent :type Primitive%20Component%20Object%20Reference) (OtherActor :type Actor%20Object%20Reference) (OtherComp :type Primitive%20Component%20Object%20Reference) (OtherBodyIndex :type Integer) (bFromSweep :type Boolean) (SweepResult :type Hit%20Result%20Structure%20%28by%20ref%29))
  (bind _asbp_magnet_key (Utilities|Casting|CastToBP_MagnetKey OtherActor))
  (Utilities|Casting|CastToSphereComponent OtherComp)
  (if (Utilities|Enum|Equal(Enum) (Variables|/Game/Engineers/Blueprints/Parents/BP_MagnetKey.BP_MagnetKey_C|GetHand _asbp_magnet_key) "Left")
    (Variables|Default|SetLeftMagKey _asbp_magnet_key)))

(event OnComponentEndOverlap(RightHandle)
  (params (OverlappedComponent :type Primitive%20Component%20Object%20Reference) (OtherActor :type Actor%20Object%20Reference) (OtherComp :type Primitive%20Component%20Object%20Reference) (OtherBodyIndex :type Integer))
  (bind _asbp_magnet_key (Utilities|Casting|CastToBP_MagnetKey OtherActor))
  (if (Utilities|Enum|Equal(Enum) (Variables|/Game/Engineers/Blueprints/Parents/BP_MagnetKey.BP_MagnetKey_C|GetHand _asbp_magnet_key) "Right")
    (if (Utilities|IsValid (Variables|Default|GetRightMagKey))
      (if (not (Variables|/Game/Engineers/Blueprints/Parents/BP_MagnetKey.BP_MagnetKey_C|GetisOn (Variables|Default|GetRightMagKey)))
        (Variables|Default|SetRightMagKey 0)))))

(event OnComponentEndOverlap(LeftHandle)
  (params (OverlappedComponent :type Primitive%20Component%20Object%20Reference) (OtherActor :type Actor%20Object%20Reference) (OtherComp :type Primitive%20Component%20Object%20Reference) (OtherBodyIndex :type Integer))
  (bind _asbp_magnet_key (Utilities|Casting|CastToBP_MagnetKey OtherActor))
  (if (Utilities|Enum|Equal(Enum) (Variables|/Game/Engineers/Blueprints/Parents/BP_MagnetKey.BP_MagnetKey_C|GetHand _asbp_magnet_key) "Left")
    (if (Utilities|IsValid (Variables|Default|GetLeftMagKey))
      (if (not (Variables|/Game/Engineers/Blueprints/Parents/BP_MagnetKey.BP_MagnetKey_C|GetisOn (Variables|Default|GetLeftMagKey)))
        (Variables|Default|SetLeftMagKey 0)))))

(event OnComponentBeginOverlap(RightHandle)
  (params (OverlappedComponent :type Primitive%20Component%20Object%20Reference) (OtherActor :type Actor%20Object%20Reference) (OtherComp :type Primitive%20Component%20Object%20Reference) (OtherBodyIndex :type Integer) (bFromSweep :type Boolean) (SweepResult :type Hit%20Result%20Structure%20%28by%20ref%29))
  (bind _asbp_magnet_key (Utilities|Casting|CastToBP_MagnetKey OtherActor))
  (Utilities|Casting|CastToSphereComponent OtherComp)
  (if (Utilities|Enum|Equal(Enum) (Variables|/Game/Engineers/Blueprints/Parents/BP_MagnetKey.BP_MagnetKey_C|GetHand _asbp_magnet_key) "Right")
    (Variables|Default|SetRightMagKey _asbp_magnet_key)))

(event Custom|TurnOffMagnet
  (Variables|Default|SetMagKeyReference 0))

(event EventTick
  (params (DeltaSeconds :type Float%20%28single-precision%29))
  (bind _rightmagkey (Variables|Default|GetRightMagKey))
  (bind _leftmagkey (Variables|Default|GetLeftMagKey))
  (if (not (Variables|Default|GetisConnectedToPlayer))
    (if (and (Utilities|IsValid (Variables|Default|GetLeftMagKey)) (Utilities|IsValid (Variables|Default|GetRightMagKey)))
      (Utilities|FlowControl|Sequence
        (:then_0
          (if (and (Variables|/Game/Engineers/Blueprints/Parents/BP_MagnetKey.BP_MagnetKey_C|GetisOn (Variables|Default|GetRightMagKey)) (Variables|/Game/Engineers/Blueprints/Parents/BP_MagnetKey.BP_MagnetKey_C|GetisOn (Variables|Default|GetLeftMagKey)))
            (Transformation|SetWorldLocation (Variables|Default|GetGoggles) (/ (+ (+ (Transformation|GetActorLocation _rightmagkey) (* (Transformation|GetActorForwardVector _rightmagkey) (Variables|Default|GetFwdDistance))) (+ (Transformation|GetActorLocation _leftmagkey) (* (Transformation|GetActorForwardVector _leftmagkey) (Variables|Default|GetFwdDistance)))) 2.0) false true)))))))

(event EventBeginPlay
  (bind _asbp_main_pawn (Utilities|Casting|CastToBP_MainPawn (Game|Player|GetPlayerPawn 0)))
  (Variables|Default|SetPlayerReference _asbp_main_pawn))

(event Collision|EventActorEndOverlap
  (params (OtherActor :type Actor%20Object%20Reference)))

(event Collision|EventActorBeginOverlap
  (params (OtherActor :type Actor%20Object%20Reference)))

(fn ConstructionScript)