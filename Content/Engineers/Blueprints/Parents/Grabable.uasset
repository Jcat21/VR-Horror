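; Grabable base component that lets a hand pick up, throw, slide or turn its owner's volume, with highlighting and grab, release, move and thumb/index action notifies.
; Relative and Fixed grabs attach the owner to the hand and log recent positions to derive throw velocity on release.
; Directional and Rotational grabs track the hand along one axis, optionally clamped, and release it when it strays beyond tolerance.
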(event EventBeginPlay)

(event EventTick
  (params (DeltaSeconds :type Float%20%28single-precision%29))
  (if (CallFunction|IsGrabbed)
    (switch Utilities|FlowControl|Switch|SwitchonGrabTypes (Variables|Default|GetGrabType)
      (:NewEnumerator0
        ;[1 1 1] Log location
        (bind _output_get (Variables|Default|SetTime (+ DeltaSeconds (Variables|Default|GetTime)) :!label _label))
        (bind _returnvalue (Utilities|Array|Add (Variables|Default|GetLocationLog) (Utilities|Struct|MakeLocationLog _output_get (Transformation|GetActorLocation (Components|GetOwner)))))
        ;[1 1 1] Remove all items above 200ms except one
        (if (> _returnvalue 1)
          (if (> (- (Variables|Default|GetTime) (.Time (Utilities|Struct|BreakLocationLog (Utilities|Array|Get(acopy) (Variables|Default|GetLocationLog) 1)))) 0.2) :!label _label_2
            (Utilities|Array|RemoveIndex (Variables|Default|GetLocationLog))
            (goto _label_2))))
      (:NewEnumerator1
        (goto _label))
      (:NewEnumerator2
        (CallFunction|TickDirectionalGrab))
      (:NewEnumerator3
        (CallFunction|TickRotationalGrab)))))

(fn Grabbed
  (params (Hand :type Hand%20BP%20Object%20Reference) (GrabBase :type Scene%20Component%20Object%20Reference))
  (bind _returnvalue (Components|GetOwner))
  (bind _volume (Variables|Components|GetVolume))
  (if (CallFunction|IsGrabbed)
    (Actions|StopActions)
    (Default|OffhandGrab (Variables|Default|GetHand))
    (else
      (Variables|Default|SetSimulationPhysics (Physics|IsSimulatingPhysics _volume "None"))
      (Variables|Default|SetGravityEnabled (Class|PrimitiveComponent|IsGravityEnabled _volume))))
  (bind _output_get (Variables|Default|SetHand Hand))
  (Default|SetGrabAnimation _output_get (Variables|Default|GetGrabAnimation))
  (Physics|SetSimulatePhysics _volume false)
  (Physics|SetEnableGravity _volume false)
  (Default|CallGrabNotify)
  (Variables|Default|SetTime 0.0)
  (Utilities|Array|Clear (Variables|Default|GetLocationLog))
  (switch Utilities|FlowControl|Switch|SwitchonGrabTypes (Variables|Default|GetGrabType)
    (:NewEnumerator0
      (Transformation|AttachComponentToComponent _returnvalue GrabBase "None" "KeepWorld" "KeepWorld" "KeepWorld" true))
    (:NewEnumerator1
      (switch Utilities|FlowControl|Switch|SwitchonEControllerHand (Variables|/Game/Engineers/Blueprints/Parents/HandBP.HandBP_C|GetHandType (Variables|Default|GetHand))
        (:Left
          (Transformation|SetRelativeTransform GrabBase (Variables|Default|GetFixedGrabTransformLeft) false false))
        (:Right
          (Transformation|SetRelativeTransform GrabBase (Variables|Default|GetFixedGrabTransformRight) false false)))
      (Transformation|AttachComponentToComponent _returnvalue GrabBase "None" "SnapToTarget" "SnapToTarget" "KeepWorld" true))))

(fn Released
  (bind _simulationphysics (Variables|Default|GetSimulationPhysics))
  (bind _locationlog (Variables|Default|GetLocationLog))
  (bind _output (Utilities|Array|Get(acopy) _locationlog))
  (bind (_time _location) (Utilities|Struct|BreakLocationLog _output))
  (Utilities|FlowControl|Sequence
    (:then_0
      (Actions|StopActions)
      (Physics|SetSimulatePhysics (Variables|Components|GetVolume) _simulationphysics)
      (if _simulationphysics
        ;[1 1 1] Add velocity based on movement last 200ms, for more realistic throws
        (Physics|SetPhysicsLinearVelocity (Variables|Components|GetVolume) (/ (/ (- (Transformation|GetActorLocation (Components|GetOwner)) _location) (- (Variables|Default|GetTime) _time)) 2.0) true "None"))
      (Physics|SetEnableGravity (Variables|Components|GetVolume) (Variables|Default|GetGravityEnabled))
      (Variables|Default|SetHand 0)
      (switch Utilities|FlowControl|Switch|SwitchonGrabTypes (Variables|Default|GetGrabType)
        (:NewEnumerator0
          _)
        (:NewEnumerator1
          _))
      (Transformation|DetachFromActor (Components|GetOwner self) "KeepWorld" "KeepWorld" "KeepWorld"))
    (:then_1
      (Default|CallReleaseNotify))))

(fn SetRelativeGrab
  (params (Volume :type Primitive%20Component%20Object%20Reference%20%28by%20ref%29) (Animation :type Anim%20Sequence%20Object%20Reference))
  (bind _output_get (Variables|Components|SetVolume Volume))
  (Variables|Components|SetHighlightVolume _output_get)
  (Variables|Default|SetGrabType "NewEnumerator0")
  (Variables|Default|SetGrabAnimation Animation)
  (Variables|Default|SetGrabAllowed true))

(fn GetVolume
  (return (Variables|Components|GetVolume)))

(fn SetFixedGrab
  (params (Volume :type Primitive%20Component%20Object%20Reference%20%28by%20ref%29) (GrabTransformLeft :type Transform) (Animation :type Anim%20Sequence%20Object%20Reference) (GrabTransFormRight :type Transform))
  (Variables|Default|SetGrabAnimation Animation)
  (bind _output_get (Variables|Components|SetVolume Volume))
  (Variables|Components|SetHighlightVolume _output_get)
  (Variables|Default|SetGrabType "NewEnumerator1")
  (Variables|Default|SetFixedGrabTransformLeft GrabTransformLeft)
  (Variables|Default|SetFixedGrabTransformRight GrabTransFormRight)
  (Variables|Default|SetGrabAllowed true))

(fn IsGrabbed
  (return (Utilities|IsValid (Variables|Default|GetHand))))

(fn FireThumbAction
  (Variables|Actions|SetbThumbAction true)
  (Default|CallThumbAction))

(fn FireIndexAction
  (Variables|Actions|SetbIndexAction false)
  (Default|CallIndexAction))

(fn StopThumbAction
  (Variables|Actions|SetbThumbAction false)
  (Default|CallThumbActionStop))

(fn StopIndexAction
  (Variables|Actions|SetbIndexAction false)
  (Default|CallIndexActionStop))

(fn StopActions
  (if (Variables|Actions|GetbThumbAction)
    (Actions|StopThumbAction))
  (if (Variables|Actions|GetbIndexAction)
    (Actions|StopIndexAction)))

(fn ClearGrab
  (if (CallFunction|IsGrabbed)
    (Default|Release (Variables|Default|GetHand)))
  (Variables|Components|SetVolume 0)
  (Variables|Default|SetGrabAllowed false))

(fn Highlight
  (bind _highlightvolume (Variables|Components|GetHighlightVolume))
  (Rendering|SetRenderCustomDepth _highlightvolume true)
  (Class|PrimitiveComponent|SetCustomDepthStencilWriteMask _highlightvolume "ERSM_8")
  (Rendering|SetCustomDepthStencilValue _highlightvolume 8))

(fn ClearHighlight
  (Rendering|SetRenderCustomDepth (Variables|Components|GetHighlightVolume) false))

(fn SetDirectionalGrab
  (params (Axis :type ESplineMeshAxis%20Enum :default "X") (GrabPoint :type Vector) (Volume :type Primitive%20Component%20Object%20Reference%20%28by%20ref%29) (DistanceMin :type Float%20%28single-precision%29) (DistanceMax :type Float%20%28single-precision%29) (DistanceTolerance :type Float%20%28single-precision%29) (GrabAnim :type Anim%20Sequence%20Object%20Reference) (HighlightVolume :type Primitive%20Component%20Object%20Reference) (EnforceLimits :type Boolean))
  (Variables|Default|SetGrabAxis Axis)
  (Variables|Default|SetGrabPoint GrabPoint)
  (Variables|Components|SetVolume Volume)
  (Variables|Default|SetDistanceMin DistanceMin)
  (Variables|Default|SetDIstanceMax DistanceMax)
  (Variables|Default|SetToleranceSQ (Math|Float|Square DistanceTolerance))
  (Variables|Default|SetGrabAnimation GrabAnim)
  (Variables|Components|SetHighlightVolume HighlightVolume)
  (Variables|Default|SetEnforceLimits EnforceLimits)
  (Variables|Default|SetGrabAllowed true)
  (Variables|Default|SetGrabType "NewEnumerator2"))

(fn TickDirectionalGrab
  (bind _grabaxis (Variables|Default|GetGrabAxis))
  (bind _hand (Variables|Default|GetHand))
  (bind _volume (Variables|Components|GetVolume))
  (bind _grabpoint (Variables|Default|GetGrabPoint))
  (bind _returnvalue (Transformation|GetWorldTransform _volume))
  (bind (_x _y _z) (Math|Vector|BreakVector _grabpoint))
  (bind _grabbase (Variables|/Game/Engineers/Blueprints/Parents/HandBP.HandBP_C|GetGrabBase _hand))
  (bind _returnvalue_2 (Transformation|GetWorldLocation _grabbase))
  (bind _returnvalue_3 (Math|Transform|InvertTransform _returnvalue))
  (bind _returnvalue_4 (Math|Transform|TransformLocation _returnvalue_3 _returnvalue_2))
  (bind (_x_2 _y_2 _z_2) (Math|Vector|BreakVector _returnvalue_4))
  (CallFunction|MovetoDistance (+ (Variables|Default|GetDistance) (- (Utilities|Select :Index _grabaxis :X _x_2 :Y _y_2 :Z _z_2) (Utilities|Select :Index _grabaxis :X _x :Y _y :Z _z))))
  (CallFunction|CheckHandDistance))

(fn SetRotationalGrab
  (params (Axis :type ESplineMeshAxis%20Enum :default "X") (Volume :type Primitive%20Component%20Object%20Reference) (HighlightVolume :type Primitive%20Component%20Object%20Reference) (GrabPoint :type Vector) (RotationMin :type Float%20%28single-precision%29) (RotationMax :type Float%20%28single-precision%29) (EnforceLimits :type Boolean) (Distance%20Tolerance :type Float%20%28single-precision%29) (Grab%20Anim :type Anim%20Sequence%20Object%20Reference))
  (Variables|Default|SetGrabAxis Axis)
  (Variables|Components|SetVolume Volume)
  (Variables|Components|SetHighlightVolume HighlightVolume)
  (Variables|Default|SetGrabPoint GrabPoint)
  (Variables|Default|SetDistanceMin RotationMin)
  (Variables|Default|SetDIstanceMax RotationMax)
  (Variables|Default|SetEnforceLimits EnforceLimits)
  (Variables|Default|SetToleranceSQ (Math|Float|Square Distance%20Tolerance))
  (Variables|Default|SetGrabAnimation Grab%20Anim)
  (Variables|Default|SetGrabType "NewEnumerator3")
  (Variables|Default|SetGrabAllowed true))

(fn TickRotationalGrab
  (bind _hand (Variables|Default|GetHand))
  (bind _volume (Variables|Components|GetVolume))
  (bind _grabaxis (Variables|Default|GetGrabAxis))
  (bind _grabpoint (Variables|Default|GetGrabPoint))
  (bind _returnvalue (Transformation|GetWorldTransform _volume))
  (bind (_x _y _z) (Math|Vector|BreakVector _grabpoint))
  (bind _grabbase (Variables|/Game/Engineers/Blueprints/Parents/HandBP.HandBP_C|GetGrabBase _hand))
  (bind _returnvalue_2 (Transformation|GetWorldLocation _grabbase))
  (bind _returnvalue_3 (Math|Transform|InvertTransform _returnvalue))
  (bind _returnvalue_4 (Class|KismetMathLibrary|DegAtan2 _y _z))
  (bind _returnvalue_5 (Class|KismetMathLibrary|DegAtan2 _z _x))
  (bind _returnvalue_6 (Class|KismetMathLibrary|DegAtan2 _y _x))
  (bind _returnvalue_7 (Math|Transform|TransformLocation _returnvalue_3 _returnvalue_2))
  (bind _returnvalue_8 (Utilities|Select :Index _grabaxis :X _returnvalue_4 :Y _returnvalue_5 :Z _returnvalue_6))
  (bind (_x_2 _y_2 _z_2) (Math|Vector|BreakVector _returnvalue_7))
  (bind _returnvalue_9 (Class|KismetMathLibrary|DegAtan2 _y_2 _x_2))
  (bind _returnvalue_10 (Class|KismetMathLibrary|DegAtan2 _z_2 _x_2))
  (bind _returnvalue_11 (Class|KismetMathLibrary|DegAtan2 _y_2 _z_2))
  (bind _returnvalue_12 (Utilities|Select :Index _grabaxis :X _returnvalue_11 :Y _returnvalue_10 :Z _returnvalue_9))
  (bind _returnvalue_13 (- _returnvalue_12 _returnvalue_8))
  (bind _returnvalue_14 (Math|Float|Absolute(Float) _returnvalue_13))
  (CallFunction|MovetoDistance (+ (Variables|Default|GetDistance) (Math|Float|SelectFloat (+ _returnvalue_13 (* (/ _returnvalue_13 _returnvalue_14) -3.6e+02)) _returnvalue_13 (> _returnvalue_14 1.8e+02))))
  (CallFunction|CheckHandDistance))

(fn MovetoDistance
  (params (DesiredDistance :type Float%20%28single-precision%29))
  (bind _distancemax (Variables|Default|GetDIstanceMax))
  (bind _distancemin (Variables|Default|GetDistanceMin))
  (bind _volume (Variables|Components|GetVolume))
  (bind _volume_2 (Variables|Components|GetVolume))
  (bind _returnvalue (Math|Float|Clamp(Float) DesiredDistance _distancemin _distancemax))
  ;[1 1 1] Limit corrections
  (LocalVariables|SetTravelDifference (- DesiredDistance (Variables|Default|GetDistance)))
  (Variables|Default|SetDistance _returnvalue)
  (switch Utilities|FlowControl|Switch|SwitchonGrabTypes (Variables|Default|GetGrabType)
    (:NewEnumerator2
      ;[1 1 1] Directional Move
      (Transformation|SetWorldLocation _volume (Math|Transform|TransformLocation (Transformation|GetWorldTransform _volume) (Utilities|Select :Index (Variables|Default|GetGrabAxis) :X (Math|Vector|MakeVector (Math|Float|SelectFloat (- (LocalVariables|GetTravelDifference) (- DesiredDistance _returnvalue)) (LocalVariables|GetTravelDifference) (Variables|Default|GetEnforceLimits)) 0.0 0.0) :Y (Math|Vector|MakeVector 0.0 (Math|Float|SelectFloat (- (LocalVariables|GetTravelDifference) (- DesiredDistance _returnvalue)) (LocalVariables|GetTravelDifference) (Variables|Default|GetEnforceLimits)) 0.0) :Z (Math|Vector|MakeVector 0.0 0.0 (Math|Float|SelectFloat (- (LocalVariables|GetTravelDifference) (- DesiredDistance _returnvalue)) (LocalVariables|GetTravelDifference) (Variables|Default|GetEnforceLimits))))) false false))
    (:NewEnumerator3
      ;[1 1 1] Rotational Move
      (Transformation|SetWorldRotation _volume_2 (Math|Transform|TransformRotation (Transformation|GetWorldTransform _volume_2) (Utilities|Select :Index (Variables|Default|GetGrabAxis) :X (Math|Rotator|MakeRotator (Math|Float|SelectFloat (- (LocalVariables|GetTravelDifference) (- DesiredDistance _returnvalue)) (LocalVariables|GetTravelDifference) (Variables|Default|GetEnforceLimits)) 0.0 0.0) :Y (Math|Rotator|MakeRotator 0.0 (Math|Float|SelectFloat (- (LocalVariables|GetTravelDifference) (- DesiredDistance _returnvalue)) (LocalVariables|GetTravelDifference) (Variables|Default|GetEnforceLimits)) 0.0) :Z (Math|Rotator|MakeRotator 0.0 0.0 (Math|Float|SelectFloat (- (LocalVariables|GetTravelDifference) (- DesiredDistance _returnvalue)) (LocalVariables|GetTravelDifference) (Variables|Default|GetEnforceLimits))))) false false)))
  (Default|CallMoveNotify (Variables|Default|GetDistance)))

(fn CheckHandDistance
  (if (and (> (Math|Vector|VectorLengthSquared (- (Math|Transform|TransformLocation (Math|Transform|InvertTransform (Transformation|GetWorldTransform (Variables|Components|GetVolume))) (Transformation|GetWorldLocation (Variables|/Game/Engineers/Blueprints/Parents/HandBP.HandBP_C|GetGrabBase (Variables|Default|GetHand)))) (Variables|Default|GetGrabPoint))) (Variables|Default|GetToleranceSQ)) (> (Variables|Default|GetToleranceSQ) 0.0))
    (Default|Release (Variables|Default|GetHand))))