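; BP_PCMCube is a numbered puzzle cube that a magnet key carries and drops into slots on the referenced PCM test actor.
; On overlap it binds pickup and drop to the key's on and off events.
; A drop snaps it to the nearest free overlapped slot, colors its number green or red for correctness, and checks for a win.
; Without a slot, it spawns a replacement at its start transform and destroys itself.
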(event Custom|PickupCube
  (bind _magkey (Variables|Default|GetMagKey))
  (bind _currentslotname (Variables|Default|GetCurrentSlotName))
  (if (not (Variables|/Game/Engineers/Blueprints/Parents/BP_MagnetKey.BP_MagnetKey_C|GetIsHoldingSomething _magkey))
    (Transformation|AttachActorToActor _magkey "None" "KeepWorld" "KeepWorld" "KeepRelative" true)
    (Variables|/Game/Engineers/Blueprints/Parents/BP_MagnetKey.BP_MagnetKey_C|SetIsHoldingSomething _magkey true)
    (if (Utilities|Enum|NotEqual(Enum) _currentslotname "")
      (Default|UnfillPosition (Variables|Default|GetPCMTestRef) _currentslotname))))

(event Custom|DropCube
  (bind _textrender (Variables|Default|GetTextRender))
  (bind _magkey (Variables|Default|GetMagKey))
  (Variables|/Game/Engineers/Blueprints/Parents/BP_MagnetKey.BP_MagnetKey_C|SetIsHoldingSomething (Variables|Default|GetMagKey) false)
  (if (Collision|IsOverlappingActor (Variables|Default|GetPCMTestRef) :!class /Script/Engine.Actor)
    (bind _array_element (Utilities|Array|ForEachLoopwithBreak (Class|PrimitiveComponent|GetOverlappingComponents (Variables|Default|GetCube)))
      (:LoopBody
        (if (== (Components|GetOwner _array_element) (Variables|Default|GetPCMTestRef))
          (bind _filled (Default|CheckFilledPosition (Variables|Default|GetPCMTestRef) (Utilities|GetObjectName _array_element)))
          (if (not _filled)
            (if (< (Math|Vector|VectorLength (- (Transformation|GetActorLocation) (Transformation|GetWorldLocation _array_element))) (Variables|Default|GetClosestDistance))
              (Variables|Default|SetCurrentSlotName (Utilities|GetObjectName _array_element))
              (Variables|Default|SetClosestDistance (Math|Vector|VectorLength (- (Transformation|GetActorLocation) (Transformation|GetWorldLocation _array_element))))
              (Variables|Default|SetClosestLoc (Transformation|GetWorldLocation _array_element))))))
      (:Completed
        (if (Math|Vector|Equal(Vector) (Variables|Default|GetClosestLoc) "0, 0, 0" 0.0001)
          (bind _returnvalue (Game|SpawnActorfromClass "BP_PCMCube_C" (Variables|Default|GetSpawnTransform) "AdjustIfPossibleButAlwaysSpawn" 0 0 :!label _label))
          (Variables|BP_PCMCube_C|SetNumber _returnvalue (Variables|Default|GetNumber))
          (Rendering|Components|TextRender|SetText (Variables|BP_PCMCube_C|GetTextRender _returnvalue) (Utilities|Text|ToText(String) (Utilities|String|ToString(Integer) (Variables|Default|GetNumber))))
          (Variables|BP_PCMCube_C|SetPCMTestRef _returnvalue (Variables|Default|GetPCMTestRef))
          (Actor|DestroyActor)
          (else
            (Transformation|DetachFromActor "KeepWorld" "KeepWorld" "KeepWorld")
            (Transformation|SetActorLocationAndRotation (Variables|Default|GetClosestLoc) (Transformation|GetActorRotation (Variables|Default|GetPCMTestRef)) false true)
            (Default|FillPosition (Variables|Default|GetPCMTestRef) (Variables|Default|GetCurrentSlotName) (Variables|Default|GetNumber))
            (Variables|Default|SetClosestDistance 1e+04)
            (Variables|Default|SetClosestLoc "0, 0, 0")
            (Utilities|FlowControl|Sequence
              (:then_0
                (bind _iscorrectposition (Default|CheckCorrectPosition (Variables|Default|GetPCMTestRef) (Variables|Default|GetCurrentSlotName)))
                (if _iscorrectposition
                  (Rendering|Components|TextRender|SetTextRenderColor _textrender (Math|Color|MakeColor 0 255 0 255))
                  (else
                    (Rendering|Components|TextRender|SetTextRenderColor _textrender (Math|Color|MakeColor 0 0 255 255))))
                (if (Utilities|IsValid _magkey) :!label _label_2
                  (EventDispatchers|UnbindEventfromTurnedOff _magkey (delegate Custom|DropCube))
                  (EventDispatchers|UnbindEventfromTurnedon _magkey (delegate Custom|PickupCube))))
              (:then_1
                (bind _won_ (Default|CheckWin (Variables|Default|GetPCMTestRef)))
                (if _won_
                  (Rendering|SetVisibility (Variables|/Game/Engineers/Blueprints/Parents/BP_PCMTest.BP_PCMTest_C|GetTextRender (Variables|Default|GetPCMTestRef)) true false)
                  (goto _label_2))))))))
    (else
      (goto _label))))

(event EventBeginPlay
  (Variables|Default|SetSpawnTransform (Transformation|GetWorldTransform (Variables|Default|GetCube))))

(event Collision|EventActorEndOverlap
  (params (OtherActor :type Actor%20Object%20Reference))
  (if (and (== OtherActor (Variables|Default|GetMagKey)) (Utilities|IsValid (Variables|Default|GetMagKey)))
    (if (not (Variables|/Game/Engineers/Blueprints/Parents/BP_MagnetKey.BP_MagnetKey_C|GetisOn (Variables|Default|GetMagKey)))
      (EventDispatchers|UnbindEventfromTurnedOff (Variables|Default|GetMagKey) (delegate Custom|DropCube))
      (EventDispatchers|UnbindEventfromTurnedon (Variables|Default|GetMagKey) (delegate Custom|PickupCube))
      (Variables|Default|SetMagKey 0))))

(event Collision|EventActorBeginOverlap
  (params (OtherActor :type Actor%20Object%20Reference))
  (bind _asbp_magnet_key (Utilities|Casting|CastToBP_MagnetKey OtherActor))
  (if (Math|Boolean|ANDBoolean (Class|PrimitiveComponent|IsOverlappingComponent (Variables|Default|GetCube) (Variables|/Game/Engineers/Blueprints/Parents/BP_MagnetKey.BP_MagnetKey_C|GetMagnetTrigger _asbp_magnet_key)) (not (Variables|/Game/Engineers/Blueprints/Parents/BP_MagnetKey.BP_MagnetKey_C|GetIsHoldingSomething _asbp_magnet_key)) (not (Utilities|IsValid (Variables|Default|GetMagKey))))
    (bind _output_get (Variables|Default|SetMagKey _asbp_magnet_key))
    (EventDispatchers|BindEventtoTurnedon _output_get (delegate Custom|PickupCube))
    (EventDispatchers|BindEventtoTurnedOff _output_get (delegate Custom|DropCube))))

(fn ConstructionScript
  (Rendering|Components|TextRender|SetText (Variables|Default|GetTextRender) (Utilities|Text|ToText(String) (Utilities|String|ToString(Integer) (Variables|Default|GetNumber)))))