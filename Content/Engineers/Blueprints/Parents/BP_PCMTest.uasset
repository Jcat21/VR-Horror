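; BP_PCMTest is an Engineers parent Blueprint that tracks a seven-slot ordering puzzle.
; A Posits map stores a number per slot name, with zero meaning empty, and functions fill, clear and query slots.
; A slot is correct when its value equals the digit ending its name, parsed from the character code.
; CheckWin returns true only when Slot1 through Slot7 each hold their matching number.
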(fn ConstructionScript)

(fn CheckFilledPosition
  (params (Name :type String))
  (return (!= (.Value (Utilities|Map|Find (Variables|Default|GetPosits) Name)) 0)))

(fn FillPosition
  (params (name :type String) (value :type Integer))
  (Utilities|Map|Add (Variables|Default|GetPosits) name value)
  (return))

(fn UnfillPosition
  (params (name :type String))
  (Utilities|Map|Add (Variables|Default|GetPosits) name 0)
  (return))

(fn CheckWin
  (bind _posits (Variables|Default|GetPosits))
  (return (Math|Boolean|ANDBoolean (== (.Value (Utilities|Map|Find _posits "Slot1")) 1) (== (.Value (Utilities|Map|Find _posits "Slot2")) 2) (== (.Value (Utilities|Map|Find _posits "Slot3")) 3) (== (.Value (Utilities|Map|Find _posits "Slot4")) 4) (== (.Value (Utilities|Map|Find _posits "Slot5")) 5) (== (.Value (Utilities|Map|Find _posits "Slot6")) 6) (== (.Value (Utilities|Map|Find _posits "Slot7")) 7))))

(fn CheckCorrectPosition
  (params (Name :type String))
  (return (== (- (Utilities|String|GetCharacterasNumber Name (- (Utilities|String|Len Name) 1)) 48) (.Value (Utilities|Map|Find (Variables|Default|GetPosits) Name)))))