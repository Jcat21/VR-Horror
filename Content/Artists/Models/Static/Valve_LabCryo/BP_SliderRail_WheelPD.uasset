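; Slider rail puzzle piece in which a hand-specific magnet key drags a ball along a spline to turn a linked wheel actor.
; The construction script builds the rail from spline meshes, and BeginPlay places the ball at the start with a material matching its allowed hand.
; Overlap events register matching keys.
; Each tick, an active key snaps the ball to the nearest spline point, converting its normalized input key into incremental wheel pitch.
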(event EventBeginPlay
  (bind _ball (Variables|Default|GetBall))
  (Transformation|SetWorldLocation (Variables|Default|GetBall) (Spline|GetLocationatDistanceAlongSpline (Variables|Default|GetPath) 0.0 "World") false true)
  (switch Utilities|FlowControl|Switch|SwitchonSliderRotatorTypes (Variables|Default|GetType)
    (:NewEnumerator0
      (Rendering|Material|SetMaterial _ball 0 "/Game/Artists/Materials/M_LeftMagnetKeyDecal.M_LeftMagnetKeyDecal"))
    (:NewEnumerator1
      (Rendering|Material|SetMaterial _ball 0 "/Game/Artists/Materials/M_RightMagnetKeyDecal.M_RightMagnetKeyDecal"))
    (:NewEnumerator2
      (Rendering|Material|SetMaterial _ball 0 "/Game/Artists/Materials/M_MagnetKeyBoth.M_MagnetKeyBoth"))))

(event EventTick
  (params (DeltaSeconds :type Float%20%28single-precision%29))
  (bind _path (Variables|Default|GetPath))
  (bind _magnetkey (Variables|Default|GetmagnetKey))
  (bind _path_2 (Variables|Default|GetPath))
  (bind _magnettrigger (Variables|/Game/Engineers/Blueprints/Parents/BP_MagnetKey.BP_MagnetKey_C|GetMagnetTrigger _magnetkey))
  (bind _returnvalue (Transformation|GetWorldLocation _magnettrigger))
  (bind _returnvalue_2 (Spline|FindLocationClosesttoWorldLocation _path_2 _returnvalue "World"))
  (if (and (Variables|Default|GetisInteractingWithMagnetKey) (Utilities|IsValid _magnetkey))
    (if (and (Variables|/Game/Engineers/Blueprints/Parents/BP_MagnetKey.BP_MagnetKey_C|GetisOn _magnetkey) (Class|PrimitiveComponent|IsOverlappingComponent _magnettrigger (Variables|Default|GetBall)))
      (Transformation|SetWorldLocation (Variables|Default|GetBall) _returnvalue_2 false true)
      (bind _distance (CallFunction|FindDistanceAlongSpline _path _returnvalue_2))
      (Transformation|AddActorLocalRotation (Variables|Default|GetWheelReference) (Math|Rotator|MakeRotator 0.0 (- (Math|Float|MapRangeClamped (/ _distance (Math|Conversions|ToFloat(Integer) (- (Spline|GetNumberOfSplinePoints _path) 1))) 0.0 1.0 0.0 -1.8e+02) (Variables|Default|GetLastValue)) 0.0) false false)
      (Variables|Default|SetLastValue (Math|Float|MapRangeClamped (/ _distance (Math|Conversions|ToFloat(Integer) (- (Spline|GetNumberOfSplinePoints _path) 1))) 0.0 1.0 0.0 -1.8e+02)))))

(event Collision|EventActorBeginOverlap
  (params (OtherActor :type Actor%20Object%20Reference))
  (bind _type (Variables|Default|GetType))
  (bind _asbp_magnet_key (Utilities|Casting|CastToBP_MagnetKey OtherActor))
  (if (Math|Boolean|ORBoolean (and (Utilities|Enum|Equal(Enum) (Variables|/Game/Engineers/Blueprints/Parents/BP_MagnetKey.BP_MagnetKey_C|GetHand _asbp_magnet_key) "Left") (Utilities|Enum|Equal(Enum) _type "NewEnumerator0")) (Utilities|Enum|Equal(Enum) _type "NewEnumerator2") (and (Utilities|Enum|Equal(Enum) _type "NewEnumerator1") (Utilities|Enum|Equal(Enum) (Variables|/Game/Engineers/Blueprints/Parents/BP_MagnetKey.BP_MagnetKey_C|GetHand _asbp_magnet_key) "Right")))
    (Variables|Default|SetisInteractingWithMagnetKey true)
    (Variables|Default|SetmagnetKey _asbp_magnet_key)
    (Variables|/Game/Engineers/Blueprints/Parents/BP_MagnetKey.BP_MagnetKey_C|SetIsInteractingWithSomething _asbp_magnet_key true)
    (Default|TurnOffLight _asbp_magnet_key)))

(event Collision|EventActorEndOverlap
  (params (OtherActor :type Actor%20Object%20Reference))
  (bind _asbp_magnet_key (Utilities|Casting|CastToBP_MagnetKey OtherActor))
  (Variables|Default|SetisInteractingWithMagnetKey false)
  (Variables|/Game/Engineers/Blueprints/Parents/BP_MagnetKey.BP_MagnetKey_C|SetIsInteractingWithSomething _asbp_magnet_key false)
  (Default|ChangetoDimmerMaterial _asbp_magnet_key)
  (Variables|Default|SetmagnetKey 0))

(fn ConstructionScript
  (bind _path (Variables|Default|GetPath))
  (for _index (range 0 (- (Spline|GetNumberOfSplinePoints (Variables|Default|GetPath)) 2))
    (bind _returnvalue (AddComponent|AddSplineMeshComponent false))
    (Components|StaticMesh|SetStaticMesh _returnvalue (Variables|Default|GetpathMesh))
    (SplineMesh|SetForwardAxis _returnvalue (Variables|Default|GetForward%20Axis) true)
    (Transformation|AttachComponentToComponent _returnvalue (Variables|Default|GetPath) "None" "KeepRelative" "KeepRelative" "KeepRelative" true)
    (SplineMesh|SetStartandEnd _returnvalue (Spline|GetLocationatSplinePoint _path _index "Local") (Spline|GetTangentatSplinePoint _path _index "Local") (Spline|GetLocationatSplinePoint _path (+ _index 1) "Local") (Spline|GetTangentatSplinePoint _path (+ _index 1) "Local") true :!class /Script/Engine.SplineMeshComponent)))

(fn FindDistanceAlongSpline
  (params (Spline :type Spline%20Component%20Object%20Reference) (Location :type Vector))
  (return (Class|SplineComponent|FindInputKeyClosesttoWorldLocation Spline Location)))